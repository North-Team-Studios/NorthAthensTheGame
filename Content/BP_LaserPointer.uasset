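; Laser pointer Blueprint that draws a Niagara beam toward whatever is under the mouse cursor.
; Each Tick shows the beam unless the player character moves fast.
; While tracing is activated, it sets the beam length from the pointer mesh to the cursor hit and hides both beam and mesh during reloads.
; An impact reticle effect spawns hidden at BeginPlay, but its update logic and several alternative traces are disconnected.
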(event `LaserPointer`
  (bind _returnvalue (`GameplayStatics.GetPlayerCharacter` 0))
  (`/Engine/EditorBlueprintResources/StandardMacros.IsValid` _returnvalue
    (:`Is Valid`
      (if (> (`KismetMathLibrary.VSize` (`self.GetVelocity` _returnvalue)) 400.0)
        (`SceneComponent.SetVisibility` (`self.Niagara_LaserPointer`) false false)
        (else
          (`SceneComponent.SetVisibility` (`self.Niagara_LaserPointer`) true false))))))

(event `self.ReceiveBeginPlay`
  (bind _returnvalue (`NiagaraFunctionLibrary.SpawnSystemAtLocation` "/Game/_Materials/VFX/FX_Pointer.FX_Pointer"))
  (set `self.VFX_Mira` _returnvalue)
  (`SceneComponent.SetVisibility` (`self.VFX_Mira`) false false))

(event `self.ReceiveTick`
  (params (DeltaSeconds :type "Float (single-precision)"))
  (`self.LaserPointer`)
  (if (`self.Line Trace Activated?`)
    (`self.LineTrace`)
    (if (`/Game/Characters/Jogador/Blueprint/BP_Jogador.isReloading?` (`/Game/_Mechanics/QuestSystem/BPL_CommonFunctionLibrary.GetMyPlayerCharacter`))
      (`SceneComponent.SetVisibility` (`self.Niagara_LaserPointer`) false false)
      (`SceneComponent.SetVisibility` (`self.SM_LaserPointer`) false false))))

(event `LineTrace`
  (`FXSystemComponent.SetVectorParameter` (`self.Niagara_LaserPointer`) "Beam End" (`KismetMathLibrary.MakeVector` (`KismetMathLibrary.Vector_Distance` (`SceneComponent.K2_GetComponentLocation` (`self.SM_LaserPointer`)) (`.Location` (`GameplayStatics.BreakHitResult` (`PlayerController.GetHitResultUnderCursorByChannel` (`GameplayStatics.GetPlayerController` 0) "TraceTypeQuery2" true)))))))

(fn `UserConstructionScript`)