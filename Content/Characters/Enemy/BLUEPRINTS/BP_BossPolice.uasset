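; BP_BossPolice is an enemy character Blueprint for a police boss, with an inactive event graph and a construction script that only calls its parent.
; SetMovementSpeed maps a movement state from idle to sprinting onto the CharacterMovement max walk speed and returns that value.
; GetMaxHealth reads maximum health from the BPCDamageSystem component.
; NewFunction is an empty stub.
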(fn `GetMaxHealth`
  (returns (MaxHealth :type "Float (double-precision)"))
  (return (`/Game/_Mechanics/DamageSystem/BPC_DamageSystem.MaxHealth` (`self.BPC_DamageSystem`))))

(fn `NewFunction`)

(fn `SetMovementSpeed`
  (params (Speed :type "/Game/Enemy/Ai/Enums/E_MovementSpeed Enum" :default "NewEnumerator0"))
  (returns (SpeedValue :type "Float (double-precision)"))
  (bind _output_get (set `CharacterMovementComponent.MaxWalkSpeed` (select `/Game/Enemy/Ai/Enums/E_MovementSpeed` Speed :`NewEnumerator1` 100.0 :`NewEnumerator2` 300.0 :`NewEnumerator3` 425.0 :!type "Float (single-precision)") (`self.CharacterMovement`)))
  (return _output_get))

(fn `UserConstructionScript`
  (`parent.UserConstructionScript`))