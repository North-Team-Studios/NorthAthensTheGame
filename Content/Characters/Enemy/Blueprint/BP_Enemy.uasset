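; Enemy character Blueprint that carries player-style input movement, ammo bookkeeping and a health system, and triggers game over when it dies.
; Health, healing and damage calls forward to BPCDamageSystem, whose death, block and damage-response events are bound in the construction script.
; Death disables mesh collision and player input and shows WB_GameOver, while block and damage responses only print debug text.
; Enhanced Input mapping applies only under BP_PlayerController.
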(event `self.ReceiveBeginPlay`
  ;[0.0625 0.0625 0.0625] AI Begin Play
  (bind _asbp_player_controller (cast `/Game/Characters/Jogador/BP_PlayerController` (`self.GetController`)))
  (`EnhancedInputSubsystemInterface.AddMappingContext` (pcsubsystem `EnhancedInputLocalPlayerSubsystem` _asbp_player_controller) "/Game/ThirdPerson/Input/IMC_Default.IMC_Default" 0 (struct)))

(event `EnhancedInput|/Game/ThirdPerson/Input/Actions/IA_Move`
  (params (ActionValue :type "Vector2D Structure") (ElapsedSeconds :type "Float (double-precision)") (TriggeredSeconds :type "Float (double-precision)") (InputAction :type "InputAction Object Reference" :default "/Game/ThirdPerson/Input/Actions/IA_Move.IA_Move"))
  ;[0.0625 0.0625 0.0625] AI Move
  (:`Triggered`
    (`self.AddMovementInput` (`self.GetActorForwardVector`) ActionValue_Y)
    (`self.AddMovementInput` (`self.GetActorRightVector`) ActionValue_X)))

(event `Blocked`
  (params (`Can Be Parried` :type Boolean))
  ;[0.07812 0.07812 0.07812] Comment
  (`KismetSystemLibrary.PrintString` "Blocked"))

(event `DamageResponse`
  (params (DamageResponse :type "/Game/DamageSystem/E_DamageResponse Enum" :default "NewEnumerator0"))
  ;[0.07812 0.07812 0.07812] Comment
  (`KismetSystemLibrary.PrintString` (`|GetEnumeratorNameAsString` DamageResponse)))

(event `Death`
  (bind _returnvalue (`GameplayStatics.GetPlayerController` 0))
  (bind _mesh (`self.Mesh`))
  ;[0.1146 0.1146 0.1146] Death
  (`PrimitiveComponent.SetSimulatePhysics` _mesh false)
  (`PrimitiveComponent.SetCollisionEnabled` _mesh "NoCollision")
  (`self.DisableInput` _returnvalue null)
  (bind _returnvalue_2 (`|CreateWidget` "/Game/Layout/WB_GameOver.WB_GameOver_C"))
  (bind _output_get (set `self.Game Over Menu` _returnvalue_2))
  (`UserWidget.AddToViewport` _output_get 0)
  (`WidgetBlueprintLibrary.SetInputMode_GameAndUIEx` _returnvalue (`self.Game Over Menu`))
  (set `PlayerController.bShowMouseCursor` false _returnvalue))

(fn `GetCurrentHealth`
  (returns (Health :type "Float (double-precision)"))
  (return (`/Game/DamageSystem/BPC_DamageSystem.Health` (`self.BPC_DamageSystem`))))

(fn `GetMaxHealth`
  (returns (MaxHealth :type "Float (double-precision)"))
  (return (`/Game/DamageSystem/BPC_DamageSystem.MaxHealth` (`self.BPC_DamageSystem`))))

(fn `Heal`
  (params (Amount :type "Float (double-precision)"))
  (returns (NewHealth :type "Float (double-precision)"))
  (bind _newhealth (`/Game/DamageSystem/BPC_DamageSystem.Heal` (`self.BPC_DamageSystem`) Amount))
  (return _newhealth))

(fn `Reload`
  (locals (TempAmmo :type Integer))
  (bind _ammo (`self.Ammo`))
  (set `local.TempAmmo` _ammo)
  (set `self.Ammo` (`KismetMathLibrary.Clamp` (- _ammo (- 8 (`self.Current Ammo`))) 0 (`self.Ammo`)))
  (set `self.no_ammo` false)
  (set `self.Current Ammo` (+ (- (`local.TempAmmo`) (`self.Ammo`)) (`self.Current Ammo`)))
  (if (`self.InifiniteAmmo?`)
    (set `self.Ammo` 999)))

(fn `TakeDamage`
  (params (DamageInfo :type "/Game/DamageSystem/S_DamageInfo Structure"))
  (returns (WasDamaged :type Boolean))
  (bind _wasdamaged (`/Game/DamageSystem/BPC_DamageSystem.TakeDamage` (`self.BPC_DamageSystem`) DamageInfo))
  (return _wasdamaged))

(fn `time`
  (params (Limite :type Integer))
  (returns (finalizado :type Boolean))
  (locals (TimeOAUX :type Integer))
  (if (== (- 61 (`self.seconds`)) Limite)
    (return true)))

(fn `Use Ammo`
  (set `self.Current Ammo` (`KismetMathLibrary.Clamp` (- (`self.Current Ammo`) 1) 0 30)))

(fn `UserConstructionScript`
  (add `/Game/DamageSystem/BPC_DamageSystem.OnDeath` (`self.BPC_DamageSystem`) (`|CreateDelegate` :!event `Death`))
  (add `/Game/DamageSystem/BPC_DamageSystem.OnBlocked` (`self.BPC_DamageSystem`) (`|CreateDelegate` :!event `Blocked`))
  (add `/Game/DamageSystem/BPC_DamageSystem.OnDamageRespone` (`self.BPC_DamageSystem`) (`|CreateDelegate` :!event `DamageResponse`)))