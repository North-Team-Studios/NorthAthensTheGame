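; BP_Clide is the player character Blueprint, handling pause menu toggling and a modular jacket mesh.
; The IA_Escape Enhanced Input action flips IsPauseMenu to create or remove WB_PauseMenu, switching game pause, input mode and mouse cursor with it.
; The construction script sets the main Mesh as leader pose for the Jaqueta (jacket) component, so the jacket follows the body's animation.
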(event `EnhancedInput|/Game/ThirdPerson/Input/Actions/IA_Escape`
  (params (ActionValue :type Boolean) (ElapsedSeconds :type "Float (double-precision)") (TriggeredSeconds :type "Float (double-precision)") (InputAction :type "InputAction Object Reference" :default "/Game/ThirdPerson/Input/Actions/IA_Escape.IA_Escape"))
  (bind _returnvalue (`GameplayStatics.GetPlayerController` 0))
  (bind _returnvalue_2 (`GameplayStatics.GetPlayerController` 0))
  (:`Started`
    (if (not (`self.IsPauseMenu`))
      (set `self.IsPauseMenu` true)
      (bind _returnvalue_3 (`|CreateWidget` "/Game/_Layout/HUD/WB_PauseMenu.WB_PauseMenu_C" _returnvalue))
      (bind _output_get (set `self.Pause Menu` _returnvalue_3))
      (`UserWidget.AddToViewport` _output_get 0)
      (`WidgetBlueprintLibrary.SetInputMode_GameAndUIEx` _returnvalue null)
      (set `PlayerController.bShowMouseCursor` true (`GameplayStatics.GetPlayerController` 0))
      (`GameplayStatics.SetGamePaused` true)
      (else
        (set `self.IsPauseMenu` false)
        (`Widget.RemoveFromParent` (`self.Pause Menu`))
        (`GameplayStatics.SetGamePaused` false)
        (`WidgetBlueprintLibrary.SetInputMode_GameOnly` _returnvalue_2)
        (set `PlayerController.bShowMouseCursor` false _returnvalue_2)))))

(event `self.ReceiveBeginPlay`)

(fn `UserConstructionScript`
  (`SkinnedMeshComponent.SetLeaderPoseComponent` (`self.Jaqueta`) (`self.Mesh`) false false))