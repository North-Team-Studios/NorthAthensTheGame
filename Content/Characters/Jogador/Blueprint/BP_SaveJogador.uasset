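; Player character Blueprint with Enhanced Input movement, pause menu, ammo tracking and a stage countdown that triggers death at zero.
; BPCDamageSystem handles health, healing and damage through wrapper functions, and its death event pauses the game and shows game over with the score.
; Tick drives the timer through a one-second Delay and polls health and empty ammo.
; Skill 1 grants a timed gun damage bonus, with delay loops counting duration and cooldown.
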(event `EnhancedInput|/Game/MainPlayer/Input/Actions/IA_PauseGame`
  (params (ActionValue :type Boolean) (ElapsedSeconds :type "Float (double-precision)") (TriggeredSeconds :type "Float (double-precision)") (InputAction :type "InputAction Object Reference" :default "/Game/MainPlayer/Input/Actions/IA_PauseGame.IA_PauseGame"))
  (bind _returnvalue (`GameplayStatics.GetPlayerController` 0))
  (bind _returnvalue_2 (`GameplayStatics.GetPlayerController` 0))
  ;[0.09375 0.09375 0.09375] PauseMenu
  (:`Started`
    (if (not (`self.IsPauseMenu`))
      (set `self.IsPauseMenu` true)
      (bind _returnvalue_3 (`|CreateWidget` "/Game/Layout/WB_PauseMenu.WB_PauseMenu_C" _returnvalue))
      (bind _output_get (set `self.PauseMenu` _returnvalue_3))
      (`UserWidget.AddToViewport` _output_get 0)
      (`WidgetBlueprintLibrary.SetInputMode_GameAndUIEx` _returnvalue null)
      (set `PlayerController.bShowMouseCursor` true (`GameplayStatics.GetPlayerController` 0))
      (`GameplayStatics.SetGamePaused` true)
      (else
        (set `self.IsPauseMenu` false)
        (`Widget.RemoveFromParent` (`self.PauseMenu`))
        (`GameplayStatics.SetGamePaused` false)
        (`WidgetBlueprintLibrary.SetInputMode_GameOnly` _returnvalue_2)
        (set `PlayerController.bShowMouseCursor` false _returnvalue_2)))))

(event `self.ReceiveBeginPlay`
  ;[0.0625 0.0625 0.0625] AI Begin Play
  (set `self.Score` 0)
  (bind _asbp_player_controller (cast `/Game/Characters/Jogador/BP_PlayerController` (`self.GetController`)))
  (`EnhancedInputSubsystemInterface.AddMappingContext` (pcsubsystem `EnhancedInputLocalPlayerSubsystem` _asbp_player_controller) "/Game/ThirdPerson/Input/IMC_Default.IMC_Default" 0 (struct))
  ;[0.276 0.276 0.276] Health
  (set `self.MaxHealth` (`/Game/DamageSystem/BPC_DamageSystem.MaxHealth` (`self.BPC_DamageSystem`))))

(event `EnhancedInput|/Game/ThirdPerson/Input/Actions/IA_Move`
  (params (ActionValue :type "Vector2D Structure") (ElapsedSeconds :type "Float (double-precision)") (TriggeredSeconds :type "Float (double-precision)") (InputAction :type "InputAction Object Reference" :default "/Game/ThirdPerson/Input/Actions/IA_Move.IA_Move"))
  (bind (_returnvalue_roll _returnvalue_pitch _returnvalue_yaw) (`KismetMathLibrary.BreakRotator` (`self.GetControlRotation`)))
  (bind (_returnvalue_roll_2 _returnvalue_pitch_2 _returnvalue_yaw_2) (`KismetMathLibrary.BreakRotator` (`self.GetControlRotation`)))
  ;[0.0625 0.0625 0.0625] AI Move
  (:`Triggered`
    (`self.AddMovementInput` (`KismetMathLibrary.GetRightVector` (`KismetMathLibrary.MakeRotator` _returnvalue_roll_2 0.0 _returnvalue_yaw_2)) ActionValue_X)
    (`self.AddMovementInput` (`KismetMathLibrary.GetForwardVector` (`KismetMathLibrary.MakeRotator` 0.0 0.0 _returnvalue_yaw)) ActionValue_Y)))

(event `Blocked`
  (params (`Can Be Parried` :type Boolean))
  ;[0.2656 0.2656 0.2656] Comment
  (`KismetSystemLibrary.PrintString` "Blocked"))

(event `DamageResponse`
  (params (DamageResponse :type "/Game/DamageSystem/E_DamageResponse Enum" :default "NewEnumerator0"))
  ;[0.2656 0.2656 0.2656] Comment
  (`KismetSystemLibrary.PrintString` (`|GetEnumeratorNameAsString` DamageResponse)))

(event `Death`
  (bind _returnvalue (`GameplayStatics.GetPlayerController` 0))
  (bind _mesh (`self.Mesh`))
  ;[0.1146 0.1146 0.1146] Death
  (`GameplayStatics.SetGamePaused` true)
  (`PrimitiveComponent.SetSimulatePhysics` _mesh false)
  (`PrimitiveComponent.SetCollisionEnabled` _mesh "NoCollision")
  (`self.DisableInput` _returnvalue null)
  (bind _returnvalue_2 (`|CreateWidget` "/Game/Layout/WB_GameOver.WB_GameOver_C"))
  (bind _output_get (set `self.Game Over Menu` _returnvalue_2))
  (set `/Game/Layout/WB_GameOver.FinalScore` (`self.Score`) _output_get)
  (`UserWidget.AddToViewport` _output_get 0)
  (`WidgetBlueprintLibrary.SetInputMode_GameAndUIEx` _returnvalue (`self.Game Over Menu`))
  (set `PlayerController.bShowMouseCursor` true _returnvalue))

(event `self.ReceiveTick`
  (params (DeltaSeconds :type "Float (single-precision)"))
  (bind _seconds (`self.seconds`))
  ;[0.1198 0.1198 0.1198] Event Tick
  (`|ExecutionSequence`
    (:`then_0`
      ;;[1 0.2708 0.5357] Set Max Time
      (`/Engine/EditorBlueprintResources/StandardMacros.DoOnce` false
        (:`Completed`
          (set `self.max_time` (+ (* (`self.minutes`) 60) (`self.seconds`))))))
    (:`then_1`
      ;;[0.1357 0.2884 1] Check State - No Ammo
      (`/Engine/EditorBlueprintResources/StandardMacros.CompareInt` (`self.Current Ammo`)
        (:`==`
          (set `self.no_ammo` true))))
    (:`then_2`
      ;;[0.1043 1 0.1512] Stage Timer
      (`/Engine/EditorBlueprintResources/StandardMacros.CompareInt` (+ (`self.minutes`) (`self.seconds`))
        (:`>`
          (`KismetSystemLibrary.Delay` 1.0)
          (`/Engine/EditorBlueprintResources/StandardMacros.CompareInt` _seconds
            (:`>`
              (set `self.seconds` (- _seconds 1)))
            (:`==`
              (`/Engine/EditorBlueprintResources/StandardMacros.CompareInt` (`self.minutes`)
                (:`>`
                  (set `self.seconds` 59)
                  (set `self.minutes` (- (`self.minutes`) 1))))))
          ;;[1 0.8904 0.2517] set_max_timer
          (set `self.current_time` (+ (* (`self.minutes`) 60) (`self.seconds`)))
          (if (== (`self.current_time`) 0)
            (`self.Death`)))))
    (:`then_3`
      ;;[0.1979 0.1979 0.1979] Update Health
      (set `self.CurrentHealth` (`/Game/DamageSystem/BPC_DamageSystem.Health` (`self.BPC_DamageSystem`))))))

(event `EnhancedInput|/Game/ThirdPerson/Input/Actions/IA_Skill1`
  (params (ActionValue :type Boolean) (ElapsedSeconds :type "Float (double-precision)") (TriggeredSeconds :type "Float (double-precision)") (InputAction :type "InputAction Object Reference" :default "/Game/ThirdPerson/Input/Actions/IA_Skill1.IA_Skill1"))
  (bind _skill1_current_cooltime (`self.skill1_current_cooltime`))
  ;[0.004949 1 0.01923] Skill Mechs
  (:`Triggered`
    (if (and (`self.skill1_active`) (not (`self.skill1_cooldown`)))
      (`KismetSystemLibrary.PrintString` "Skill já está ativa")
      (elif (not (or (`self.skill1_active`) (`self.skill1_cooldown`)))
        (`self.Skill_AddDamageBonus`)
        (if (>= (`self.skill1_current_duration`) (`self.skill1_duration`)) :!label _label
          (set `self.skill1_active` false)
          (set `self.skill1_current_duration` 0.0)
          (set `self.Gun Damage Bonus` 0.0)
          (set `self.skill1_cooldown` true)
          (set `self.skill1_current_cooltime` (`self.skill1_cooltime`))
          (if (== (`self.skill1_current_cooltime`) 0.0) :!label _label_2
            (set `self.skill1_cooldown` false)
            (else
              (`/Engine/EditorBlueprintResources/StandardMacros.CompareFloat` _skill1_current_cooltime
                (:`>`
                  (`KismetSystemLibrary.Delay` 1.0)
                  (set `self.skill1_current_cooltime` (- _skill1_current_cooltime 1.0))
                  (goto _label_2)))))
          (else
            (`KismetSystemLibrary.RetriggerableDelay` 1.0)
            (set `self.skill1_current_duration` (+ (`self.skill1_current_duration`) 1.0))
            (goto _label)))
        (elif (`self.skill1_cooldown`)
          (set `self.show_warning_skill_hud` true)
          (`KismetSystemLibrary.Delay` 1.0)
          (set `self.show_warning_skill_hud` false))))))

(fn `GetCurrentHealth`
  (returns (Health :type "Float (double-precision)"))
  (return (`/Game/DamageSystem/BPC_DamageSystem.Health` (`self.BPC_DamageSystem`))))

(fn `GetMaxHealth`
  (returns (MaxHealth :type "Float (double-precision)"))
  (return (`/Game/DamageSystem/BPC_DamageSystem.MaxHealth` (`self.BPC_DamageSystem`))))

(fn `Heal`
  (params (Amount :type "Float (double-precision)"))
  (returns (NewHealth :type "Float (double-precision)"))
  (bind _newhealth (`/Game/DamageSystem/BPC_DamageSystem.Heal` (`self.BPC_DamageSystem`) Amount))
  (return _newhealth))

(fn `OLDReload`
  (locals (TempAmmo :type Integer))
  (bind _ammo (`self.Ammo`))
  (set `local.TempAmmo` _ammo)
  (set `self.Ammo` (`KismetMathLibrary.Clamp` (- _ammo (- 8 (`self.Current Ammo`))) 0 (`self.Ammo`)))
  (set `self.no_ammo` false)
  (set `self.Current Ammo` (+ (- (`local.TempAmmo`) (`self.Ammo`)) (`self.Current Ammo`)))
  (if (`self.InifiniteAmmo?`)
    (set `self.Ammo` 999)))

(fn `Skill_AddDamageBonus`
  (set `self.skill1_active` true)
  (set `self.Gun Damage Bonus` (+ 40.0 0.0))
  (`GameplayStatics.PlaySound2D` "/Game/Audio/SFX_Hud/SFX_PowerUp.SFX_PowerUp" 0.3 1.0 0.0 null null)
  (`GameplayStatics.PlaySound2D` "/Game/Audio/SFX_Karen/SFX_Karen_PowerUps.SFX_Karen_PowerUps" 3.0 1.0 0.0 null null))

(fn `TakeDamage`
  (params (DamageInfo :type "/Game/DamageSystem/S_DamageInfo Structure"))
  (returns (WasDamaged :type Boolean))
  (bind _wasdamaged (`/Game/DamageSystem/BPC_DamageSystem.TakeDamage` (`self.BPC_DamageSystem`) DamageInfo))
  (return _wasdamaged))

(fn `time`
  (params (Limite :type Integer))
  (returns (finalizado :type Boolean))
  (locals (TimeOAUX :type Integer))
  (if (== (- 61 (`self.seconds`)) Limite)
    (return true)))

(fn `Use Ammo`
  (set `self.Current Ammo` (`KismetMathLibrary.Clamp` (- (`self.Current Ammo`) 1) 0 30)))

(fn `UserConstructionScript`
  (add `/Game/DamageSystem/BPC_DamageSystem.OnDeath` (`self.BPC_DamageSystem`) (`|CreateDelegate` :!event `Death`))
  (add `/Game/DamageSystem/BPC_DamageSystem.OnBlocked` (`self.BPC_DamageSystem`) (`|CreateDelegate` :!event `Blocked`))
  (add `/Game/DamageSystem/BPC_DamageSystem.OnDamageRespone` (`self.BPC_DamageSystem`) (`|CreateDelegate` :!event `DamageResponse`))
  (`SkinnedMeshComponent.SetLeaderPoseComponent` (`self.Jaqueta`) (`self.Mesh`) false false))