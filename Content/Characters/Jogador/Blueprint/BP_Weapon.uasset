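; BP_Weapon is the player's gun, handling ammo, projectile firing and hit damage.
; On BeginPlay it fills the ammo and picks a damage bonus from DT_HPVariables' pistol row by the Game Instance's TestDamage level.
; Shoot makes noise, spends a round without checking ammo, and spawns a BP_Tiro whose impact event applies damage and sparks to non-player hits.
; An unreachable older firing path uses the player's GunDamageBonus instead.
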(event `self.ReceiveBeginPlay`
  (set `self.Current Ammo` (`self.MaxAmmo`))
  (bind _asbp_jogador (cast `/Game/Characters/Jogador/Blueprint/BP_Jogador` (`GameplayStatics.GetPlayerCharacter` 0)))
  (set `self.Jogador` _asbp_jogador)
  (bind _asbpi_game_instance (cast `/Game/_Mechanics/SaveGame/BPI_GameInstance` (`GameplayStatics.GetGameInstance`)))
  (bind _output_get (set `self.GameInstance` _asbpi_game_instance))
  (bind _returnvalue (`|GetDataTableRow` "/Game/_Mechanics/DamageSystem/GeneralValues/DT_HPVariables.DT_HPVariables" "PistolDamageBonus")
    (:`then`
      (switch `int` (`/Game/_Mechanics/SaveGame/BPI_GameInstance.TestDamage` _output_get)
        (:`0`
          (bind (_damageinfo _levelone _leveltwo _levelthree _levelfour _levelfive) (break `/Game/_Mechanics/DamageSystem/GeneralValues/DamageStructure` _returnvalue))
          (set `self.DamageLevel` _levelone :!label _label))
        (:`1`
          (goto _label))
        (:`2`
          (set `self.DamageLevel` _leveltwo))
        (:`3`
          (set `self.DamageLevel` _levelthree))
        (:`4`
          (set `self.DamageLevel` _levelfour))
        (:`5`
          (set `self.DamageLevel` _levelfive))))))

(event `Shoot`
  (bind _myplayercharacter (`/Game/_Mechanics/QuestSystem/BPL_CommonFunctionLibrary.GetMyPlayerCharacter`))
  (bind _returnvalue (`SceneComponent.K2_GetComponentRotation` (`self.Arrow`)))
  (bind _returnvalue_2 (+ (`SceneComponent.K2_GetComponentLocation` (`self.Arrow`)) _returnvalue))
  (bind _returnvalue_3 (`KismetMathLibrary.MakeTransform` _returnvalue_2 _returnvalue))
  (`self.MakeNoise` 1.0 _myplayercharacter (`self.K2_GetActorLocation` _myplayercharacter))
  (`self.MenosUmTiro`)
  (`GameplayStatics.SpawnEmitterAtLocation` (`self.Muzzle Flash`) _returnvalue_2 (struct) (1.5 1.5 1.5))
  (bind _returnvalue_4 (`|SpawnActorFromClass` "/Game/Weapons/Blueprint/BP_Tiro.BP_Tiro_C" (`KismetMathLibrary.MakeTransform` (`KismetMathLibrary.MakeVector` (.x (.location _returnvalue_3)) (.y (.location _returnvalue_3)) (.z (.location _returnvalue_3))) (`KismetMathLibrary.MakeRotator` 0.0 (.pitch (.rotation _returnvalue_3)) (.yaw (.rotation _returnvalue_3)))) "Undefined" "MultiplyWithRoot" self (`self.WeaponVellocity`) 0.0 null (`GameplayStatics.GetPlayerCharacter` 0)))
  (add `/Game/Weapons/Blueprint/BP_BaseProjectile.OnProjectileImpact` _returnvalue_4 (delegate `Projectile Impact`))
  (`PrimitiveComponent.IgnoreActorWhenMoving` (`self.Weapon`) null false))

(event `Projectile Impact`
  (params (`Other Actror` :type "Actor Object Reference") (Hit :type "HitResult Structure"))
  (if (!= Hit_HitActor (`/Game/_Mechanics/QuestSystem/BPL_CommonFunctionLibrary.GetMyPlayerCharacter`))
    (message `/Game/_Mechanics/DamageSystem/BPI_Damagable.TakeDamage` Hit_HitActor (make `/Game/_Mechanics/DamageSystem/S_DamageInfo` (+ (`self.DamageLevel`) 10.0) (`self.Damage Type`) "NewEnumerator1"))
    (`GameplayStatics.SpawnEmitterAtLocation` "/Game/Weapons/FX/P_Impact_Metal_Small_01.P_Impact_Metal_Small_01" Hit_TraceStart (struct) (0.5 0.5 0.5))))

(event `CustomEvent`
  (params (`Other Actror` :type "Actor Object Reference") (Hit :type "HitResult Structure"))
  (bind _asbp_jogador (cast `/Game/Characters/Jogador/Blueprint/BP_Jogador` (`GameplayStatics.GetPlayerCharacter` 0)))
  (message `/Game/_Mechanics/DamageSystem/BPI_Damagable.TakeDamage` Hit_HitActor (make `/Game/_Mechanics/DamageSystem/S_DamageInfo` (+ (`/Game/Characters/Jogador/Blueprint/BP_Jogador.Gun Damage Bonus` _asbp_jogador) 10.0) (`self.Damage Type`) "NewEnumerator1"))
  (`GameplayStatics.SpawnEmitterAtLocation` (`self.Muzzle Flash`) Hit_TraceStart (struct) (2.0 2.0 2.0)))

(fn `Ammo In Weapon?`
  (returns (IsAmmo :type Boolean))
  (return (!= (`self.Current Ammo`) 0)))

(fn `MenosUmTiro`
  (set `self.Current Ammo` (- (`self.Current Ammo`) 1)))

(fn `Reload`
  (set `self.Current Ammo` (`self.MaxAmmo`)))

(fn `UserConstructionScript`)