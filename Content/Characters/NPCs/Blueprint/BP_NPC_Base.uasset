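; Base NPC Blueprint that shows a widget when the player enters its interaction box and a name label set from CharacterName at construction.
; An interactable-state event toggles the name label.
; Look-at starts the player's interact transition and shows the cursor; closing conversation notifies the instigator, restores game-only input and ends the transition.
; InteractWith returns an empty value, and the UI-only input lock is disconnected.
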(event `self.InteractionWBox.OnComponentBeginOverlap`
  (params (OverlappedComponent :type "PrimitiveComponent Object Reference") (OtherActor :type "Actor Object Reference") (OtherComp :type "PrimitiveComponent Object Reference") (OtherBodyIndex :type Integer) (bFromSweep :type Boolean) (SweepResult :type "HitResult Structure (by ref)"))
  (if (== (`/Game/_Mechanics/QuestSystem/BPL_CommonFunctionLibrary.GetMyPlayerCharacter`) OtherActor)
    (`SceneComponent.SetVisibility` (`self.Widget`) true false)))

(event `self.InteractionWBox.OnComponentEndOverlap`
  (params (OverlappedComponent :type "PrimitiveComponent Object Reference") (OtherActor :type "Actor Object Reference") (OtherComp :type "PrimitiveComponent Object Reference") (OtherBodyIndex :type Integer))
  (`SceneComponent.SetVisibility` (`self.Widget`) false false))

(event `/Game/_Mechanics/BPI_MainInteract.SetInteractableState`
  (params (NewParam :type Boolean))
  (if NewParam
    (`SceneComponent.SetVisibility` (`self.Txt_CharacterName`) true false)
    (else
      (`SceneComponent.SetVisibility` (`self.Txt_CharacterName`) false false))))

(event `/Game/_Mechanics/BPI_MainInteract.ConversationClosed`
  (message `/Game/_Mechanics/DialogueSystem/BPI_Interactable.ConversationClosed` (`self.InteractInstigator`))
  (set `PlayerController.bShowMouseCursor` false (`GameplayStatics.GetPlayerController` 0))
  (`WidgetBlueprintLibrary.SetInputMode_GameOnly` (`GameplayStatics.GetPlayerController` 0))
  (`/Game/Characters/Jogador/Blueprint/BP_Jogador.InteractTransitionEnd` (`/Game/_Mechanics/QuestSystem/BPL_CommonFunctionLibrary.GetMyPlayerCharacter`)))

(event `/Game/_Mechanics/BPI_MainInteract.LookAt`
  (`/Game/Characters/Jogador/Blueprint/BP_Jogador.InteractTransitionBegin` (`/Game/_Mechanics/QuestSystem/BPL_CommonFunctionLibrary.GetMyPlayerCharacter`))
  (set `PlayerController.bShowMouseCursor` true (`GameplayStatics.GetPlayerController` 0)))

(fn `Interact With`
  (returns (ObjectiveID :type String))
  (return ""))

(fn `UserConstructionScript`
  (`TextRenderComponent.K2_SetText` (`self.Txt_CharacterName`) (`self.CharacterName`)))