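; Base NPC Blueprint that displays a character name label and responds to interaction and conversation events.
; The construction script writes the character name into the text component, and the interactable-state event shows or hides that label.
; When a conversation closes, it forwards a conversation-closed message to the interaction instigator.
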(event `self.SetInteractableState`
  (params (bCanShowInteractable :type Boolean))
  (if bCanShowInteractable
    (`SceneComponent.SetVisibility` (`self.Txt_CharacterName`) true false)
    (else
      (`SceneComponent.SetVisibility` (`self.Txt_CharacterName`) false false))))

(event `self.ConversationClosed`
  (message `/Game/_Mechanics/DialogueSystem/BPI_Interactable.ConversationClosed` (`self.InteractInstigator`)))

(fn `UserConstructionScript`
  (`TextRenderComponent.K2_SetText` (`self.Txt_CharacterName`) (`self.CharacterName`)))