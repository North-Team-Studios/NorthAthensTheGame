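; NPC Blueprint for Karen, who starts a conversation when looked at and can give a quest.
; On BeginPlay it reads game progress from the GameInstance interface to choose its starting State.
; Look-at runs the parent logic and opens the Karen dialogue component, briefly switching State at later progress.
; The dialogue's NewQuest event calls the quest-giver component and stores the returned objective ID.
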(event `self.ReceiveBeginPlay`
  (bind _asbpi_game_instance (cast `/Game/_Mechanics/SaveGame/BPI_GameInstance` (`GameplayStatics.GetGameInstance`)))
  (bind _progress (`/Game/_Mechanics/SaveGame/BPI_GameInstance.GetGameProgress` _asbpi_game_instance))
  (if (>= _progress 5)
    (set `self.State` "NewEnumerator0")
    (else
      (set `self.State` "NewEnumerator1"))))

(event `/Game/_Mechanics/BPI_MainInteract.LookAt`
  (`parent.LookAt`)
  (set `self.InteractInstigator` (`/Game/_Mechanics/QuestSystem/BPL_CommonFunctionLibrary.GetMyPlayerCharacter`))
  (`/Game/_Mechanics/DialogueSystem/BPC_DialogueBase.OpenConversation` (`self.BPC_KarenDialogue`))
  ;[1 1 1] CONSERTÁ
  (if (>= (stale `self.ReceiveBeginPlay` _progress) 5)
    (set `self.State` "NewEnumerator2")
    (`KismetSystemLibrary.Delay` 3.0)
    (set `self.State` "NewEnumerator0")))

(event `self.BPC_KarenDialogue.NewQuest`
  (bind _objectiveid (`/Game/_Mechanics/QuestSystem/BPC_QuestGiven.Interact With` (`self.BPC_QuestGiven`)))
  (set `self.Objective ID Local` _objectiveid))

(fn `Interact With`
  (returns (ObjectiveID :type String))
  (return ""))

(fn `NewQuest`
  (returns (ObjectiveID :type String))
  (bind _objectiveid (`/Game/_Mechanics/BPI_MainInteract.Interact With` (`self.BPC_QuestGiven`)))
  (return _objectiveid))

(fn `UserConstructionScript`
  (`parent.UserConstructionScript`))