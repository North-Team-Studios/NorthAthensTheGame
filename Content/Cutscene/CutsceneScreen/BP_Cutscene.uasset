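; Cutscene trigger actor that plays a media video in a fullscreen widget when the local player character enters its box.
; A DoOnce precedes the player check, so only the first overlap by any actor counts.
; It shows WB_CutsceneScreen, opens the media source, switches input mapping and pauses the game.
; Video end calls the widget's CloseCutscene, and its OnCrose event stops the media sound.
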(event `self.ReceiveBeginPlay`
  (`MediaSoundComponent.SetMediaPlayer` (`self.MediaSound`) "/Game/Cutscene/CutsceneScreen/MP_Cutscenes.MP_Cutscenes")
  (add `MediaPlayer.OnEndReached` (`self.Media Player`) (delegate `CloseVideo`)))

(event `CloseVideo`
  (bind _widgetcutscene (`self.WidgetCutscene`)
    (:`then`
      (`/Game/Cutscene/CutsceneScreen/WB_CutsceneScreen.CloseCutscene` _widgetcutscene))
    (:`else`)))

(event `self.Box.OnComponentBeginOverlap`
  (params (OverlappedComponent :type "PrimitiveComponent Object Reference") (OtherActor :type "Actor Object Reference") (OtherComp :type "PrimitiveComponent Object Reference") (OtherBodyIndex :type Integer) (bFromSweep :type Boolean) (SweepResult :type "HitResult Structure (by ref)"))
  (`/Engine/EditorBlueprintResources/StandardMacros.DoOnce` false
    (:`Completed`
      (if (== OtherActor (`/Game/_Mechanics/QuestSystem/BPL_CommonFunctionLibrary.GetMyPlayerCharacter`))
        (`self.WidgetCutscene`
          (:`then`
            _)
          (:`else`
            (bind _returnvalue (`|CreateWidget` "/Game/Cutscene/CutsceneScreen/WB_CutsceneScreen.WB_CutsceneScreen_C"))
            (bind _output_get (set `self.WidgetCutscene` _returnvalue))))
        (`UserWidget.AddToViewport` _output_get 0)
        (`Widget.SetKeyboardFocus` _returnvalue)
        (`MediaPlayer.OpenSource` (`self.Media Player`) (`self.Media Source`))
        (`/Game/_Mechanics/QuestSystem/BPL_CommonFunctionLibrary.SwitchMappingContext` "NewEnumerator1")
        (`GameplayStatics.SetGamePaused` true)
        (add `/Game/Cutscene/CutsceneScreen/WB_CutsceneScreen.On Crose` _output_get (delegate `StopAudio`))))))

(event `StopAudio`
  (`SynthComponent.Stop` (`self.MediaSound`))
  (`KismetSystemLibrary.PrintString` "piriquita")
  (`SynthComponent.Stop` (`self.MediaSound`)))

(fn `UserConstructionScript`)