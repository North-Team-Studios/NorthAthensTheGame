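; Actor component that manages health, healing, damage and death for its owner.
; TakeDamage reads a DamageInfo struct and branches through CanBeDamage into block, damage or no-damage paths, based on death, invincibility and blocking.
; OnBlocked, OnDeath and OnDamageRespone dispatchers report the outcomes, with damage responses firing only when interruptible or forced.
; Heal clamps Health to MaxHealth and is ignored once dead.
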(event `self.ReceiveBeginPlay`)

(event `self.ReceiveTick`
  (params (DeltaSeconds :type "Float (single-precision)")))

(fn `Heal`
  (params (Amount :type "Float (double-precision)"))
  (returns (NewHealth :type "Float (double-precision)"))
  (if (not (`self.IsDead`))
    (bind _output_get (set `self.Health` (`KismetMathLibrary.FClamp` (+ Amount (`self.Health`)) 0.0 (`self.MaxHealth`))))
    (return _output_get)))

(fn `TakeDamage`
  (params (DamageInfo :type "/Game/DamageSystem/S_DamageInfo Structure"))
  (returns (WasDamaged :type Boolean))
  (bind (_amount _damagetype _damageresponse _shoulddamageinvicible _canbeblocked _canbeparried _shouldforceinterrupt) (break `/Game/DamageSystem/S_DamageInfo` DamageInfo))
  (`self.CanBeDamage` _shoulddamageinvicible _canbeblocked
    (:`BlockDamage`
      (`self.OnBlocked` _canbeparried)
      (return false))
    (:`DoDamage`
      (bind _output_get (set `self.Health` (- (`self.Health`) _amount)))
      (if (<= _output_get 0.0)
        (`self.OnDeath`)
        (set `self.IsDead` true)
        (return true)
        (elif (or (`self.IsInterruptible`) _shouldforceinterrupt)
          (`self.OnDamageRespone` _damageresponse)
          (return true))))
    (:`noDamage`
      (return false))))