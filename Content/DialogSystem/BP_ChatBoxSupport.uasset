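; BP_ChatBoxSupport is a trigger Blueprint in the dialog system that shows a text popup on screen.
; The first begin overlap on BoxActivate creates a WB_PopText widget, fills it from the Text variable and adds it to the viewport.
; The first end overlap removes the widget, as does a long timed delay.
; DoOnce gates make each overlap response single-use, with no check on the overlapping actor.
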(event `self.BoxActivate.OnComponentBeginOverlap`
  (params (OverlappedComponent :type "PrimitiveComponent Object Reference") (OtherActor :type "Actor Object Reference") (OtherComp :type "PrimitiveComponent Object Reference") (OtherBodyIndex :type Integer) (bFromSweep :type Boolean) (SweepResult :type "HitResult Structure (by ref)"))
  (bind _widget (`self.Widget`))
  (`/Engine/EditorBlueprintResources/StandardMacros.DoOnce` false
    (:`Completed`
      (bind _returnvalue (`|CreateWidget` "/Game/Layout/HUD/Content/WB_PopText.WB_PopText_C"))
      (bind _output_get (set `self.Widget` _returnvalue))
      (set `/Game/Layout/HUD/Content/WB_PopText.Main_ext` (`self.Text`) _output_get)
      (`UserWidget.AddToViewport` _widget 0)
      (`KismetSystemLibrary.Delay` 50.0)
      (`Widget.RemoveFromParent` _widget))))

(event `self.BoxActivate.OnComponentEndOverlap`
  (params (OverlappedComponent :type "PrimitiveComponent Object Reference") (OtherActor :type "Actor Object Reference") (OtherComp :type "PrimitiveComponent Object Reference") (OtherBodyIndex :type Integer))
  (`/Engine/EditorBlueprintResources/StandardMacros.DoOnce` false
    (:`Completed`
      (`Widget.RemoveFromParent` (`self.Widget`)))))

(fn `UserConstructionScript`)