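; NPC Blueprint that shows its dialogue one line at a time in a WB_DialogueBox widget.
; Each Talk event reuses or creates the box, fills in line and character name, then advances TalkIndex.
; IdleChat or end of dialogue removes the box and resets the index.
; That branch also creates an unused widget and clears UITalkBox before writing DiscardChat to it, so that text cannot display.
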(event `self.Talk`
  (bind _ui_talkbox (`self.UI TalkBox`))
  (bind _ui_talkbox_2 (`self.UI TalkBox`))
  (bind _dialogue (`self.Dialogue`))
  (if (`self.IdleChat?`)
    (`Widget.RemoveFromParent` (`self.UI TalkBox`) :!label _label)
    (set `self.TalkIndex` 0)
    (`|CreateWidget` "/Game/DialogSystem/WB_DialogueBox.WB_DialogueBox_C" (`GameplayStatics.GetPlayerController` 0))
    (set `self.UI TalkBox` null)
    (`TextBlock.SetText` (`/Game/DialogSystem/WB_DialogueBox.TalkText` _ui_talkbox_2) (`KismetTextLibrary.Conv_StringToText` (`self.DiscardChat`)))
    (`TextBlock.SetText` (`/Game/DialogSystem/WB_DialogueBox.TalkTextCharName` _ui_talkbox_2) (`KismetTextLibrary.Conv_StringToText` (`self.CharName`)))
    (elif (< (`self.TalkIndex`) (`KismetArrayLibrary.Array_Length` _dialogue))
      (`self.UI TalkBox`
        (:`then`
          _)
        (:`else`
          (bind _returnvalue (`|CreateWidget` "/Game/DialogSystem/WB_DialogueBox.WB_DialogueBox_C" (`GameplayStatics.GetPlayerController` 0)))
          (set `self.UI TalkBox` _returnvalue)))
      (`TextBlock.SetText` (`/Game/DialogSystem/WB_DialogueBox.TalkText` _ui_talkbox) (`KismetTextLibrary.Conv_StringToText` (`|GetArrayItem` _dialogue (`self.TalkIndex`))))
      (`TextBlock.SetText` (`/Game/DialogSystem/WB_DialogueBox.TalkTextCharName` _ui_talkbox) (`KismetTextLibrary.Conv_StringToText` (`self.CharName`)))
      (`UserWidget.AddToViewport` (`self.UI TalkBox`) 0)
      (`/Engine/EditorBlueprintResources/StandardMacros.IncrementInt` (`self.TalkIndex`))
      (else
        (goto _label)))))

(fn `UserConstructionScript`)