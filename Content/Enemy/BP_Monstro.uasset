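; BP_Monstro is a zombie enemy character that attacks the player and awards score when killed.
; Health, healing and damage calls forward to BPCDamageSystem, whose callbacks are bound in the construction script for death, blocks and hit reactions.
; Attack plays a montage and, on a notify, damages the player if their PlayerHit flag is set.
; Death ragdolls the mesh, then removes capsule and mesh after delays; IA_Move movement input is also handled.
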(event `Attack`
  (bind _jogador (`self.Jogador`))
  ;[1 1 1] Comment
  (bind _notifyname (`|PlayMontage` (`self.Mesh`) "/Game/Characters/Enemy/Animations/RTG_Unreal/Zombie/AM_Attack.AM_Attack" 2.0)
    (:`OnCompleted`
      (`self.OnAttackEnd` :!label _label))
    (:`OnInterrupted`
      (goto _label))
    (:`OnNotifyBegin`
      (switch `name` _notifyname
        (:`test`
          (if (`/Game/Characters/Jogador/Blueprint/BP_Jogador.PlayerHit` _jogador)
            (message `/Game/DamageSystem/BPI_Damagable.TakeDamage` _jogador (make `/Game/DamageSystem/S_DamageInfo` (`self.Damage`) "NewEnumerator1" "NewEnumerator1" false false true))
            (set `/Game/Characters/Jogador/Blueprint/BP_Jogador.PlayerHit` false (`self.Jogador`))
            (goto _label)))))))

(event `self.ReceiveBeginPlay`
  (bind _asbp_jogador (cast `/Game/Characters/Jogador/Blueprint/BP_Jogador` (`GameplayStatics.GetPlayerPawn` 0)))
  (set `self.Jogador` _asbp_jogador))

(event `EnhancedInput|/Game/ThirdPerson/Input/Actions/IA_Move`
  (params (ActionValue :type "Vector2D Structure") (ElapsedSeconds :type "Float (double-precision)") (TriggeredSeconds :type "Float (double-precision)") (InputAction :type "InputAction Object Reference" :default "/Game/ThirdPerson/Input/Actions/IA_Move.IA_Move"))
  ;[1 1 1] Movement
  (:`Triggered`
    (`self.AddMovementInput` (`self.GetActorRightVector`) ActionValue_X)
    (`self.AddMovementInput` (`self.GetActorForwardVector`) ActionValue_Y)))

(event `Death`
  (bind _mesh (`self.Mesh`))
  (bind _jogador (`self.Jogador`))
  (`PrimitiveComponent.SetSimulatePhysics` _mesh true)
  ;[0.08218 1 0.00757] Jogador Pontua
  (set `/Game/Characters/Jogador/Blueprint/BP_Jogador.Score` (+ (`/Game/Characters/Jogador/Blueprint/BP_Jogador.Score` _jogador) 100) _jogador)
  ;[0.08038 1 0] SFX - Zombie Death Generator
  (`GameplayStatics.PlaySound2D` "/Game/Audio/SFX_Zombies/SFX_Zombie.SFX_Zombie" 0.6 (`KismetMathLibrary.RandomFloatInRange` 0.5 1.0) 0.0 null null)
  (`PrimitiveComponent.SetCollisionEnabled` _mesh "QueryAndPhysics")
  (`KismetSystemLibrary.Delay` 0.2)
  (`ActorComponent.K2_DestroyComponent` (`self.CapsuleComponent`))
  (`KismetSystemLibrary.PrintString` "morreu!!!!!!!]")
  (`KismetSystemLibrary.Delay` 10.0)
  (`ActorComponent.K2_DestroyComponent` (`self.Mesh`)))

(event `Blocked`
  (params (CanBeParried :type Boolean))
  (`KismetSystemLibrary.PrintString` "Blocked"))

(event `DamageResponse`
  (params (DamageResponse :type "/Game/DamageSystem/E_DamageResponse Enum" :default "NewEnumerator0"))
  (bind _mesh (`self.Mesh`))
  (`KismetSystemLibrary.PrintString` (`|GetEnumeratorNameAsString` DamageResponse))
  (switch `/Game/DamageSystem/E_DamageResponse` DamageResponse
    (:`NewEnumerator1`
      (`GameplayStatics.SpawnEmitterAtLocation` "/Game/Realistic_Starter_VFX_Pack_Vol2/Particles/Blood/P_Blood_Splat_Cone.P_Blood_Splat_Cone" (`SceneComponent.K2_GetComponentLocation` _mesh) (`SceneComponent.K2_GetComponentRotation` _mesh) (2.0 2.0 2.0) true "AutoRelease")
      (`MovementComponent.StopMovementImmediately` (`self.CharacterMovement`))
      (`self.PlayAnimMontage` "/Game/Enemy/Animations/AnimMontage/AM_Zombie_Reaction_Hit.AM_Zombie_Reaction_Hit"))))

(fn `GetCurrentHealth`
  (returns (Health :type "Float (double-precision)"))
  (return (`/Game/DamageSystem/BPC_DamageSystem.Health` (`self.BPC_DamageSystem`))))

(fn `GetMaxHealth`
  (returns (MaxHealth :type "Float (double-precision)"))
  (return (`/Game/DamageSystem/BPC_DamageSystem.MaxHealth` (`self.BPC_DamageSystem`))))

(fn `Heal`
  (params (Amount :type "Float (double-precision)"))
  (returns (NewHealth :type "Float (double-precision)"))
  (bind _newhealth (`/Game/DamageSystem/BPC_DamageSystem.Heal` (`self.BPC_DamageSystem`) Amount))
  (return _newhealth))

(fn `TakeDamage`
  (params (DamageInfo :type "/Game/DamageSystem/S_DamageInfo Structure"))
  (returns (WasDamaged :type Boolean))
  (bind _wasdamaged (`/Game/DamageSystem/BPC_DamageSystem.TakeDamage` (`self.BPC_DamageSystem`) DamageInfo))
  (return _wasdamaged))

(fn `UserConstructionScript`
  (bind _bpc_damagesystem (`self.BPC_DamageSystem`))
  (add `/Game/DamageSystem/BPC_DamageSystem.OnDeath` _bpc_damagesystem (`|CreateDelegate` :!event `Death`))
  (add `/Game/DamageSystem/BPC_DamageSystem.OnBlocked` _bpc_damagesystem (`|CreateDelegate` :!event `Blocked`))
  (add `/Game/DamageSystem/BPC_DamageSystem.OnDamageRespone` _bpc_damagesystem (`|CreateDelegate` :!event `DamageResponse`)))