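; BP_Zumbi is a zombie enemy Blueprint built on a damage system component, with reactions that are still debug prints.
; The Construction Script binds the component's death, blocked and damage response delegates to those prints.
; A left mouse input runs a debug-drawn pawn sphere trace, sends damage by interface message and spawns an explosion on success.
; The trace end multiplies a fixed forward vector by actor location instead of offsetting from it.
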(event `Death`
  (`KismetSystemLibrary.PrintString` "Death"))

(event `Blocked`
  (params (CanBeParrie :type Boolean))
  (`KismetSystemLibrary.PrintString` "Blocked"))

(event `DamageResponse`
  (params (DamageResponse :type Byte :default 0))
  (`KismetSystemLibrary.PrintString` (`|GetEnumeratorNameAsString` DamageResponse)))

(event `EnhancedInput|/Game/_Mechanics/Input/Actions/IA_LeftMouse`
  (params (ActionValue :type Boolean) (ElapsedSeconds :type "Float (double-precision)") (TriggeredSeconds :type "Float (double-precision)") (InputAction :type "InputAction Object Reference" :default "/Game/_Mechanics/Input/Actions/IA_LeftMouse.IA_LeftMouse"))
  (bind _returnvalue (`self.K2_GetActorLocation`))
  (:`Triggered`
    (bind (_outhit _returnvalue_2) (`KismetSystemLibrary.SphereTraceSingleForObjects` :`Start` _returnvalue :`End` (* (* (`KismetMathLibrary.GetForwardVector` (struct)) 100.0) _returnvalue) :`Radius` 20.0 :`ObjectTypes` (`|MakeArray` "ObjectTypeQuery3" :!type "EObjectTypeQuery Enum") :`DrawDebugType` "ForDuration" :`DrawTime` 1.0))
    (if _returnvalue_2
      (bind (_bblockinghit _binitialoverlap _time _distance _location _impactpoint _normal _impactnormal _physmat _hitactor) (`GameplayStatics.BreakHitResult` _outhit))
      (bind _wasdamaged (message `/Game/Enemy/BP_Zumbi.TakeDamage` _hitactor (make `` 10.0 0 0)))
      (if _wasdamaged
        (`GameplayStatics.SpawnEmitterAtLocation` "/Game/StarterContent/Particles/P_Explosion.P_Explosion" _location)))))

(fn `UserConstructionScript`
  (bind _bpc_damagesystem (`self.BPC_DamageSystem`))
  (add `self.OnDeath` _bpc_damagesystem (`|CreateDelegate` :!event `Death`))
  (add `self.OnBlocked` _bpc_damagesystem (`|CreateDelegate` :!event `Blocked`))
  (add `self.OnDamageRespone` _bpc_damagesystem (`|CreateDelegate` :!event `DamageResponse`)))