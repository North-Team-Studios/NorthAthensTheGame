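; Enemy spawner Blueprint that creates an AI pawn of a configurable class at its own location.
; The AddEnemy event does the spawn from PawnClass and the root component's world position; nothing runs on BeginPlay, overlap or Tick.
; Health, damage, patrol route and movement speed functions are stubs returning empty or default values, and a damage-response binding in the construction script is never executed.
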(event `AddEnemy`
  (`AIBlueprintHelperLibrary.SpawnAIFromClass` (`self.Pawn Class`) null (`SceneComponent.K2_GetComponentLocation` (`self.RootComponent`)) (struct) false null))

(fn `GetCurrentHealth`
  (returns (Health :type "Float (double-precision)"))
  (return 0.0))

(fn `GetMaxHealth`
  (returns (MaxHealth :type "Float (double-precision)"))
  (return 0.0))

(fn `GetPatrolRoute`
  (returns (PatrolRoute :type "/Game/Enemy/Ai/BP_PatrolRoutes Object Reference"))
  (return null))

(fn `Heal`
  (params (Amount :type "Float (double-precision)"))
  (returns (NewHealth :type "Float (double-precision)"))
  (return 0.0))

(fn `SetMovementSpeed`
  (params (Speed :type "/Game/Enemy/Ai/Enums/E_MovementSpeed Enum" :default "NewEnumerator0"))
  (returns (SpeedValue :type "Float (double-precision)"))
  (return 0.0))

(fn `TakeDamage`
  (params (DamageInfo :type "/Game/_Mechanics/DamageSystem/S_DamageInfo Structure"))
  (returns (WasDamaged :type Boolean))
  (return false))

(fn `UserConstructionScript`)