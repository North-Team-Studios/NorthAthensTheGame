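; Spawner actor that places a single BP_BaseEnemy at its own location shortly after play begins.
; BeginPlay sets a non-looping timer that fires SpawnEnemy, which spawns the AI with the BT_Enemy_Base behavior tree and stores it in Spawned.
; Health, damage, patrol route and movement speed functions are empty stubs returning default values.
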(event `SpawnEnemy`
  (bind _returnvalue (`AIBlueprintHelperLibrary.SpawnAIFromClass` "/Game/Enemy/BP_BaseEnemy.BP_BaseEnemy_C" "/Game/Enemy/Ai/BT_Enemy_Base.BT_Enemy_Base" (`self.K2_GetActorLocation`) (struct) false null))
  (set `self.Spawned` _returnvalue))

(event `self.ReceiveBeginPlay`
  (`KismetSystemLibrary.K2_SetTimerDelegate` (delegate `SpawnEnemy`) 2.0))

(fn `GetCurrentHealth`
  (returns (Health :type "Float (double-precision)"))
  (return 0.0))

(fn `GetMaxHealth`
  (returns (MaxHealth :type "Float (double-precision)"))
  (return 0.0))

(fn `GetPatrolRoute`
  (returns (PatrolRoute :type "/Game/Enemy/Ai/BP_PatrolRoutes Object Reference"))
  (return null))

(fn `Heal`
  (params (Amount :type "Float (double-precision)"))
  (returns (NewHealth :type "Float (double-precision)"))
  (return 0.0))

(fn `SetMovementSpeed`
  (params (Speed :type "/Game/Enemy/Ai/Enums/E_MovementSpeed Enum" :default "NewEnumerator0"))
  (returns (SpeedValue :type "Float (double-precision)"))
  (return 0.0))

(fn `TakeDamage`
  (params (DamageInfo :type "/Game/_Mechanics/DamageSystem/S_DamageInfo Structure"))
  (returns (WasDamaged :type Boolean))
  (return false))

(fn `UserConstructionScript`)