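; Zombie enemy character that starts passive when given a patrol route and otherwise attacks the player.
; BPCDamageSystem handles health and drives hit reactions and death, which ragdolls the body and reports the kill to the game mode.
; The attack montage's notify damages the player if their PlayerHit flag is set.
; Movement speeds are randomized per state, and a temporary outlined slow effect blocks speed changes while active.
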(event `self.ReceiveBeginPlay`
  (bind _asaic_enemy_base (cast `/Game/Enemy/Ai/AIC_Enemy_Base` (`AIBlueprintHelperLibrary.GetAIController` self)))
  (set `self.As AIC Enemy Base` _asaic_enemy_base)
  (`self.PatrolRoute`
    (:`then`
      (`/Game/Enemy/Ai/AIC_Enemy_Base.Set StateAsPassive` (`self.As AIC Enemy Base`)))
    (:`else`
      (`/Game/Enemy/Ai/AIC_Enemy_Base.Set StateAsAttacking` (`self.As AIC Enemy Base`) (`/Game/_Mechanics/QuestSystem/BPL_CommonFunctionLibrary.GetMyPlayerCharacter`)))))

(event `Blocked`
  (params (CanBeParried :type Boolean)))

(event `Attack`
  (bind _myplayercharacter (`/Game/_Mechanics/QuestSystem/BPL_CommonFunctionLibrary.GetMyPlayerCharacter`))
  ;[0.1875 0.1875 0.1875] Attack - To Fix
  (bind _notifyname (`|PlayMontage` (`self.Mesh`) "/Game/Characters/Enemy/Animations/RTG_Unreal/Zombie/AM_Attack.AM_Attack" 2.0)
    (:`OnCompleted`
      (`self.OnAttackEnd` :!label _label))
    (:`OnInterrupted`
      (goto _label))
    (:`OnNotifyBegin`
      (switch `name` _notifyname
        (:`test`
          (if (`/Game/Characters/Jogador/Blueprint/BP_Jogador.PlayerHit` _myplayercharacter)
            (message `/Game/_Mechanics/DamageSystem/BPI_Damagable.TakeDamage` _myplayercharacter (make `/Game/_Mechanics/DamageSystem/S_DamageInfo` (`self.Damage`) "NewEnumerator1" "NewEnumerator1" false false true))
            (set `/Game/Characters/Jogador/Blueprint/BP_Jogador.PlayerHit` false (`/Game/_Mechanics/QuestSystem/BPL_CommonFunctionLibrary.GetMyPlayerCharacter`))
            (goto _label)))))))

(event `Death`
  (bind _returnvalue (`GameplayStatics.GetGameMode`))
  (bind _mesh (`self.Mesh`))
  ;[0.2292 0.2292 0.2292] Death
  (bind _asgm_level (cast `/Game/_Maps/GameModes/GM_Level` _returnvalue)
    (:`then`
      (`/Game/_Maps/GameModes/GM_Level.Enemies Killed` _asgm_level))
    (:`CastFailed`
      (bind _asgm_minigame (cast `/Game/_Mechanics/AlternativeMode/GM_Minigame` _returnvalue))
      (`/Game/_Mechanics/AlternativeMode/GM_Minigame.Enemies Killed` _asgm_minigame)))
  (`GameplayStatics.PlaySound2D` "/Game/_Materials/Sounds/Zombie/SFX_Zombie.SFX_Zombie" 0.6 (`KismetMathLibrary.RandomFloatInRange` 0.5 1.0) 0.0 null null)
  (`MeshComponent.SetOverlayMaterial` _mesh null)
  (`PrimitiveComponent.SetSimulatePhysics` _mesh true)
  (`PrimitiveComponent.SetCollisionEnabled` _mesh "PhysicsOnly")
  (`KismetSystemLibrary.Delay` 0.2)
  (`ActorComponent.K2_DestroyComponent` (`self.CapsuleComponent`))
  (`KismetSystemLibrary.Delay` 5.0)
  (`ActorComponent.K2_DestroyComponent` (`self.Mesh`)))

(event `DamageResponse`
  (params (DamageResponse :type "/Game/_Mechanics/DamageSystem/E_DamageResponse Enum" :default "NewEnumerator0"))
  (bind _myplayercharacter (`/Game/_Mechanics/QuestSystem/BPL_CommonFunctionLibrary.GetMyPlayerCharacter`))
  (bind _mesh (`self.Mesh`))
  ;[0.2188 0.2188 0.2188] Enemy Take Damage - Response
  (`AISense_Damage.ReportDamageEvent` self _myplayercharacter 10.0 (`self.K2_GetActorLocation` _myplayercharacter))
  (switch `/Game/_Mechanics/DamageSystem/E_DamageResponse` DamageResponse
    (:`NewEnumerator1`
      (`GameplayStatics.SpawnEmitterAtLocation` "/Game/_Materials/Packs/VFX_Starter_Pack/Particles/Blood/P_Blood_Splat_Cone.P_Blood_Splat_Cone" (`SceneComponent.K2_GetComponentLocation` _mesh) (`SceneComponent.K2_GetComponentRotation` _mesh) (1.0 1.0 1.5) true "AutoRelease")
      (`MovementComponent.StopMovementImmediately` (`self.CharacterMovement`))
      (`self.PlayAnimMontage` "/Game/Enemy/Animations/AnimMontage/AM_Zombie_Reaction_Hit.AM_Zombie_Reaction_Hit"))))

(event `NegativeEffect`
  (bind _mesh (`self.Mesh`))
  (if (not (`self.ActivatedEffect`))
    (message `/Game/Enemy/Ai/BPI_EnemyAI.SetMovementSpeed` self "NewEnumerator1")
    (set `self.ActivatedEffect` true)
    (`MeshComponent.SetOverlayMaterial` (`self.Mesh`) "/Game/_Materials/VFX/VFX_Slow/M_OutlineSlow_Inst.M_OutlineSlow_Inst")
    (`KismetSystemLibrary.Delay` 10.0)
    (message `/Game/Enemy/Ai/BPI_EnemyAI.SetMovementSpeed` self "NewEnumerator2")
    (set `self.ActivatedEffect` false)
    (`/Engine/EditorBlueprintResources/StandardMacros.IsValid` _mesh
      (:`Is Valid`
        (`MeshComponent.SetOverlayMaterial` _mesh null)))))

(fn `GetCurrentHealth`
  (returns (Health :type "Float (double-precision)"))
  (return (`/Game/_Mechanics/DamageSystem/BPC_DamageSystem.Health` (`self.BPC_DamageSystem`))))

(fn `GetMaxHealth`
  (returns (MaxHealth :type "Float (double-precision)"))
  (return (`/Game/_Mechanics/DamageSystem/BPC_DamageSystem.MaxHealth` (`self.BPC_DamageSystem`))))

(fn `GetPatrolRoute`
  (returns (PatrolRoute :type "/Game/Enemy/Ai/BP_PatrolRoutes Object Reference"))
  (return (`self.PatrolRoute`)))

(fn `Heal`
  (params (Amount :type "Float (double-precision)"))
  (returns (NewHealth :type "Float (double-precision)"))
  (bind _newhealth (`/Game/_Mechanics/DamageSystem/BPC_DamageSystem.Heal` (`self.BPC_DamageSystem`) Amount))
  (return _newhealth))

(fn `SetMovementSpeed`
  (params (Speed :type "/Game/Enemy/Ai/Enums/E_MovementSpeed Enum" :default "NewEnumerator0"))
  (returns (SpeedValue :type "Float (double-precision)"))
  (bind _returnvalue (select `/Game/Enemy/Ai/Enums/E_MovementSpeed` Speed :`NewEnumerator1` 50.0 :`NewEnumerator2` 150.0 :`NewEnumerator3` 250.0 :!type "Float (single-precision)"))
  (if (not (`self.ActivatedEffect`))
    (bind _output_get (set `CharacterMovementComponent.MaxWalkSpeed` (`KismetMathLibrary.RandomFloatInRange` (/ _returnvalue 1.2) _returnvalue) (`self.CharacterMovement`)))
    (return _output_get)))

(fn `TakeDamage`
  (params (DamageInfo :type "/Game/_Mechanics/DamageSystem/S_DamageInfo Structure"))
  (returns (WasDamaged :type Boolean))
  (bind _wasdamaged (`/Game/_Mechanics/DamageSystem/BPC_DamageSystem.TakeDamage` (`self.BPC_DamageSystem`) DamageInfo))
  (return _wasdamaged))

(fn `UserConstructionScript`
  (bind _bpc_damagesystem (`self.BPC_DamageSystem`))
  (add `/Game/_Mechanics/DamageSystem/BPC_DamageSystem.OnDeath` _bpc_damagesystem (`|CreateDelegate` :!event `Death`))
  (add `/Game/_Mechanics/DamageSystem/BPC_DamageSystem.OnBlocked` _bpc_damagesystem (`|CreateDelegate` :!event `Blocked`))
  (add `/Game/_Mechanics/DamageSystem/BPC_DamageSystem.OnDamageRespone` _bpc_damagesystem (`|CreateDelegate` :!event `DamageResponse`)))