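; BP_EndGame is a trigger actor that ends the game when the player (BP_Jogador) overlaps its Collision component.
; On overlap it creates the WB_EndGame widget, passes it the player's Score as the final score and adds it to the viewport.
; It then pauses the game, switches input to Game and UI focused on the widget, and shows the mouse cursor.
; An OpenLevel call to "FimDoJogo" is present but never runs.
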(event `self.Collision.OnComponentBeginOverlap`
  (params (OverlappedComponent :type "PrimitiveComponent Object Reference") (OtherActor :type "Actor Object Reference") (OtherComp :type "PrimitiveComponent Object Reference") (OtherBodyIndex :type Integer) (bFromSweep :type Boolean) (SweepResult :type "HitResult Structure (by ref)"))
  (bind _returnvalue (`GameplayStatics.GetPlayerController` 0))
  (bind _asbp_jogador (cast `/Game/Characters/Jogador/Blueprint/BP_Jogador` OtherActor))
  (if (`KismetSystemLibrary.IsValid` _asbp_jogador)
    (bind _returnvalue_2 (`|CreateWidget` "/Game/_Layout/HUD/WB_EndGame.WB_EndGame_C"))
    (bind _output_get (set `self.End Game` _returnvalue_2))
    (set `/Game/_Layout/HUD/WB_EndGame.Final Score` (`/Game/Characters/Jogador/Blueprint/BP_Jogador.Score` _asbp_jogador) _output_get)
    (`UserWidget.AddToViewport` _output_get 0)
    (`GameplayStatics.SetGamePaused` true)
    (`WidgetBlueprintLibrary.SetInputMode_GameAndUIEx` _returnvalue (`self.End Game`))
    (set `PlayerController.bShowMouseCursor` true _returnvalue)))

(fn `UserConstructionScript`)