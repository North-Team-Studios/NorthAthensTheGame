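; Safe Haven table of plants that the player inspects for a scripted monologue on each plant's properties, ending in a plan.
; A box overlap shows prompt widgets while the game instance's table interaction flag allows it.
; Lookat hides them, disables input and plays timed WB_PopDialog balloons through delays and a DoOnce-guarded helper.
; It then restores input, reports the interaction to the game instance and toggles the table off.
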(event `self.ReceiveBeginPlay`
  (bind _asbpi_game_instance (cast `/Game/_Mechanics/SaveGame/BPI_GameInstance` (`GameplayStatics.GetGameInstance`)))
  (set `self.As BPI Game Instance` _asbpi_game_instance))

(event `self.ReceiveTick`
  (params (DeltaSeconds :type "Float (single-precision)")))

(event `self.Box.OnComponentBeginOverlap`
  (params (OverlappedComponent :type "PrimitiveComponent Object Reference") (OtherActor :type "Actor Object Reference") (OtherComp :type "PrimitiveComponent Object Reference") (OtherBodyIndex :type Integer) (bFromSweep :type Boolean) (SweepResult :type "HitResult Structure (by ref)"))
  (bind _toggle_table (`/Game/_Mechanics/SaveGame/BPI_GameInstance.ToggleTableInteraction` (`self.As BPI Game Instance`)))
  (if _toggle_table
    (if (== OtherActor (`GameplayStatics.GetPlayerCharacter` 0))
      (`SceneComponent.SetVisibility` (`self.Widget`) true false)
      (`SceneComponent.SetVisibility` (`self.Dohere`) true false))))

(event `self.Box.OnComponentEndOverlap`
  (params (OverlappedComponent :type "PrimitiveComponent Object Reference") (OtherActor :type "Actor Object Reference") (OtherComp :type "PrimitiveComponent Object Reference") (OtherBodyIndex :type Integer))
  (`SceneComponent.SetVisibility` (`self.Widget`) false false))

(event `/Game/_Mechanics/BPI_MainInteract.LookAt`
  (bind _returnvalue (`GameplayStatics.GetPlayerController` 0))
  (bind _as_bpi_game_instance (`self.As BPI Game Instance`))
  (bind _returnvalue_2 (`Controller.K2_GetPawn` _returnvalue))
  (bind _toggle_table (`/Game/_Mechanics/SaveGame/BPI_GameInstance.ToggleTableInteraction` (`self.As BPI Game Instance`)))
  (if _toggle_table
    (`SceneComponent.SetVisibility` (`self.Widget`) false false)
    (`SceneComponent.SetVisibility` (`self.DoHere`) false false)
    (`self.DisableInput` _returnvalue_2 _returnvalue)
    (`self.AddDialogue` "There are four plants in the table." 3.0)
    (`KismetSystemLibrary.Delay` 3.2)
    (`self.AddDialogue` "The first one, NOMEDAPLANTA1, has healing properties." 3.0)
    (`KismetSystemLibrary.Delay` 3.2)
    (`self.AddDialogue` "You feel better standing next to it." 3.0)
    (`KismetSystemLibrary.Delay` 3.2)
    (`self.AddDialogue` "The second one, NOMEDAPLANTA2, has dangerous properties." 3.0)
    (`KismetSystemLibrary.Delay` 3.2)
    (`self.AddDialogue` "Its leaves has oxalate crystals that cause a lot of damage." 3.0)
    (`KismetSystemLibrary.Delay` 3.2)
    (`self.AddDialogue` "The third one, NOMEDAPLANTA3, has restrictive properties." 3.0)
    (`KismetSystemLibrary.Delay` 3.2)
    (`self.AddDialogue` "It can make everything around it slower." 3.0)
    (`KismetSystemLibrary.Delay` 3.2)
    (`self.AddDialogue` "The last one is unknown to me." 3.0)
    (`KismetSystemLibrary.Delay` 3.2)
    (`self.AddDialogue` "It resembles the giant tree in the Haven. You come up with a plan." 3.0)
    (`KismetSystemLibrary.Delay` 3.2)
    (`self.EnableInput` _returnvalue_2 _returnvalue)
    (`/Game/_Mechanics/SaveGame/BPI_GameInstance.TableInteract` _as_bpi_game_instance)
    (`/Game/_Mechanics/SaveGame/BPI_GameInstance.Toggle Table` _as_bpi_game_instance false)))

(event `AddDialogue`
  (params (Text :type Text) (`Duration of Balloon` :type "Float (double-precision)"))
  (`/Engine/EditorBlueprintResources/StandardMacros.DoOnce` false :!label _label
    (:`Completed`
      (bind _returnvalue (`|CreateWidget` "/Game/_Layout/HUD/Content/WB_PopDialog.WB_PopDialog_C" null Text))
      (`UserWidget.AddToViewport` _returnvalue 0)
      (`KismetSystemLibrary.Delay` `Duration of Balloon`)
      (`Widget.RemoveFromParent` _returnvalue)
      (goto _label :!via `Reset`))))

(fn `Interact With`
  (returns (ObjectiveID :type String))
  (return ""))

(fn `UserConstructionScript`)