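; Double door prop for the police station (Delegacia), with two animated leaves, a frame and interaction widgets.
; Its proximity open/close logic, which plays leaf animations and toggles frame collision for the player, is disconnected, so the Box overlap events do nothing.
; SwitchWidget swaps visibility between the progress and pop-up interaction widgets, but its only call here sits in that unreachable logic.
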(event `self.Box.OnComponentBeginOverlap`
  (params (OverlappedComponent :type "PrimitiveComponent Object Reference") (OtherActor :type "Actor Object Reference") (OtherComp :type "PrimitiveComponent Object Reference") (OtherBodyIndex :type Integer) (bFromSweep :type Boolean) (SweepResult :type "HitResult Structure (by ref)")))

(event `self.Box.OnComponentEndOverlap`
  (params (OverlappedComponent :type "PrimitiveComponent Object Reference") (OtherActor :type "Actor Object Reference") (OtherComp :type "PrimitiveComponent Object Reference") (OtherBodyIndex :type Integer)))

(fn `SwitchWidget`
  (params (`Repair?` :type Boolean))
  (if `Repair?`
    (`SceneComponent.SetVisibility` (`self.Progress_Interaction`) true false)
    (`SceneComponent.SetVisibility` (`self.PopUp_Interaction`) false false)
    (else
      (`SceneComponent.SetVisibility` (`self.Progress_Interaction`) false false)
      (`SceneComponent.SetVisibility` (`self.PopUp_Interaction`) true false))))

(fn `UserConstructionScript`)