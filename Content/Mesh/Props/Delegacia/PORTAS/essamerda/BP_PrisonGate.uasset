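; BP_PrisonGate is a key-locked prison gate the player opens through a look-at interaction.
; A box overlap shows the prompt and allows interaction, and PickUpKey sets the flag that Lookat checks.
; With the key, the gate animates open, plays a sound, shows an "opened" popup and calls ShowRoom on a valid ORM reference.
; Without it, a DoOnce-guarded bang sound and timed "Locked" warning naming the key play.
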(event `self.ReceiveBeginPlay`
  (bind _returnvalue (`|CreateWidget` "/Game/_Mechanics/InventorySystem/DoorLockSystem/WB_DoorPopText.WB_DoorPopText_C" null "You opened: " (`self.Room Reference`)))
  (set `self.DoorPopUp` _returnvalue)
  (bind _returnvalue_2 (`|CreateWidget` "/Game/_Mechanics/InventorySystem/DoorLockSystem/WB_DoorPopText.WB_DoorPopText_C" null "Locked. Label says:" (`self.Room Reference`) "NewEnumerator1"))
  (set `self.Warning Pop Up` _returnvalue_2))

(event `self.Box.OnComponentBeginOverlap`
  (params (OverlappedComponent :type "PrimitiveComponent Object Reference") (OtherActor :type "Actor Object Reference") (OtherComp :type "PrimitiveComponent Object Reference") (OtherBodyIndex :type Integer) (bFromSweep :type Boolean) (SweepResult :type "HitResult Structure (by ref)"))
  (if (and (== OtherActor (`/Game/_Mechanics/QuestSystem/BPL_CommonFunctionLibrary.GetMyPlayerCharacter`)) (not (`self.isOpen?`)))
    (`SceneComponent.SetVisibility` (`self.PopUp_Interaction`) true false)
    (set `self.InteractAllowed?` true)))

(event `self.Box.OnComponentEndOverlap`
  (params (OverlappedComponent :type "PrimitiveComponent Object Reference") (OtherActor :type "Actor Object Reference") (OtherComp :type "PrimitiveComponent Object Reference") (OtherBodyIndex :type Integer))
  (if (== OtherActor (`/Game/_Mechanics/QuestSystem/BPL_CommonFunctionLibrary.GetMyPlayerCharacter`))
    (`SceneComponent.SetVisibility` (`self.PopUp_Interaction`) false false)
    (set `self.InteractAllowed?` false)))

(event `self.LookAt`
  (bind _warning_pop_up (`self.Warning Pop Up`))
  (bind _orm (`self.ORM`))
  (if (`self.isOpen?`)
    _
    (elif (`self.InteractAllowed?`)
      (if (`self.Has Key?`)
        (`GameplayStatics.PlaySound2D` "/Game/_Materials/Sounds/Effects/SFX_OpenDoor.SFX_OpenDoor" 1.0 1.0 0.0 null null)
        (set `self.isOpen?` true)
        (`SkeletalMeshComponent.PlayAnimation` (`self.door_anim`) "/Game/Mesh/Props/Delegacia/PORTAS/PortasMetal/portas_prisao_Anim.portas_prisao_Anim" false)
        (`SceneComponent.SetVisibility` (`self.PopUp_Interaction`) false false)
        (`self.ShowMessage`)
        (`/Engine/EditorBlueprintResources/StandardMacros.IsValid` _orm
          (:`Is Valid`
            (`/Game/_Mechanics/InventorySystem/DoorLockSystem/BPI_DoorLockSystem.ShowRoom` _orm)
            (set `self.InteractAllowed?` false)))
        (else
          (`/Engine/EditorBlueprintResources/StandardMacros.DoOnce` false :!label _label
            (:`Completed`
              (`GameplayStatics.PlaySound2D` "/Game/_Materials/Sounds/Effects/SFX_DoorBang.SFX_DoorBang" 1.0 1.0 0.0 null null)
              (`UserWidget.AddToViewport` _warning_pop_up 0)
              (`KismetSystemLibrary.Delay` 2.0)
              (`Widget.RemoveFromParent` _warning_pop_up)
              (goto _label :!via `Reset`))))))))

(event `self.PickUpKey`
  (set `self.Has Key?` true))

(event `ShowMessage`
  (bind _doorpopup (`self.DoorPopUp`))
  (`UserWidget.AddToViewport` _doorpopup 0)
  (`KismetSystemLibrary.Delay` 3.0)
  (`Widget.RemoveFromParent` _doorpopup))

(fn `Interact With`
  (returns (ObjectiveID :type String))
  (return ""))

(fn `SwitchWidget`
  (params (`Repair?` :type Boolean))
  (if `Repair?`
    (`SceneComponent.SetVisibility` (`self.PopUp_Interaction`) false false)
    (else
      (`SceneComponent.SetVisibility` (`self.PopUp_Interaction`) true false))))

(fn `UserConstructionScript`)