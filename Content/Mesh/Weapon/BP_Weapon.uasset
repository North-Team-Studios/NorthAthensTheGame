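; Weapon actor that fires BP_Tiro projectiles for the player character and tracks ammo.
; Shoot decrements ammo and spawns a projectile at the Arrow, feeding only the roll of the camera's forward rotation into its transform.
; The projectile's impact event applies fixed damage and spawns the muzzle flash, both using a Hit variable this file never sets.
; Reload refills ammo, but the empty-ammo check that calls it is disconnected.
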(event `self.ReceiveBeginPlay`
  (set `self.Current Ammo` (`self.MaxAmmo`))
  (bind _asbp_jogador (cast `/Game/Characters/Jogador/Blueprint/BP_Jogador` (`GameplayStatics.GetPlayerCharacter` 0)))
  (set `self.Jogador` _asbp_jogador))

(event `Shoot`
  (bind _returnvalue_roll (`KismetMathLibrary.BreakRotator` (`KismetMathLibrary.Conv_VectorToRotator` (`SceneComponent.GetForwardVector` (`/Game/Characters/Jogador/Blueprint/BP_Jogador.MainCamera` (`self.Jogador`))))))
  (`self.MenosUmTiro`)
  (bind _returnvalue (`|SpawnActorFromClass` "/Game/Weapons/BP_Tiro.BP_Tiro_C" (`KismetMathLibrary.MakeTransform` (`SceneComponent.K2_GetComponentLocation` (`self.Arrow`)) (`KismetMathLibrary.MakeRotator` _returnvalue_roll)) "Undefined" "MultiplyWithRoot" self (`self.WeaponVellocity`) 0.0 null (`GameplayStatics.GetPlayerCharacter` 0)))
  (add `/Game/Weapons/BP_BaseProjectile.OnProjectileImpact` _returnvalue (delegate `Projectile Impact`))
  (`PrimitiveComponent.IgnoreActorWhenMoving` (`self.Weapon`) null false))

(event `Projectile Impact`
  (params (`Other Actror` :type "Actor Object Reference") (Hit :type "HitResult Structure"))
  (message `/Game/DamageSystem/BPI_Damagable.TakeDamage` Hit_HitActor (make `/Game/DamageSystem/S_DamageInfo` 10.0 (`self.Damage Type`) "NewEnumerator1"))
  (`GameplayStatics.SpawnEmitterAtLocation` (`self.Muzzle Flash`) Hit_TraceStart))

(fn `IsAmmo?`
  (returns (IsAmmo :type Boolean))
  (bind _returnvalue (!= (`self.Current Ammo`) 0))
  (`KismetSystemLibrary.PrintString` (`KismetStringLibrary.Conv_BoolToString` _returnvalue))
  (return _returnvalue))

(fn `MenosUmTiro`
  (set `self.Current Ammo` (- (`self.Current Ammo`) 1)))

(fn `Reload`
  (set `self.Current Ammo` (`self.MaxAmmo`)))

(fn `UserConstructionScript`)