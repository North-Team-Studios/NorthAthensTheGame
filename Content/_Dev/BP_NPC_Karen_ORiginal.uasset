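; BP_NPC_Karen_ORiginal is a dev-folder Blueprint for the NPC Karen, who offers dialogue and quest interaction.
; Interact stores the instigator and opens a conversation through the Karen dialogue component.
; That component's NewQuest event calls InteractWith on the quest-giver component and caches the returned objective ID.
; The actor's own InteractWith returns that cached ID, while a separate NewQuest function returns the quest-giver's result directly.
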(event `self.Interact`
  (params (Instigator :type "Actor Object Reference"))
  (set `self.InteractInstigator` Instigator)
  (`/Game/_Mechanics/DialogueSystem/BPC_DialogueBase.OpenConversation` (`self.BPC_KarenDialogue`)))

(event `self.BPC_KarenDialogue.NewQuest`
  (bind _objectiveid (`/Game/_Mechanics/QuestSystem/BPC_QuestGiven.Interact With` (`self.BPC_QuestGiven`)))
  (set `self.Objective ID Local` _objectiveid))

(fn `Interact With`
  (returns (ObjectiveID :type String))
  (return (`self.Objective ID Local`)))

(fn `NewQuest`
  (returns (ObjectiveID :type String))
  (bind _objectiveid (`/Game/_Mechanics/BPI_MainInteract.Interact With` (`self.BPC_QuestGiven`)))
  (return _objectiveid))

(fn `UserConstructionScript`
  (`parent.UserConstructionScript`))