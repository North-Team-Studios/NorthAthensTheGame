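; BP_NPC is a dialogue NPC that shows its lines and character name in a talk box widget.
; Each Talk call displays the next Dialogue entry via TalkIndex, creating the widget when the UITalkBox reference is invalid.
; A call after the last line closes the box and sets IsConversationOver.
; Later calls use a FlipFlop to alternately show the ConversationOver line and remove the box.
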(event `self.Talk`
  (bind (_ui_talkbox _ui_talkbox_2) (`self.UI TalkBox`))
  (bind _dialogue (`self.Dialogue`))
  (if (`self.IsConversationOver?`)
    (`/Engine/EditorBlueprintResources/StandardMacros.FlipFlop`
      (:`A`
        (`self.UI TalkBox`
          (:`then`
            _)
          (:`else`
            (bind _returnvalue (`|CreateWidget` null (`GameplayStatics.GetPlayerController` 0)))
            (set `self.UI TalkBox` null _returnvalue)))
        (`TextBlock.SetText` (`/Game/_Dev/DialogSystem/BP_NPC.TalkText` _ui_talkbox_2) (`KismetTextLibrary.Conv_StringToText` (`self.ConversationOver`)))
        (`TextBlock.SetText` (`/Game/_Dev/DialogSystem/BP_NPC.TalkTextCharName` _ui_talkbox_2) (`KismetTextLibrary.Conv_StringToText` (`self.CharName`)))
        (`UserWidget.AddToViewport` (`.UI TalkBox` (`self.UI TalkBox`)) 0))
      (:`B`
        (`Widget.RemoveFromParent` (`.UI TalkBox` (`self.UI TalkBox`)))))
    (elif (< (`self.TalkIndex`) (`KismetArrayLibrary.Array_Length` _dialogue))
      (`self.UI TalkBox`
        (:`then`
          _)
        (:`else`
          (bind _returnvalue_2 (`|CreateWidget` null (`GameplayStatics.GetPlayerController` 0)))
          (bind (_output_get _output_get_2) (set `self.UI TalkBox` null _returnvalue_2))))
      (`TextBlock.SetText` (`/Game/_Dev/DialogSystem/BP_NPC.TalkText` _output_get_2) (`KismetTextLibrary.Conv_StringToText` (`|GetArrayItem` _dialogue (`self.TalkIndex`))))
      (`TextBlock.SetText` (`/Game/_Dev/DialogSystem/BP_NPC.TalkTextCharName` _output_get_2) (`KismetTextLibrary.Conv_StringToText` (`self.CharName`)))
      (`UserWidget.AddToViewport` (`.UI TalkBox` (`self.UI TalkBox`)) 0)
      (`/Engine/EditorBlueprintResources/StandardMacros.IncrementInt` (`self.TalkIndex`))
      (else
        (`Widget.RemoveFromParent` (`.UI TalkBox` (`self.UI TalkBox`)))
        (set `self.IsConversationOver?` true)))))

(fn `UserConstructionScript`)