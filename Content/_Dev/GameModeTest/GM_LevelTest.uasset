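; Test level game mode that holds a stage countdown timer and sets up the player on start.
; BeginPlay resets the countdown to the max stage time, saves the current level through the game instance, then enables the player's weapon and switches their camera.
; StartCountdow lowers the timer by delta time per call, clamped at zero, and GetCountdown exposes it; neither is called within this graph.
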(event `self.ReceiveBeginPlay`
  (set `self.Countdown` (`self.MaxStageTime`))
  (bind _asbpi_game_instance (cast `/Game/_Mechanics/SaveGame/BPI_GameInstance` (`GameplayStatics.GetGameInstance`)))
  (`/Game/_Mechanics/SaveGame/BPI_GameInstance.Save Current Level` _asbpi_game_instance)
  (bind _asbp_jogador_teste (cast `/Game/_Dev/ClideTest/BP_Jogador_Teste` (`GameplayStatics.GetPlayerPawn` 0)))
  (bind _output_get (set `/Game/_Dev/ClideTest/BP_Jogador_Teste.AllowWeapon?` true _asbp_jogador_teste))
  (`/Game/_Dev/ClideTest/BP_Jogador_Teste.Switch Camera` _asbp_jogador_teste _output_get))

(fn `GetCountdown`
  (returns (Countdown :type "Float (double-precision)"))
  (return (`self.Countdown`)))

(fn `StartCountdow`
  (set `self.Countdown` (`KismetMathLibrary.FClamp` (- (`self.Countdown`) (`GameplayStatics.GetWorldDeltaSeconds`)) 0.0 (`self.MaxStageTime`))))

(fn `UserConstructionScript`)