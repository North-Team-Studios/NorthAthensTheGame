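; Two-leaf gate that opens once the level's unlock condition is met, triggering enemies at its target points.
; It polls GM_Level's UnlockCondition with its OpenCondition on Tick, then fires once to animate, play a collapse sound and call AddEnemy on each TargetPoint.
; A timeline rotates both leaves (LadoDireito, LadoEsquerdo) open and disables their collision.
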(event `self.ReceiveBeginPlay`
  (bind _asgm_level (cast `/Game/_Maps/GameModes/GM_Level` (`GameplayStatics.GetGameMode`)))
  (set `self.As GM Level` _asgm_level))

(event `self.ReceiveTick`
  (params (DeltaSeconds :type "Float (single-precision)"))
  (bind _enable (`/Game/_Maps/GameModes/GM_Level.Unlock Condition` (`self.As GM Level`) (`self.Open Condition`)))
  (if _enable
    (`/Engine/EditorBlueprintResources/StandardMacros.DoOnce` false
      (:`Completed`
        (`self.PlayOpenAnimation`)
        (`GameplayStatics.PlaySoundAtLocation` "/Game/StarterContent/Audio/Collapse_Cue.Collapse_Cue" (`SceneComponent.K2_GetComponentLocation` (`self.DefaultSceneRoot`)) (struct) 1.0 1.0 0.0 null null null null)
        (for _array_element (`self.TargetPoints`)
          (`/Game/Enemy/Spawn/BP_SpawnEnemy.AddEnemy` _array_element))))))

(event `PlayOpenAnimation`
  (bind _ladoesquerdo (`self.LadoEsquerdo`))
  (`/Engine/EditorBlueprintResources/StandardMacros.DoOnce` false
    (:`Completed`
      (bind (_direction _dooropening) (`Timeline|Timeline`)
        (:`Update`
          (bind _returnvalue (`KismetMathLibrary.Lerp` 0.0 90.0 _dooropening))
          (`SceneComponent.K2_SetRelativeRotation` (`self.LadoDireito`) (`KismetMathLibrary.MakeRotator` -12.0 _returnvalue) false false)
          (`SceneComponent.K2_SetRelativeRotation` _ladoesquerdo (`KismetMathLibrary.MakeRotator` 35.0 _returnvalue) false false)
          (`PrimitiveComponent.SetCollisionEnabled` _ladoesquerdo "NoCollision")
          (`PrimitiveComponent.SetCollisionEnabled` (`self.LadoDireito`) "NoCollision"))))))

(fn `UserConstructionScript`)