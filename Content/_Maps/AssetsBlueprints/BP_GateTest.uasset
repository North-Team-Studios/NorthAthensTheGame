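; BP_GateTest is a two-panel gate that opens when the level's unlock condition for it is met.
; Every Tick it asks GM_Level to evaluate its OpenCondition, then, guarded by DoOnce, triggers the opening and a 2D creature-stretch sound.
; A timeline slides LadoDireito and LadoEsquerdo apart along relative Y, with no closing logic.
; Leftover electricity-based Box collision logic is disconnected and never runs.
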(event `self.ReceiveTick`
  (params (DeltaSeconds :type "Float (single-precision)"))
  (bind _asgm_level (cast `/Game/_Maps/GameModes/GM_Level` (`GameplayStatics.GetGameMode`)))
  (bind _enable (`/Game/_Maps/GameModes/GM_Level.Unlock Condition` _asgm_level (`self.Open Condition`)))
  (if _enable
    (`/Engine/EditorBlueprintResources/StandardMacros.DoOnce` false
      (:`Completed`
        (`self.PlayOpenAnimation`)
        (`GameplayStatics.PlaySound2D` "/Game/_Materials/Sounds/Zombie/172004__skinnysoundguy__creature-beast-retch.172004__skinnysoundguy__creature-beast-retch" 1.0 1.0 0.0 null null)))))

(event `PlayOpenAnimation`
  (`/Engine/EditorBlueprintResources/StandardMacros.DoOnce` false
    (:`Completed`
      (bind (_direction _dooropening) (`Timeline|Timeline`)
        (:`Update`
          (`SceneComponent.K2_SetRelativeLocation` (`self.LadoDireito`) (`KismetMathLibrary.MakeVector` 0.0 (`KismetMathLibrary.Lerp` 0.0 -250.0 _dooropening)) false false)
          (`SceneComponent.K2_SetRelativeLocation` (`self.LadoEsquerdo`) (`KismetMathLibrary.MakeVector` 0.0 (`KismetMathLibrary.Lerp` 0.0 500.0 _dooropening)) false false))))))

(fn `UserConstructionScript`)