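; Level transition trigger that lets the player travel to the next saved level when the game instance permits teleporting.
; Box overlap shows an interaction widget and arms Lookat, which freezes movement, shows a loading screen, then opens NextLevel from save Slot01 and updates game progress.
; BeginPlay picks the new progress value from current progress, but only inside the ShowDebugBox branch.
; InteractWith returns the actor's ObjectiveID.
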(event `self.ReceiveBeginPlay`
  (`BoxComponent.SetBoxExtent` (`self.Box`) (`self.In Box Extent`) true)
  (if (`self.ShowDebugBox?`)
    (`KismetSystemLibrary.DrawDebugBox` (`self.K2_GetActorLocation`) (`self.In Box Extent`) (struct :`G` 0.131249 :`B` 1.0 :`A` 1.0) (struct) 999.0 5.0)
    (bind _asbpi_game_instance (cast `/Game/_Mechanics/SaveGame/BPI_GameInstance` (`GameplayStatics.GetGameInstance`)))
    (bind _output_get (set `self.As BPI Game Instance` _asbpi_game_instance))
    (bind _progress (`/Game/_Mechanics/SaveGame/BPI_GameInstance.GetGameProgress` _output_get))
    (if (>= _progress 4)
      (set `self.NewProgress` 11)
      (else
        (set `self.NewProgress` 4)))))

(event `/Game/_Mechanics/BPI_MainInteract.LookAt`
  (if (`self.InteractAllow?`)
    (bind _asbpi_game_instance (cast `/Game/_Mechanics/SaveGame/BPI_GameInstance` (`GameplayStatics.GetGameInstance`)))
    (bind _enable_ (`/Game/_Mechanics/SaveGame/BPI_GameInstance.TP_Enable?` _asbpi_game_instance))
    (if _enable_
      (`CharacterMovementComponent.DisableMovement` (`Character.CharacterMovement` (`GameplayStatics.GetPlayerCharacter` 0)))
      (bind _returnvalue (`|CreateWidget` "/Game/_Layout/HUD/WB_LoadingScreen.WB_LoadingScreen_C"))
      (`UserWidget.AddToViewport` _returnvalue 0)
      (`KismetSystemLibrary.Delay` 2.0)
      (bind _returnvalue_2 (`GameplayStatics.LoadGameFromSlot` "Slot01"))
      (bind _asbsg_game_save (cast `/Game/_Mechanics/SaveGame/BSG_GameSave` _returnvalue_2))
      (`GameplayStatics.OpenLevel` (`/Game/_Mechanics/SaveGame/BSG_GameSave.NextLevel` _asbsg_game_save))
      (`/Game/_Mechanics/SaveGame/BPI_GameInstance.SetNewProgress` _asbpi_game_instance (`self.NewProgress`)))))

(event `self.Box.OnComponentBeginOverlap`
  (params (OverlappedComponent :type "PrimitiveComponent Object Reference") (OtherActor :type "Actor Object Reference") (OtherComp :type "PrimitiveComponent Object Reference") (OtherBodyIndex :type Integer) (bFromSweep :type Boolean) (SweepResult :type "HitResult Structure (by ref)"))
  (bind _asbpi_game_instance (cast `/Game/_Mechanics/SaveGame/BPI_GameInstance` (`GameplayStatics.GetGameInstance`)))
  (bind _enable_ (`/Game/_Mechanics/SaveGame/BPI_GameInstance.TP_Enable?` _asbpi_game_instance))
  (if _enable_
    (if (== OtherActor (`GameplayStatics.GetPlayerCharacter` 0))
      (`SceneComponent.SetVisibility` (`self.Widget`) true false)
      (set `self.InteractAllow?` true))))

(event `self.Box.OnComponentEndOverlap`
  (params (OverlappedComponent :type "PrimitiveComponent Object Reference") (OtherActor :type "Actor Object Reference") (OtherComp :type "PrimitiveComponent Object Reference") (OtherBodyIndex :type Integer))
  (`SceneComponent.SetVisibility` (`self.Widget`) false false)
  (set `self.InteractAllow?` false))

(fn `Interact With`
  (returns (ObjectiveID :type String))
  (return (`self.Objective ID`)))

(fn `UserConstructionScript`)