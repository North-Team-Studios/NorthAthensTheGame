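; BP_NextLevel is an interactable trigger volume, apparently intended as a level exit, that returns an ObjectiveID when interacted with.
; BeginPlay sizes the Box and optionally draws it for debugging.
; Box overlaps toggle a Widget for any actor, as the player comparison leads nowhere.
; InteractWith prints and returns the ID, while player caching, end-game screen and level-loading logic are disconnected and never run.
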(event `self.ReceiveBeginPlay`
  (`BoxComponent.SetBoxExtent` (`self.Box`) (`self.In Box Extent`) true)
  (if (`self.ShowDebugBox?`)
    (`KismetSystemLibrary.DrawDebugBox` (`self.K2_GetActorLocation`) (`self.In Box Extent`) (struct :`G` 0.131249 :`B` 1.0 :`A` 1.0) (struct) 999.0 5.0)))

(event `self.Box.OnComponentBeginOverlap`
  (params (OverlappedComponent :type "PrimitiveComponent Object Reference") (OtherActor :type "Actor Object Reference") (OtherComp :type "PrimitiveComponent Object Reference") (OtherBodyIndex :type Integer) (bFromSweep :type Boolean) (SweepResult :type "HitResult Structure (by ref)"))
  (`SceneComponent.SetVisibility` (`self.Widget`) true false)
  (bind _jogador (`self.Jogador`)
    (:`then`
      (if (== _jogador OtherActor)
        _))
    (:`else`)))

(event `self.Box.OnComponentEndOverlap`
  (params (OverlappedComponent :type "PrimitiveComponent Object Reference") (OtherActor :type "Actor Object Reference") (OtherComp :type "PrimitiveComponent Object Reference") (OtherBodyIndex :type Integer))
  (`SceneComponent.SetVisibility` (`self.Widget`) false false))

(fn `Interact With`
  (returns (ObjectiveID :type String))
  (bind _objective_id (`self.Objective ID`))
  (`KismetSystemLibrary.PrintString` _objective_id)
  (return _objective_id))

(fn `UserConstructionScript`)