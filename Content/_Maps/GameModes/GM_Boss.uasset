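; Game mode for the police boss stage: the player must defeat BP_BossPolice before a countdown runs out.
; BeginPlay saves the level, sets a crosshair, enables the player's weapon and camera switch, starts music and finds the boss.
; Tick polls boss health and the countdown, applying delayed, repeating player damage at zero time or updating progress and loading 02AreaSegura on boss death.
; An enemy kill counter is exposed through helper functions.
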(event `self.ReceiveBeginPlay`
  (bind _returnvalue (`GameplayStatics.GetPlayerController` 0))
  (bind _asbpi_game_instance (cast `/Game/_Mechanics/SaveGame/BPI_GameInstance` (`GameplayStatics.GetGameInstance`)))
  (`|ExecutionSequence`
    (:`then_0`
      (`/Game/_Mechanics/SaveGame/BPI_GameInstance.AllowTP` _asbpi_game_instance)
      (`/Game/_Mechanics/SaveGame/BPI_GameInstance.SetNextMap` _asbpi_game_instance "02AreaSegura")
      (`PlayerController.SetMouseCursorWidget` _returnvalue "Crosshairs" null)
      (set `PlayerController.CurrentMouseCursor` "Crosshairs" _returnvalue))
    (:`then_1`
      (`/Game/_Mechanics/SaveGame/BPI_GameInstance.Save Current Level` _asbpi_game_instance))
    (:`then_2`
      (bind _asbp_jogador (cast `/Game/Characters/Jogador/Blueprint/BP_Jogador` (`GameplayStatics.GetPlayerPawn` 0)))
      (bind _output_get (set `/Game/Characters/Jogador/Blueprint/BP_Jogador.AllowWeapon?` true _asbp_jogador))
      (`/Game/Characters/Jogador/Blueprint/BP_Jogador.Switch Camera` _asbp_jogador _output_get)
      (bind _returnvalue_2 (`GameplayStatics.CreateSound2D` "/Game/_Materials/Sounds/epic-and-dramatic-109076__1_.epic-and-dramatic-109076__1_" 0.15 1.03 0.0 null false false))
      (`AudioComponent.Play` _returnvalue_2 0.0)
      (set `self.EnemyCount` 0))
    (:`then_3`
      (bind _outactors (`GameplayStatics.GetAllActorsOfClass` "/Game/Characters/Enemy/Boss/PoliceStationBoss/BP_BossPolice.BP_BossPolice_C"))
      (set `self.BossReference` (`|GetArrayItem` _outactors)))))

(event `self.ReceiveTick`
  (params (DeltaSeconds :type "Float (single-precision)"))
  (bind _bossreference (`self.BossReference`))
  (bind _health (`/Game/Enemy/BP_BaseEnemy.GetCurrentHealth` _bossreference))
  (bind _output_get (set `self.BossHPCurrent` _health))
  (bind _maxhealth (`/Game/Enemy/BP_BaseEnemy.GetMaxHealth` _bossreference))
  (set `self.BossHPMax` _maxhealth)
  (bind _remainingtime (`self.Start Countdown` (`self.Countdown`)))
  (`|ExecutionSequence`
    (:`then_0`
      ;[1 1 1] Time's Up
      (if (<= _remainingtime 0.0)
        (`self.DeathByTimeOver` (`self.DelayToDamage`))))
    (:`then_1`
      (if (<= _output_get 0.0)
        (bind _asbpi_game_instance (cast `/Game/_Mechanics/SaveGame/BPI_GameInstance` (`GameplayStatics.GetGameInstance`)))
        (`/Game/_Mechanics/SaveGame/BPI_GameInstance.SetNewProgress` _asbpi_game_instance 19)
        (`/Game/_Mechanics/SaveGame/BPI_GameInstance.LoadNewLevel` _asbpi_game_instance "02AreaSegura" false)))))

(event `Enemies Killed`
  (set `self.EnemyCount` (+ (`self.EnemyCount`) 1)))

(event `DeathByTimeOver`
  (params (DOT :type "Float (double-precision)"))
  (bind _myplayercharacter (`/Game/_Mechanics/QuestSystem/BPL_CommonFunctionLibrary.GetMyPlayerCharacter`))
  (bind _health (`/Game/Characters/Jogador/Blueprint/BP_Jogador.GetCurrentHealth` _myplayercharacter))
  (if (>= _health 0.0)
    (`KismetSystemLibrary.Delay` DOT)
    (`/Game/_Mechanics/DamageSystem/BPI_Damagable.TakeDamage` _myplayercharacter (make `/Game/_Mechanics/DamageSystem/S_DamageInfo` 10.0 "NewEnumerator4"))))

(fn `Get Enemies Killed`
  (returns (EnemyCount :type Integer))
  (return (`self.EnemyCount`)))

(fn `GetCountdown`
  (returns (Countdown :type "Float (double-precision)"))
  (return (`self.Countdown`)))

(fn `Start Countdown`
  (params (MaxStageTime :type "Float (double-precision)"))
  (returns (RemainingTime :type "Float (double-precision)"))
  (bind _output_get (set `self.Countdown` (`KismetMathLibrary.FClamp` (- (`self.Countdown`) (`GameplayStatics.GetWorldDeltaSeconds`)) 0.0 MaxStageTime)))
  (return _output_get))

(fn `Unlock Condition`
  (params (`Kill Condition` :type Integer))
  (returns (Enable :type Boolean))
  (bind _returnvalue (>= (`self.EnemyCount`) `Kill Condition`))
  (if _returnvalue
    (return _returnvalue)))

(fn `UserConstructionScript`)