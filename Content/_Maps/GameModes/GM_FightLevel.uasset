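; GM_FightLevel is the game mode for fight levels, running the stage countdown timer.
; On BeginPlay it resets the countdown to the maximum stage time, saves the current level through the game instance interface and plays the main stage sound.
; Tick subtracts world delta seconds from the countdown, clamped between zero and the maximum, and GetCountdown exposes the remaining time.
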(event `self.ReceiveBeginPlay`
  (set `self.Countdown` (`self.MaxStageTime`))
  (bind _asbpi_game_instance (cast `/Game/_Mechanics/SaveGame/BPI_GameInstance` (`GameplayStatics.GetGameInstance`)))
  (`/Game/_Mechanics/SaveGame/BPI_GameInstance.Save Current Level` _asbpi_game_instance)
  (`GameplayStatics.PlaySound2D` "/Game/_Materials/Sounds/UI/ActionLevel/SUI_MainStage.SUI_MainStage" 0.2 1.0 0.0 null null))

(event `self.ReceiveTick`
  (params (DeltaSeconds :type "Float (single-precision)"))
  (`self.StartCountdow`))

(fn `GetCountdown`
  (returns (Countdown :type "Float (double-precision)"))
  (return (`self.Countdown`)))

(fn `StartCountdow`
  (set `self.Countdown` (`KismetMathLibrary.FClamp` (- (`self.Countdown`) (`GameplayStatics.GetWorldDeltaSeconds`)) 0.0 (`self.MaxStageTime`))))

(fn `UserConstructionScript`)