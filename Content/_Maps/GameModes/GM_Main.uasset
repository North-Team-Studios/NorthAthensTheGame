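; Main game mode: on BeginPlay it allows TP, sets "02AreaSegura" as the next map and saves the level through the game instance.
; It also sets a crosshair cursor and enables the player's weapon and matching camera.
; An enemy kill counter feeds an unlock condition check.
; Countdown helpers and a delayed time-over damage event exist, but the countdown trigger and music setup are disconnected.
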(event `self.ReceiveBeginPlay`
  (bind _returnvalue (`GameplayStatics.GetPlayerController` 0))
  (bind _asbpi_game_instance (cast `/Game/_Mechanics/SaveGame/BPI_GameInstance` (`GameplayStatics.GetGameInstance`)))
  (`|ExecutionSequence`
    (:`then_0`
      (`/Game/_Mechanics/SaveGame/BPI_GameInstance.AllowTP` _asbpi_game_instance)
      (`/Game/_Mechanics/SaveGame/BPI_GameInstance.SetNextMap` _asbpi_game_instance "02AreaSegura")
      (`PlayerController.SetMouseCursorWidget` _returnvalue "Crosshairs" null)
      (set `PlayerController.CurrentMouseCursor` "Crosshairs" _returnvalue))
    (:`then_1`
      (`/Game/_Mechanics/SaveGame/BPI_GameInstance.Save Current Level` _asbpi_game_instance))
    (:`then_2`
      (bind _asbp_jogador (cast `/Game/Characters/Jogador/Blueprint/BP_Jogador` (`GameplayStatics.GetPlayerPawn` 0)))
      (bind _output_get (set `/Game/Characters/Jogador/Blueprint/BP_Jogador.AllowWeapon?` true _asbp_jogador))
      (`/Game/Characters/Jogador/Blueprint/BP_Jogador.Switch Camera` _asbp_jogador _output_get))))

(event `self.ReceiveTick`
  (params (DeltaSeconds :type "Float (single-precision)")))

(event `Enemies Killed`
  (set `self.EnemyCount` (+ (`self.EnemyCount`) 1)))

(event `DeathByTimeOver`
  (params (DOT :type "Float (double-precision)"))
  (bind _myplayercharacter (`/Game/_Mechanics/QuestSystem/BPL_CommonFunctionLibrary.GetMyPlayerCharacter`))
  (bind _health (`/Game/Characters/Jogador/Blueprint/BP_Jogador.GetCurrentHealth` _myplayercharacter))
  (if (>= _health 0.0)
    (`KismetSystemLibrary.Delay` DOT)
    (`/Game/_Mechanics/DamageSystem/BPI_Damagable.TakeDamage` _myplayercharacter (make `/Game/_Mechanics/DamageSystem/S_DamageInfo` 20.0 "NewEnumerator4"))))

(fn `Get Enemies Killed`
  (returns (EnemyCount :type Integer))
  (return (`self.EnemyCount`)))

(fn `GetCountdown`
  (returns (Countdown :type "Float (double-precision)"))
  (return (`self.Countdown`)))

(fn `Start Countdown`
  (params (MaxStageTime :type "Float (double-precision)"))
  (returns (RemainingTime :type "Float (double-precision)"))
  (bind _output_get (set `self.Countdown` (`KismetMathLibrary.FClamp` (- (`self.Countdown`) (`GameplayStatics.GetWorldDeltaSeconds`)) 0.0 MaxStageTime)))
  (return _output_get))

(fn `Unlock Condition`
  (params (`Kill Condition` :type Integer))
  (returns (Enable :type Boolean))
  (bind _returnvalue (>= (`self.EnemyCount`) `Kill Condition`))
  (if _returnvalue
    (return _returnvalue)))

(fn `UserConstructionScript`)