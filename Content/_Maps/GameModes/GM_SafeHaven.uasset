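; GM_SafeHaven is the game mode for safe haven maps, where the player cannot use weapons.
; On BeginPlay it flags the player character as in a safe area, then has the game instance save the current level and block teleporting.
; It then disallows weapons on BP_Jogador, switches its camera to match and plays a wind synth sound.
; Save-loading and gait-update chains are left unconnected.
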(event `self.ReceiveBeginPlay`
  (set `/Game/Characters/Jogador/Blueprint/BP_Jogador.AreaSegura?` true (`/Game/_Mechanics/QuestSystem/BPL_CommonFunctionLibrary.GetMyPlayerCharacter`))
  (bind _asbpi_game_instance (cast `/Game/_Mechanics/SaveGame/BPI_GameInstance` (`GameplayStatics.GetGameInstance`)))
  (`/Game/_Mechanics/SaveGame/BPI_GameInstance.Save Current Level` _asbpi_game_instance)
  (`/Game/_Mechanics/SaveGame/BPI_GameInstance.BlockTp` _asbpi_game_instance)
  (bind _asbp_jogador (cast `/Game/Characters/Jogador/Blueprint/BP_Jogador` (`GameplayStatics.GetPlayerPawn` 0)))
  (bind _output_get (set `/Game/Characters/Jogador/Blueprint/BP_Jogador.AllowWeapon?` false _asbp_jogador))
  (`/Game/Characters/Jogador/Blueprint/BP_Jogador.Switch Camera` _asbp_jogador _output_get)
  (`GameplayStatics.SpawnSound2D` "/Game/_Materials/Sounds/Atmosphere/SOW_windsynth.SOW_windsynth" 1.0 1.0 0.0 null))

(fn `UserConstructionScript`)