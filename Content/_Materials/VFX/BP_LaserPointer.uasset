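; Laser pointer Blueprint that renders a Niagara aiming beam for the player's character.
; Each Tick shows the beam, or hides it when the player moves faster than a speed threshold.
; While LineTraceActivated, the character-to-cursor-hit distance sets the beam's "Beam End" length, and reloading hides both beam and pointer mesh.
; The line trace's result is unused, and disconnected leftover nodes hold an older spawned-reticle and camera-trace approach.
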(event `self.ReceiveBeginPlay`)

(event `LaserPointer`
  (bind _returnvalue (`GameplayStatics.GetPlayerCharacter` 0))
  (`/Engine/EditorBlueprintResources/StandardMacros.IsValid` _returnvalue
    (:`Is Valid`
      (if (> (`KismetMathLibrary.VSize` (`self.GetVelocity` _returnvalue)) 400.0)
        (`SceneComponent.SetVisibility` (`self.Niagara_LaserPointer`) false false)
        (else
          (`SceneComponent.SetVisibility` (`self.Niagara_LaserPointer`) true false))))))

(event `self.ReceiveTick`
  (params (DeltaSeconds :type "Float (single-precision)"))
  (`self.LaserPointer`)
  ;[1 1 1] Comment
  (if (`self.Line Trace Activated?`)
    (`self.LineTrace`)
    (if (`/Game/Characters/Jogador/Blueprint/BP_Jogador.isReloading?` (`/Game/_Mechanics/QuestSystem/BPL_CommonFunctionLibrary.GetMyPlayerCharacter`))
      (`SceneComponent.SetVisibility` (`self.Niagara_LaserPointer`) false false)
      (`SceneComponent.SetVisibility` (`self.SM_LaserPointer`) false false))))

(event `LineTrace`
  (bind (_bblockinghit _binitialoverlap _time _distance _location _impactpoint) (`GameplayStatics.BreakHitResult` (`PlayerController.GetHitResultUnderCursorByChannel` (`GameplayStatics.GetPlayerController` 0) "TraceTypeQuery1" true)))
  (bind _returnvalue (`SceneComponent.K2_GetComponentLocation` (`Actor.RootComponent` (`/Game/_Mechanics/QuestSystem/BPL_CommonFunctionLibrary.GetMyPlayerCharacter`))))
  (`KismetSystemLibrary.LineTraceSingle` :`Start` _returnvalue :`End` _impactpoint :`TraceChannel` "TraceTypeQuery1" :`TraceColor` (struct :`G` 1.0 :`B` 0.416332 :`A` 1.0))
  (`FXSystemComponent.SetVectorParameter` (`self.Niagara_LaserPointer`) "Beam End" (`KismetMathLibrary.MakeVector` (`KismetMathLibrary.Vector_Distance` _returnvalue _impactpoint))))

(fn `UserConstructionScript`)