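; Laser pointer actor that draws a Niagara beam whose length follows the mouse cursor.
; Each tick it hides the beam while the player moves fast and, if tracing is active, hides beam and mesh during reloads.
; A forward trace sized by cursor distance sets and prints Beam End, using hit-to-cursor distance when blocked, otherwise actor-to-cursor.
; BeginPlay spawns a hidden pointer effect; an older camera-based trace is left disconnected.
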(event `LaserPointer`
  (bind _returnvalue (`GameplayStatics.GetPlayerCharacter` 0))
  (`/Engine/EditorBlueprintResources/StandardMacros.IsValid` _returnvalue
    (:`Is Valid`
      (if (> (`KismetMathLibrary.VSize` (`self.GetVelocity` _returnvalue)) 400.0)
        (`SceneComponent.SetVisibility` (`self.NiagaraLaser`) false false)
        (else
          (`SceneComponent.SetVisibility` (`self.NiagaraLaser`) true false))))))

(event `self.ReceiveBeginPlay`
  (bind _returnvalue (`NiagaraFunctionLibrary.SpawnSystemAtLocation` "/Game/_Materials/VFX/FX_Pointer.FX_Pointer"))
  (set `self.VFX_Mira` _returnvalue)
  (`SceneComponent.SetVisibility` (`self.VFX_Mira`) false false))

(event `self.ReceiveTick`
  (params (DeltaSeconds :type "Float (single-precision)"))
  (`self.LaserPointer`)
  (if (`self.Line Trace Activated?`)
    (`self.LineTrace`)
    (if (`/Game/Characters/Jogador/Blueprint/BP_Jogador.isReloading?` (`/Game/_Mechanics/QuestSystem/BPL_CommonFunctionLibrary.GetMyPlayerCharacter`))
      (`SceneComponent.SetVisibility` (`self.NiagaraLaser`) false false)
      (`SceneComponent.SetVisibility` (`self.SM_LaserPointer`) false false))))

(event `LineTrace`
  (bind _returnvalue (`SceneComponent.K2_GetComponentLocation` (`self.DefaultSceneRoot`)))
  (bind (_bblockinghit _binitialoverlap _time _distance _location) (`GameplayStatics.BreakHitResult` (`PlayerController.GetHitResultUnderCursorByChannel` (`GameplayStatics.GetPlayerController` 0) "TraceTypeQuery2" true)))
  (bind _returnvalue_2 (`KismetMathLibrary.Vector_Distance` (`self.K2_GetActorLocation`) _location))
  (bind _outhit (`KismetSystemLibrary.LineTraceSingle` _returnvalue (+ _returnvalue (* (`SceneComponent.GetForwardVector` (`self.DefaultSceneRoot`)) _returnvalue_2)) "TraceTypeQuery1"))
  (bind _returnvalue_x (`KismetMathLibrary.BreakVector` (select `bool` (`GameplayStatics.BreakHitResult` _outhit) :`false` (`KismetMathLibrary.MakeVector` _returnvalue_2) :`true` (`KismetMathLibrary.MakeVector` (`KismetMathLibrary.Vector_Distance` (`.Location` (`GameplayStatics.BreakHitResult` _outhit)) _location)) :!type "Vector Structure")))
  (`KismetSystemLibrary.PrintString` (`KismetStringLibrary.Conv_DoubleToString` _returnvalue_x) true true (struct :`G` 0.66 :`B` 1.0 :`A` 1.0) 0.0)
  (`FXSystemComponent.SetVectorParameter` (`self.NiagaraLaser`) "Beam End" (`KismetMathLibrary.MakeVector` _returnvalue_x)))

(fn `UserConstructionScript`)