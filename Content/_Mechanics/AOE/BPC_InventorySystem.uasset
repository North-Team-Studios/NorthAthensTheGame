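; BPC_InventorySystem is a component that lets the player preview and place an area heal-over-time skill in the level.
; The Slot 02 input toggles build mode, where each tick traces from the player camera along the mouse direction.
; A collision-free preview mesh, created once per session, takes the projected point's X/Y and the hit's Z.
; Interact spawns BP_AOE_OverTime_Heal at that transform, then clears the preview and resets the DoOnce.
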(event `self.ReceiveBeginPlay`
  (bind _asbp_jogador (cast `/Game/Characters/Jogador/Blueprint/BP_Jogador` (`GameplayStatics.GetPlayerPawn` 0)))
  (bind _output_get (set `self.Jogador` _asbp_jogador))
  (set `self.Camera` (`/Game/Characters/Jogador/Blueprint/BP_Jogador.MainCamera` _output_get)))

(event `self.ReceiveTick`
  (params (DeltaSeconds :type "Float (single-precision)"))
  (if (`self.inBuildMode`)
    (`self.PreviewLoop`)))

(event `PreviewLoop`
  (bind _preview_mesh (`self.Preview Mesh`))
  (bind _returnvalue_location (`KismetMathLibrary.BreakTransform` (`SceneComponent.K2_GetComponentToWorld` (`self.Camera`))))
  (bind (_returnvalue_x _returnvalue_y) (`KismetMathLibrary.BreakVector` (+ _returnvalue_location (* (`.WorldDirection` (`PlayerController.DeprojectMousePositionToWorld` (`GameplayStatics.GetPlayerController` 0))) 400.0))))
  (bind (_outhit _returnvalue) (`KismetSystemLibrary.LineTraceSingle` _returnvalue_location (`KismetMathLibrary.MakeVector` _returnvalue_x _returnvalue_y) "TraceTypeQuery1"))
  (if _returnvalue
    (`|ExecutionSequence`
      (:`then_0`
        (`/Engine/EditorBlueprintResources/StandardMacros.DoOnce` false :!label _label
          (:`Completed`
            (bind _returnvalue_2 (`|AddComponentByClass` (`self.Jogador`) "/Script/Engine.StaticMeshComponent" false (`self.PreviewTransform`)))
            (bind _output_get (set `self.Preview Mesh` _returnvalue_2))
            (`StaticMeshComponent.SetStaticMesh` _output_get (`self.Main Mesh`))
            (`PrimitiveComponent.SetMaterial` _preview_mesh 0 "/Game/_Materials/Materials/M_Preview.M_Preview")
            (`PrimitiveComponent.SetCollisionEnabled` _preview_mesh "NoCollision"))))
      (:`then_1`
        (if true
          (bind _output_get_2 (set `self.PreviewTransform` (`KismetMathLibrary.MakeTransform` (`KismetMathLibrary.MakeVector` _returnvalue_x _returnvalue_y (.z (`.Location` (`GameplayStatics.BreakHitResult` _outhit)))))))
          (`SceneComponent.K2_SetWorldTransform` (`self.Preview Mesh`) _output_get_2 false false))))))

(event `Reset Preview Mode`
  (goto _label :!via `Reset`))

(event `EnhancedInput|/Game/ThirdPerson/Input/Actions/IA_Slot_02`
  (params (ActionValue :type Boolean) (ElapsedSeconds :type "Float (double-precision)") (TriggeredSeconds :type "Float (double-precision)") (InputAction :type "InputAction Object Reference" :default "/Game/ThirdPerson/Input/Actions/IA_Slot_02.IA_Slot_02"))
  (:`Triggered`
    (set `self.Skill 01 Activated` true)
    (`/Engine/EditorBlueprintResources/StandardMacros.FlipFlop`
      (:`A`
        (set `self.inBuildMode` true))
      (:`B`
        (`self.Stop Preview`)))))

(event `EnhancedInput|/Game/ThirdPerson/Input/Actions/IA_Interact`
  (params (ActionValue :type Boolean) (ElapsedSeconds :type "Float (double-precision)") (TriggeredSeconds :type "Float (double-precision)") (InputAction :type "InputAction Object Reference" :default "/Game/ThirdPerson/Input/Actions/IA_Interact.IA_Interact"))
  (:`Triggered`
    (`self.Place Skill to Level`)))

(event `Place Skill to Level`
  (`|SpawnActorFromClass` "/Game/_Mechanics/AOE/BP_AOE_OverTime_Heal.BP_AOE_OverTime_Heal_C" (`self.PreviewTransform`) "Undefined" "MultiplyWithRoot" null 1.0 999.0 true true true null)
  (`self.Stop Preview`))

(event `Stop Preview`
  (set `self.inBuildMode` false)
  (bind _preview_mesh (`self.Preview Mesh`)
    (:`then`
      (`StaticMeshComponent.SetStaticMesh` _preview_mesh null)
      (set `self.Preview Mesh` null)
      (`self.Reset Preview Mode`))
    (:`else`)))

(event `EnhancedInput|/Game/ThirdPerson/Input/Actions/IA_LeftMouse`
  (params (ActionValue :type Boolean) (ElapsedSeconds :type "Float (double-precision)") (TriggeredSeconds :type "Float (double-precision)") (InputAction :type "InputAction Object Reference" :default "/Game/ThirdPerson/Input/Actions/IA_LeftMouse.IA_LeftMouse")))