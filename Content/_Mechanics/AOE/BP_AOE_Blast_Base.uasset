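; Base Blueprint for blast-type area-of-effect actors, adding visual and audio feedback to the parent AOE class.
; Trigger runs the parent logic, then spawns a Cascade emitter attached to the root and plays the blast sound at the actor's location, if those assets are valid.
; The actor destroys itself when the particle system finishes, or after a short delay if no effect is set.
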(event `self.SpawnAOESphere`
  (`parent.SpawnAOESphere`))

(event `self.Trigger`
  (`parent.Trigger`)
  (`self.SpawnBlastEffect`)
  (`self.PlayBlastSound`))

(event `SpawnBlastEffect`
  ;[0.2292 0.2292 0.2292] Spawn Blast Effect
  (bind _blast_effect_cascader (`self.Blast Effect Cascader`)
    (:`then`
      (bind _returnvalue (`GameplayStatics.SpawnEmitterAttached` _blast_effect_cascader (`self.DefaultSceneRoot`)))
      (add `ParticleSystemComponent.OnSystemFinished` _returnvalue (delegate `SystemFinished`)))
    (:`else`
      (`KismetSystemLibrary.Delay` 1.0)
      (`self.K2_DestroyActor`))))

(event `SystemFinished`
  (params (PSystem :type "ParticleSystemComponent Object Reference"))
  ;[0.2292 0.2292 0.2292] Spawn Blast Effect
  (`self.K2_DestroyActor`))

(event `PlayBlastSound`
  ;[0.2031 0.2031 0.2031] Play Blast Sound
  (bind _blast_sound (`self.Blast Sound`)
    (:`then`
      (`GameplayStatics.PlaySoundAtLocation` _blast_sound (`self.K2_GetActorLocation`) (struct) 1.0 1.0 0.0 null null null null))
    (:`else`)))

(fn `UserConstructionScript`
  (`parent.UserConstructionScript`))