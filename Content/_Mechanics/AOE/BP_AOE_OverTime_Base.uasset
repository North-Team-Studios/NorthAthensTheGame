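; Base Blueprint for area-of-effect actors that act over time, extending a parent AOE class.
; On Trigger it runs the parent logic, plays an optional sound at its location, starts a looping SpawnInterval timer and binds to the AOE overlap-actor event.
; A one-shot timer fires after Duration, though the timer and binding targets are not shown.
; CustonOverlap is an empty event taking an Actor.
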(event `PlayAreaSound`
  (bind _sound (`self.Sound`)
    (:`then`
      (`GameplayStatics.PlaySoundAtLocation` _sound (`self.K2_GetActorLocation`) (struct) 1.0 1.0 0.0 null null null null))
    (:`else`)))

(event `self.Trigger`
  (`parent.Trigger`)
  (`self.PlayAreaSound`)
  (`|ExecutionSequence`
    (:`then_0`
      (`KismetSystemLibrary.K2_SetTimerDelegate` (`|CreateDelegate` :!event `SpawnAOESphere`) (`self.SpawnInterval`) true)
      (add `self.OnAOEOverlapActor` (`|CreateDelegate` :!event `CustonOverlap`)))
    (:`then_1`
      (`KismetSystemLibrary.K2_SetTimerDelegate` (`|CreateDelegate` :!event `K2_DestroyActor`) (`self.Duration`)))))

(event `CustonOverlap` :!signature `self.OnAOEOverlapActor`
  (params (Actor :type "Actor Object Reference")))

(fn `UserConstructionScript`
  (`parent.UserConstructionScript`))