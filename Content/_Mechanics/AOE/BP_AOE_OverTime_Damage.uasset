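; BP_AOE_OverTime_Damage is an area-of-effect child Blueprint that, despite its Damage name, heals the player.
; On Trigger it runs the parent logic, then adds a static mesh using MainMesh and a slightly raised Niagara component at runtime.
; Its CustonOverlap event calls Heal with a fixed amount on player 0's BP_Jogador pawn.
; No timing or overlap detection is implemented in this graph.
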(event `/Game/_Mechanics/AOE/BP_AOE_Base.Trigger`
  (`parent.Trigger`)
  (bind _returnvalue (`AddComponent|NODE_AddStaticMeshComponent-0`))
  (`StaticMeshComponent.SetStaticMesh` _returnvalue (`self.Main Mesh`))
  (`AddComponent|NODE_AddNiagaraComponent-4` :`RelativeTransform` (`KismetMathLibrary.MakeTransform` (0.0 0.0 1.0))))

(event `self.CustonOverlap`
  (params (Actor :type "Actor Object Reference"))
  (bind _asbp_jogador (cast `/Game/Characters/Jogador/Blueprint/BP_Jogador` (`GameplayStatics.GetPlayerPawn` 0)))
  (`/Game/Characters/Jogador/Blueprint/BP_Jogador.Heal` _asbp_jogador 10.0))

(fn `UserConstructionScript`
  (`parent.UserConstructionScript`))