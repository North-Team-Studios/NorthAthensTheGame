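; Area-of-effect heal-over-time actor that restores health to the player.
; On Trigger it runs the parent logic, adds its main mesh and spawns a Niagara heal effect with no location set.
; CustonOverlap applies a fixed heal to player pawn 0 cast to BP_Jogador, with the repeat timing not defined in this Blueprint.
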(event `/Game/_Mechanics/AOE/BP_AOE_Base.Trigger`
  (`parent.Trigger`)
  (bind _returnvalue (`AddComponent|NODE_AddStaticMeshComponent-0`))
  (`StaticMeshComponent.SetStaticMesh` _returnvalue (`self.Main Mesh`))
  (bind _returnvalue_2 (`NiagaraFunctionLibrary.SpawnSystemAtLocation` "/Game/_Materials/VFX/VFX_Heal/Heal_FX_Niagara.Heal_FX_Niagara"))
  (`ActorComponent.Activate` _returnvalue_2 false))

(event `self.CustonOverlap`
  (params (Actor :type "Actor Object Reference"))
  (bind _asbp_jogador (cast `/Game/Characters/Jogador/Blueprint/BP_Jogador` (`GameplayStatics.GetPlayerPawn` 0)))
  (`/Game/Characters/Jogador/Blueprint/BP_Jogador.Heal` _asbp_jogador 10.0))

(fn `UserConstructionScript`
  (`parent.UserConstructionScript`))