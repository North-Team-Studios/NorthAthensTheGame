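; Area-of-effect actor, named as an over-time slow, that applies a negative effect through its overlap event.
; Trigger runs the parent logic, then adds a static mesh component showing MainMesh.
; CustonOverlap proceeds only if the actor equals the player character, then casts it to BP_BaseEnemy and calls NegativeEffect.
; Leftover caching and damage nodes are disconnected, and no slow or timing logic is defined here.
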(event `/Game/_Mechanics/AOE/BP_AOE_Base.Trigger`
  (`parent.Trigger`)
  (bind _returnvalue (`AddComponent|NODE_AddStaticMeshComponent-0`))
  (`StaticMeshComponent.SetStaticMesh` _returnvalue (`self.Main Mesh`)))

(event `self.CustonOverlap`
  (params (Actor :type "Actor Object Reference"))
  (if (== (`/Game/_Mechanics/QuestSystem/BPL_CommonFunctionLibrary.GetMyPlayerCharacter`) Actor)
    (bind _asbp_base_enemy (cast `/Game/Enemy/BP_BaseEnemy` Actor))
    (`/Game/Enemy/BP_BaseEnemy.NegativeEffect` _asbp_base_enemy)))

(fn `UserConstructionScript`
  (`parent.UserConstructionScript`))