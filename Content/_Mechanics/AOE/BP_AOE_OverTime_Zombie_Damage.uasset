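; Area-of-effect damage-over-time actor that hurts zombies and other BP_BaseEnemy actors, building on a parent AOE Blueprint.
; Trigger runs the parent logic, then adds a static mesh component to the actor.
; CustomOverlap skips the player, filters for BPI_Damagable actors that cast to BP_BaseEnemy, and sends living ones a fixed, typed damage message.
; No timing logic appears in this Blueprint itself.
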(event `/Game/_Mechanics/AOE/BP_AOE_Base.Trigger`
  (`parent.Trigger`)
  (bind _returnvalue (`AddComponent|NODE_AddStaticMeshComponent-0`))
  (`StaticMeshComponent.SetStaticMesh` _returnvalue (`self.New Mesh`)))

(event `self.CustomOverlap`
  (params (Actor :type "Actor Object Reference"))
  (if (and (!= Actor (`/Game/_Mechanics/QuestSystem/BPL_CommonFunctionLibrary.GetMyPlayerCharacter`)) (`KismetSystemLibrary.DoesImplementInterface` Actor "/Game/_Mechanics/DamageSystem/BPI_Damagable.BPI_Damagable_C"))
    (bind _asbp_base_enemy (cast `/Game/Enemy/BP_BaseEnemy` Actor))
    (bind _health (`/Game/_Mechanics/DamageSystem/BPI_Damagable.GetCurrentHealth` _asbp_base_enemy))
    (if (> _health 0.0)
      (message `/Game/_Mechanics/DamageSystem/BPI_Damagable.TakeDamage` _asbp_base_enemy (make `/Game/_Mechanics/DamageSystem/S_DamageInfo` 12.5 "NewEnumerator4" "NewEnumerator1")))))

(fn `UserConstructionScript`
  (`parent.UserConstructionScript`))