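; Game mode for a timed shooting minigame that arms the player, switches camera, sets a crosshair cursor and starts music on BeginPlay.
; Tick drains a countdown; once it hits zero, the player takes delayed, repeated damage while health remains.
; Each reported kill raises the enemy count, adds time and plays the HUD timer bar's bonus animation.
; OpenDoorCondition checks that count against a kill threshold, and GetCountdown exposes the remaining time.
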(event `self.ReceiveBeginPlay`
  (bind _returnvalue (`GameplayStatics.GetPlayerController` 0))
  (cast `/Game/_Mechanics/SaveGame/BPI_GameInstance` (`GameplayStatics.GetGameInstance`))
  (`|ExecutionSequence`
    (:`then_0`
      (`PlayerController.SetMouseCursorWidget` _returnvalue "Crosshairs" null)
      (set `PlayerController.CurrentMouseCursor` "Crosshairs" _returnvalue))
    (:`then_2`
      (bind _asbp_jogador (cast `/Game/Characters/Jogador/Blueprint/BP_Jogador` (`GameplayStatics.GetPlayerPawn` 0)))
      (bind _output_get (set `/Game/Characters/Jogador/Blueprint/BP_Jogador.AllowWeapon?` true _asbp_jogador))
      (`/Game/Characters/Jogador/Blueprint/BP_Jogador.Switch Camera` _asbp_jogador _output_get)
      (bind _returnvalue_2 (`GameplayStatics.CreateSound2D` "/Game/_Materials/Sounds/epic-and-dramatic-109076__1_.epic-and-dramatic-109076__1_" 0.2 1.1 0.0 null false false))
      (`AudioComponent.Play` _returnvalue_2 0.0))))

(event `self.ReceiveTick`
  (params (DeltaSeconds :type "Float (single-precision)"))
  (bind _remainingtime (`self.Start Countdown` (`self.Countdown`)))
  ;[1 1 1] Time's Up
  (if (<= _remainingtime 0.0)
    (`self.DeathByTimeOver` (`self.DelayToDamage`))))

(event `Enemies Killed`
  (set `self.EnemyCount` (+ (`self.EnemyCount`) 1))
  (`self.Add Timer` 5.0))

(event `DeathByTimeOver`
  (params (DOT :type "Float (double-precision)"))
  (bind _myplayercharacter (`/Game/_Mechanics/QuestSystem/BPL_CommonFunctionLibrary.GetMyPlayerCharacter`))
  (bind _health (`/Game/Characters/Jogador/Blueprint/BP_Jogador.GetCurrentHealth` _myplayercharacter))
  (if (>= _health 0.0)
    (`KismetSystemLibrary.Delay` DOT)
    (`/Game/_Mechanics/DamageSystem/BPI_Damagable.TakeDamage` _myplayercharacter (make `/Game/_Mechanics/DamageSystem/S_DamageInfo` 20.0 "NewEnumerator4"))))

(event `Add Timer`
  (params (`Time to Add` :type "Float (double-precision)"))
  (set `self.Countdown` (+ (`self.Countdown`) `Time to Add`))
  (bind _returnvalue (`GameplayStatics.GetActorOfClass` "/Game/_Layout/HUD_Jogador.HUD_Jogador_C"))
  (bind _wb_timerbar (`/Game/_Layout/HUD/GM_Huds/WB_HUD.WB_TimerBar` (`/Game/_Layout/HUD_Jogador.Stage HUD` _returnvalue)))
  ;[1 1 1] Off
  (`UserWidget.PlayAnimation` _wb_timerbar (`/Game/_Layout/HUD/Content/WB_TimerBar.PlusTimeBar` _wb_timerbar) 0.0 1 "Forward" 1.0 false))

(fn `GetCountdown`
  (returns (Countdown :type "Float (double-precision)"))
  (return (`self.Countdown`)))

(fn `Open Door Condition`
  (params (`Kill Condition` :type Integer))
  (returns (`Door Status` :type Boolean))
  (bind _returnvalue (>= (`self.EnemyCount`) `Kill Condition`))
  (if _returnvalue
    (return _returnvalue)))

(fn `Start Countdown`
  (params (MaxStageTime :type "Float (double-precision)"))
  (returns (RemainingTime :type "Float (double-precision)"))
  (bind _output_get (set `self.Countdown` (`KismetMathLibrary.FClamp` (- (`self.Countdown`) (`GameplayStatics.GetWorldDeltaSeconds`)) 0.0 MaxStageTime)))
  (return _output_get))

(fn `UserConstructionScript`)