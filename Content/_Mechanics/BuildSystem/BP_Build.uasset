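; BP_Build is a build-system actor that creates its visible mesh at runtime and checks for nearby pawns.
; On BeginPlay it adds a static mesh component using MainMesh and draws a debug sphere slightly above it.
; A sphere overlap of the same radius at the actor's location finds pawns, ignoring the instigator, and only prints their names.
; An unconnected branch would add a cube mesh when Blueprint is false.
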(event `self.ReceiveBeginPlay`
  (bind (_returnvalue_x _returnvalue_y _returnvalue_z) (`KismetMathLibrary.BreakVector` (`SceneComponent.K2_GetComponentLocation` (`self.Static Mesh`))))
  (bind _returnvalue (`|AddComponentByClass` "/Script/Engine.StaticMeshComponent"))
  (bind _output_get (set `self.Static Mesh` _returnvalue))
  (`StaticMeshComponent.SetStaticMesh` _output_get (`self.Main Mesh`))
  (`KismetSystemLibrary.DrawDebugSphere` (`KismetMathLibrary.MakeVector` _returnvalue_x _returnvalue_y (+ _returnvalue_z 20.0)) (`self.Radius`) 12 (struct :`G` 0.157874 :`B` 1.0 :`A` 1.0) 2.0 1.0)
  (bind _outactors (`KismetSystemLibrary.SphereOverlapActors` (`self.K2_GetActorLocation`) (`self.Radius`) (`|MakeArray` "ObjectTypeQuery3" :!type "EObjectTypeQuery Enum") null (select `bool` true :`true` (`|MakeArray` (`self.GetInstigator`) :!type "Actor Object Reference"))))
  (for _array_element _outactors
    (`KismetSystemLibrary.PrintString` (`KismetSystemLibrary.GetDisplayName` _array_element))))

(fn `UserConstructionScript`)