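; BP_Repair is a repairable world object with a timed hold interaction, a smoke effect and an objective ID returned by InteractWith.
; Box overlap toggles a prompt widget, which swaps to a progress bar during repair.
; Each Lookat call halts the player, accumulates delta time and plays a fix montage until TimeToBuild passes, then destroys the smoke and disables box collision.
; Cancel resets progress, prompt and montage.
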(event `self.ReceiveBeginPlay`
  (`|ExecutionSequence`
    (:`then_0`
      (if (`self.ShowDebugBox?`)
        (`KismetSystemLibrary.DrawDebugBox` (`self.K2_GetActorLocation`) (`self.In Box Extent`) (struct :`G` 0.131249 :`B` 1.0 :`A` 1.0) (struct) 999.0 5.0)))
    (:`then_1`
      (bind _returnvalue (`|CreateWidget` "/Game/_Layout/HUD/Content/Interaction/WB_Interaction.WB_Interaction_C"))
      (bind _output_get (set `self.HUD Interaction` _returnvalue))
      (`/Game/_Layout/HUD/Content/Interaction/WB_Interaction.Set_Title_Label` _output_get (`self.Title Lable`))
      (`WidgetComponent.SetWidget` (`self.Widget`) (`self.HUD Interaction`)))
    (:`then_2`
      (bind _returnvalue_2 (`|CreateWidget` "/Game/_Layout/HUD/Content/Fix/WB_RepairingBar.WB_RepairingBar_C"))
      (set `self.HUD ProgressBar` _returnvalue_2))))

(event `self.Box.OnComponentBeginOverlap`
  (params (OverlappedComponent :type "PrimitiveComponent Object Reference") (OtherActor :type "Actor Object Reference") (OtherComp :type "PrimitiveComponent Object Reference") (OtherBodyIndex :type Integer) (bFromSweep :type Boolean) (SweepResult :type "HitResult Structure (by ref)"))
  (`SceneComponent.SetVisibility` (`self.Widget`) true false)
  (set `self.Actor` OtherActor))

(event `self.Box.OnComponentEndOverlap`
  (params (OverlappedComponent :type "PrimitiveComponent Object Reference") (OtherActor :type "Actor Object Reference") (OtherComp :type "PrimitiveComponent Object Reference") (OtherBodyIndex :type Integer))
  (`SceneComponent.SetVisibility` (`self.Widget`) false false))

(event `/Game/_Mechanics/BPI_MainInteract.LookAt`
  (`MovementComponent.StopMovementImmediately` (`Character.CharacterMovement` (`GameplayStatics.GetPlayerCharacter` 0)))
  (bind _output_get (set `self.Time` (+ (`self.Time`) (`GameplayStatics.GetWorldDeltaSeconds`))))
  (if (> _output_get (`self.TimeToBuild`))
    (bind _p_smoke_d (`self.P_Smoke_D`)
      (:`then`
        (`ActorComponent.K2_DestroyComponent` _p_smoke_d)
        (`self.RemoveBoxCollider`))
      (:`else`))
    (else
      (`|ExecutionSequence`
        (:`then_0`
          (`WidgetComponent.SetWidget` (`self.Widget`) (`self.HUD ProgressBar`))
          (`/Game/_Layout/HUD/Content/Fix/WB_RepairingBar.SetPercent` (`self.HUD ProgressBar`) (`self.Time`) (`self.TimeToBuild`)))
        (:`then_1`
          (`self.Animation`))))))

(event `/Game/_Mechanics/BPI_MainInteract.Cancel`
  (set `self.Time` 0.0)
  (`WidgetComponent.SetWidget` (`self.Widget`) (`self.HUD Interaction`))
  (`/Game/_Layout/HUD/Content/Fix/WB_RepairingBar.SetPercent` (`self.HUD ProgressBar`) 0.0 (`self.TimeToBuild`))
  (`Character.StopAnimMontage` (`GameplayStatics.GetPlayerCharacter` 0) (`self.Fix Montage`)))

(event `RemoveBoxCollider`
  (`/Engine/EditorBlueprintResources/StandardMacros.DoOnce` false
    (:`Completed`
      (bind _box (`self.Box`)
        (:`then`
          (`PrimitiveComponent.SetCollisionEnabled` _box "NoCollision"))
        (:`else`)))))

(event `Animation`
  (`/Engine/EditorBlueprintResources/StandardMacros.DoOnce` false :!label _label
    (:`Completed`
      (`|PlayMontage` (`Character.Mesh` (`GameplayStatics.GetPlayerCharacter` 0)) (`self.Fix Montage`)
        (:`OnCompleted`
          (goto _label :!via `Reset`))))))

(fn `Interact With`
  (returns (ObjectiveID :type String))
  (bind _objective_id (`self.Objective ID`))
  (`KismetSystemLibrary.PrintString` _objective_id true true (struct :`G` 0.66 :`B` 1.0 :`A` 1.0) 0.0)
  (return _objective_id))

(fn `IsMoving`
  (returns (`isMoving?` :type Boolean))
  (return (> (`KismetMathLibrary.VSize` (`self.GetVelocity` (`GameplayStatics.GetPlayerCharacter` 0))) 0.0)))

(fn `UserConstructionScript`)