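; Dialogue component for the NPC Karen, extending a parent component to play her conversation for the current game progress.
; It builds speaker and line arrays from DT_KarenDialogues rows matching the GameInstance's progress, plus a looping line from the next stage.
; Dialogue refreshes stale arrays, steps through lines, then closes, updates progress or rebuilds, and sets RestorationLevel as next map.
; DisplayQuest separately shows a quest log widget from QuestData.
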(event `self.ReceiveBeginPlay`
  (bind _asbpi_game_instance (cast `/Game/_Mechanics/SaveGame/BPI_GameInstance` (`GameplayStatics.GetGameInstance`)))
  (set `self.As BPI Game Instance_0` _asbpi_game_instance)
  (`self.GenerateDialogArray`))

(fn `Dialogue`
  (locals (NewLocalVar :type Text :default "NSLOCTEXT(\"\", \"F8E967A34154A8D7A307B19FB19652CE\", \"KAREN\")"))
  (bind _gameprogresstoset (`self.GameProgressToSet`))
  (bind _dialogueindex (`self.DialogueIndex`))
  (bind _as_bpi_game_instance_0 (`self.As BPI Game Instance_0`))
  (bind _convoloop (`self.ConvoLoop`))
  ;[1 1 1] Reorganizar
  (`parent.Dialogue`)
  (bind _progress (`/Game/_Mechanics/SaveGame/BPI_GameInstance.GetGameProgress` (`self.As BPI Game Instance_0`)))
  (if (<= (`self.GameProgressToSet`) _progress)
    (`self.ClearConversation`)
    (`self.GenerateDialogArray`))
  (if (!= (`KismetArrayLibrary.Array_Length` (`self.Conversation_Speaker`)) (+ _dialogueindex 1)) :!label _label
    (bind (_speaker _dialogue) (`self.ReturnLineAddDialog` _dialogueindex))
    (bind _state (`self.AddDialogue` _speaker _dialogue))
    (switch `/Game/_Mechanics/DialogueSystem/E_DialogueState` _state
      (:`NewEnumerator0`
        (goto _label)))
    (else
      (if (not (or (`KismetTextLibrary.EqualEqual_TextText` _dialogue _convoloop) (`KismetTextLibrary.TextIsEmpty` _convoloop)))
        (bind _state_2 (`self.AddDialogue` "KAREN" _convoloop))
        (switch `/Game/_Mechanics/DialogueSystem/E_DialogueState` _state_2
          (:`NewEnumerator0`
            _)))
      (`self.SetDialogueTreeIndex` true)
      (`self.CloseConversation`)
      (bind _progress_2 (`/Game/_Mechanics/SaveGame/BPI_GameInstance.GetGameProgress` _as_bpi_game_instance_0))
      (if (<= _progress_2 _gameprogresstoset)
        (`/Game/_Mechanics/SaveGame/BPI_GameInstance.SetNewProgress` _as_bpi_game_instance_0 _gameprogresstoset)
        (else
          (`self.GenerateDialogArray`)))
      (`/Game/_Mechanics/SaveGame/BPI_GameInstance.SetNextMap` _as_bpi_game_instance_0 "RestorationLevel"))))

(fn `DisplayQuest`
  (bind (_questdata_datatable _questdata_rowname) (break `DataTableRowHandle` (`self.QuestData`)))
  (bind _returnvalue (`|GetDataTableRow` _questdata_datatable _questdata_rowname)
    (:`then`
      (bind _returnvalue_2 (`|CreateWidget` "/Game/_Layout/HUD/Content/Quest/WB_QuestLog.WB_QuestLog_C" null _returnvalue _questdata_rowname))
      (`UserWidget.AddToViewport` _returnvalue_2 0))))

(fn `GenerateDialogArray`
  (`parent.GenerateDialogArray`)
  (bind _progress (`/Game/_Mechanics/SaveGame/BPI_GameInstance.GetGameProgress` (`self.As BPI Game Instance_0`)))
  (bind _outrownames (`DataTableFunctionLibrary.GetDataTableRowNames` "/Game/_Mechanics/DataDialogSystem/DT_KarenDialogues.DT_KarenDialogues"))
  (for _array_element _outrownames
    (bind _returnvalue (`|GetDataTableRow` "/Game/_Mechanics/DataDialogSystem/DT_KarenDialogues.DT_KarenDialogues" _array_element)
      (:`then`
        (bind (_gameprogress _chatprogress _speaker _dialogue _ischatloop) (break `/Game/_Mechanics/DataDialogSystem/E_DialogStruct` _returnvalue))
        (if (== _progress _gameprogress)
          (`KismetArrayLibrary.Array_Add` (`self.Conversation_Speaker`) _speaker)
          (`KismetArrayLibrary.Array_Add` (`self.Conversation_Dialogue`) _dialogue)
          (else
            (bind _returnvalue_2 (+ _progress 1))
            (if (and _ischatloop (== _gameprogress _returnvalue_2))
              (set `self.ConvoLoop` _dialogue)
              (set `self.GameProgressToSet` _returnvalue_2))))))))

(fn `Interact With`
  (returns (ObjectiveID :type String))
  (return "KAREN"))

(fn `ReturnLineAddDialog`
  (params (DialogueIndex :type Integer))
  (returns (Speaker :type Text) (Dialogue :type Text))
  (bind _returnvalue (+ DialogueIndex 1))
  (return (`|GetArrayItem` (`self.Conversation_Speaker`) _returnvalue) (`|GetArrayItem` (`self.Conversation_Dialogue`) _returnvalue)))

(fn `toName (int)`
  (params (InInt :type Integer))
  (returns (ReturnValue :type Name))
  (return (`KismetStringLibrary.Conv_StringToName` (`KismetStringLibrary.Conv_IntToString` InInt))))