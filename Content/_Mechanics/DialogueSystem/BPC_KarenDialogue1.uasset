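; Dialogue component for the NPC Karen, holding her story conversations with Clide and identifying her for interaction.
; Dialogue reads the tree index from the Slot01 save and plays the matching linear chain of lines, then updates the index and closes.
; Some trees wait on GameInstance flags (power, tree, table), otherwise playing a reminder and rolling back progress.
; Key endings set mission progress, toggle interactables or set the next map through BPI_GameInstance.
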(event `self.ReceiveBeginPlay`
  (bind _asbpi_game_instance (cast `/Game/_Mechanics/SaveGame/BPI_GameInstance` (`GameplayStatics.GetGameInstance`)))
  (set `self.As BPI Game Instance` _asbpi_game_instance))

(fn `Dialogue`
  (locals (NewLocalVar :type Text :default "NSLOCTEXT(\"\", \"F8E967A34154A8D7A307B19FB19652CE\", \"KAREN\")"))
  (bind _as_bpi_game_instance (`self.As BPI Game Instance`))
  (bind _as_bpi_game_instance_2 (`self.As BPI Game Instance`))
  (`parent.Dialogue`)
  (bind _returnvalue (`GameplayStatics.LoadGameFromSlot` "Slot01"))
  (bind _asbsg_game_save (cast `/Game/_Mechanics/SaveGame/BSG_GameSave` _returnvalue))
  (bind _dialogueindexsaved (`/Game/_Mechanics/SaveGame/BSG_GameSave.DialogueIndexSaved` _asbsg_game_save))
  (switch `int` _dialogueindexsaved
    (:`0`
      ;[1 1 1] First Dialogue Tree
      (bind _state (`self.AddDialogue` "KAREN" "Don't worry, mate. They can't reach us here." (`|MakeArray` "..." :!type "Text")))
      (switch `/Game/_Mechanics/DialogueSystem/E_DialogueState` _state
        (:`NewEnumerator0`
          (bind _state_2 (`self.AddDialogue` "CLIDE" "What happened here? Why is everyone  acting like... Living dead?" (`|MakeArray` "..." :!type "Text")))
          (switch `/Game/_Mechanics/DialogueSystem/E_DialogueState` _state_2
            (:`NewEnumerator0`
              (bind _state_3 (`self.AddDialogue` "KAREN" "It all went down so fast. In two weeks we lost contact with the outside and the city went through martial law. " (`|MakeArray` "..." :!type "Text")))
              (switch `/Game/_Mechanics/DialogueSystem/E_DialogueState` _state_3
                (:`NewEnumerator0`
                  (bind _state_4 (`self.AddDialogue` "KAREN" "Now, mate, you tell me... Who are you and why are you here?" (`|MakeArray` "..." :!type "Text")))
                  (switch `/Game/_Mechanics/DialogueSystem/E_DialogueState` _state_4
                    (:`NewEnumerator0`
                      (bind _state_5 (`self.AddDialogue` "CLIDE" "I'm Clide. Restoration Agent sent by ERA." (`|MakeArray` "..." :!type "Text")))
                      (switch `/Game/_Mechanics/DialogueSystem/E_DialogueState` _state_5
                        (:`NewEnumerator0`
                          (bind _state_6 (`self.AddDialogue` "CLIDE" "They sent me here to restore the city's environment, but no one briefed me about \"Campasa!\"" (`|MakeArray` "..." :!type "Text")))
                          (switch `/Game/_Mechanics/DialogueSystem/E_DialogueState` _state_6
                            (:`NewEnumerator0`
                              (bind _state_7 (`self.AddDialogue` "KAREN" "They left you out of the details... To restore this, you gotta make it alive first. Name's Karen, by the way." (`|MakeArray` "..." :!type "Text")))
                              (switch `/Game/_Mechanics/DialogueSystem/E_DialogueState` _state_7
                                (:`NewEnumerator0`
                                  (`self.SetDialogueTreeIndex` false)
                                  (`self.CloseConversation`))))))))))))))))
    (:`1`
      (bind _state_8 (`self.AddDialogue` "CLIDE" "What is this place?" (`|MakeArray` "..." :!type "Text")))
      (switch `/Game/_Mechanics/DialogueSystem/E_DialogueState` _state_8
        (:`NewEnumerator0`
          (bind _state_9 (`self.AddDialogue` "KAREN" "This is North Athens' Botanical Garden. It's open for visitation. And it fits you well, tree huggers." (`|MakeArray` "..." :!type "Text")))
          (switch `/Game/_Mechanics/DialogueSystem/E_DialogueState` _state_9
            (:`NewEnumerator0`
              (bind _state_10 (`self.AddDialogue` "CLIDE" "We don't hug trees. We just can´t live without them." (`|MakeArray` "..." :!type "Text")))
              (switch `/Game/_Mechanics/DialogueSystem/E_DialogueState` _state_10
                (:`NewEnumerator0`
                  (bind _state_11 (`self.AddDialogue` "KAREN" "If you told me this before, I would laugh till I drop, mate. But I'm here, and I'm still not one of them." (`|MakeArray` "..." :!type "Text")))
                  (switch `/Game/_Mechanics/DialogueSystem/E_DialogueState` _state_11
                    (:`NewEnumerator0`
                      (bind _state_12 (`self.AddDialogue` "CLIDE" "Why didn't you run like the others?" (`|MakeArray` "..." :!type "Text")))
                      (switch `/Game/_Mechanics/DialogueSystem/E_DialogueState` _state_12
                        (:`NewEnumerator0`
                          (bind _state_13 (`self.AddDialogue` "KAREN" "Have you seen the situation out there? Where to run? It's like the city's a hell of a trap with no way in or out. " (`|MakeArray` "..." :!type "Text")))
                          (switch `/Game/_Mechanics/DialogueSystem/E_DialogueState` _state_13
                            (:`NewEnumerator0`
                              (bind _state_14 (`self.AddDialogue` "KAREN" "What do you suggest, spreading wings and fly away? Before or after suffocating over the smoke?" (`|MakeArray` "..." :!type "Text")))
                              (switch `/Game/_Mechanics/DialogueSystem/E_DialogueState` _state_14
                                (:`NewEnumerator0`
                                  (`self.SetDialogueTreeIndex` false)
                                  (`self.CloseConversation`))))))))))))))))
    (:`2`
      (bind _state_15 (`self.AddDialogue` "KAREN" "Hmph..." (`|MakeArray` "..." :!type "Text")))
      (switch `/Game/_Mechanics/DialogueSystem/E_DialogueState` _state_15
        (:`NewEnumerator0`
          (bind _state_16 (`self.AddDialogue` "CLIDE" "You okay? I saw you limping back there. Are you in pain?" (`|MakeArray` "..." :!type "Text")))
          (switch `/Game/_Mechanics/DialogueSystem/E_DialogueState` _state_16
            (:`NewEnumerator0`
              (bind _state_17 (`self.AddDialogue` "KAREN" "Yeah. I missteped after I pushed that zombie away from you." (`|MakeArray` "..." :!type "Text")))
              (switch `/Game/_Mechanics/DialogueSystem/E_DialogueState` _state_17
                (:`NewEnumerator0`
                  (bind _state_18 (`self.AddDialogue` "CLIDE" "You got hurt because of me? Really? I'm sorry, Karen." (`|MakeArray` "..." :!type "Text")))
                  (switch `/Game/_Mechanics/DialogueSystem/E_DialogueState` _state_18
                    (:`NewEnumerator0`
                      (bind _state_19 (`self.AddDialogue` "KAREN" "You owe me, green thumbs. Big pain, so big time. " (`|MakeArray` "..." :!type "Text")))
                      (switch `/Game/_Mechanics/DialogueSystem/E_DialogueState` _state_19
                        (:`NewEnumerator0`
                          (bind _state_20 (`self.AddDialogue` "CLIDE" "Do you need something? Perhaps some ice, painkillers?" (`|MakeArray` "..." :!type "Text")))
                          (switch `/Game/_Mechanics/DialogueSystem/E_DialogueState` _state_20
                            (:`NewEnumerator0`
                              (bind _state_21 (`self.AddDialogue` "KAREN" "All the supplies I need are locked inside the Haven." (`|MakeArray` "..." :!type "Text")))
                              (switch `/Game/_Mechanics/DialogueSystem/E_DialogueState` _state_21
                                (:`NewEnumerator0`
                                  (bind _state_22 (`self.AddDialogue` "KAREN" "I'll have my painkillers once the power's back again." (`|MakeArray` "..." :!type "Text")))
                                  (switch `/Game/_Mechanics/DialogueSystem/E_DialogueState` _state_22
                                    (:`NewEnumerator0`
                                      (`self.SetDialogueTreeIndex` false)
                                      (`self.CloseConversation`))))))))))))))))))
    (:`3`
      (bind _state_23 (`self.AddDialogue` "CLIDE" "You can't do too much with this leg of yours. What can I do to help?" (`|MakeArray` "..." :!type "Text")))
      (switch `/Game/_Mechanics/DialogueSystem/E_DialogueState` _state_23
        (:`NewEnumerator0`
          (bind _state_24 (`self.AddDialogue` "KAREN" "Ohh, now we're talking. You're gonna do \"Limping Karen\" a great favor." (`|MakeArray` "..." :!type "Text")))
          (switch `/Game/_Mechanics/DialogueSystem/E_DialogueState` _state_24
            (:`NewEnumerator0`
              (bind _state_25 (`self.AddDialogue` "KAREN" "I need to recover from this injury, and all my supplies are inside the Haven dome. But it's out of power." (`|MakeArray` "..." :!type "Text")))
              (switch `/Game/_Mechanics/DialogueSystem/E_DialogueState` _state_25
                (:`NewEnumerator0`
                  (bind _state_26 (`self.AddDialogue` "KAREN" "I was on my way to restore the power in the station before I tried that hero stunt. But now I'm a mess and I need you to do this for me." (`|MakeArray` "..." :!type "Text")))
                  (switch `/Game/_Mechanics/DialogueSystem/E_DialogueState` _state_26
                    (:`NewEnumerator0`
                      (bind _state_27 (`self.AddDialogue` "KAREN" "It's not hard, I'll go over the instructions through the radio. But you have to do it quick." (`|MakeArray` "..." :!type "Text")))
                      (switch `/Game/_Mechanics/DialogueSystem/E_DialogueState` _state_27
                        (:`NewEnumerator0`
                          (bind _state_28 (`self.AddDialogue` "CLIDE" "Zombies are slow, I can deal with them." (`|MakeArray` "..." :!type "Text")))
                          (switch `/Game/_Mechanics/DialogueSystem/E_DialogueState` _state_28
                            (:`NewEnumerator0`
                              (bind _state_29 (`self.AddDialogue` "KAREN" "It's not that, Clide. You should not be outside in the night." (`|MakeArray` "..." :!type "Text")))
                              (switch `/Game/_Mechanics/DialogueSystem/E_DialogueState` _state_29
                                (:`NewEnumerator0`
                                  (bind _state_30 (`self.AddDialogue` "KAREN" "Don't ask me why, but the smoke's thicker when the sun's out." (`|MakeArray` "..." :!type "Text")))
                                  (switch `/Game/_Mechanics/DialogueSystem/E_DialogueState` _state_30
                                    (:`NewEnumerator0`
                                      (bind _state_31 (`self.AddDialogue` "KAREN" "You'll cough until you die, so be quick." (`|MakeArray` "..." :!type "Text")))
                                      (switch `/Game/_Mechanics/DialogueSystem/E_DialogueState` _state_31
                                        (:`NewEnumerator0`
                                          (bind _state_32 (`self.AddDialogue` "KAREN" "I'm counting on you, mate." (`|MakeArray` "..." :!type "Text")))
                                          (switch `/Game/_Mechanics/DialogueSystem/E_DialogueState` _state_32
                                            (:`NewEnumerator0`
                                              (`self.SetDialogueTreeIndex` false)
                                              (`self.CloseConversation`)
                                              (`/Game/_Mechanics/SaveGame/BPI_GameInstance.SetNewProgress` _as_bpi_game_instance 3)
                                              (`/Game/_Mechanics/SaveGame/BPI_GameInstance.SetNextMap` _as_bpi_game_instance "RestorationLevel"))))))))))))))))))))))
    (:`4`
      (bind _electricitystatus (`/Game/_Mechanics/SaveGame/BPI_GameInstance.GetElectricityStatus` (`self.As BPI Game Instance`)))
      (if _electricitystatus
        ;[1 1 1] Comment
        (set `self.DialogueTreeIndex` _dialogueindexsaved)
        (bind _state_33 (`self.AddDialogue` "KAREN" "Hey, mate! You did it, we have power! Thank you!" (`|MakeArray` "..." :!type "Text")))
        (switch `/Game/_Mechanics/DialogueSystem/E_DialogueState` _state_33
          (:`NewEnumerator0`
            (bind _state_34 (`self.AddDialogue` "CLIDE" "No problem, Karen. I'm glad so we won't spend the night in the dark." (`|MakeArray` "..." :!type "Text")))
            (switch `/Game/_Mechanics/DialogueSystem/E_DialogueState` _state_34
              (:`NewEnumerator0`
                (bind _state_35 (`self.AddDialogue` "CLIDE" "So, mind telling me how did you survive until now? All by yourself?" (`|MakeArray` "..." :!type "Text")))
                (switch `/Game/_Mechanics/DialogueSystem/E_DialogueState` _state_35
                  (:`NewEnumerator0`
                    (bind _state_36 (`self.AddDialogue` "KAREN" "I was a cop in North Athens. Before I could act as a cop, however, they put me here as the garden keeper." (`|MakeArray` "..." :!type "Text")))
                    (switch `/Game/_Mechanics/DialogueSystem/E_DialogueState` _state_36
                      (:`NewEnumerator0`
                        (bind _state_37 (`self.AddDialogue` "KAREN" "I didn't mind; Good money, easy job." (`|MakeArray` "..." :!type "Text")))
                        (switch `/Game/_Mechanics/DialogueSystem/E_DialogueState` _state_37
                          (:`NewEnumerator0`
                            (bind _state_38 (`self.AddDialogue` "CLIDE" "So the \"zombocalypse\" happened." (`|MakeArray` "..." :!type "Text")))
                            (switch `/Game/_Mechanics/DialogueSystem/E_DialogueState` _state_38
                              (:`NewEnumerator0`
                                (bind _state_39 (`self.AddDialogue` "KAREN" "You got it, mate. I was lucky the Haven walls were sturdy. They kept the living dead in the outside." (`|MakeArray` "..." :!type "Text")))
                                (switch `/Game/_Mechanics/DialogueSystem/E_DialogueState` _state_39
                                  (:`NewEnumerator0`
                                    (`self.SetDialogueTreeIndex` false)
                                    (`self.CloseConversation`)))))))))))))))
        (else
          (bind _state_40 (`self.AddDialogue` "KAREN" "Tell me when you're on the spot. I'll help you with the Power Panel." (`|MakeArray` "..." :!type "Text")))
          (switch `/Game/_Mechanics/DialogueSystem/E_DialogueState` _state_40
            (:`NewEnumerator0`
              (`self.RemoveDialogueProgress` 1)
              (`self.CloseConversation`))))))
    (:`5`
      (bind _state_41 (`self.AddDialogue` "CLIDE" "You said something about the smoke." (`|MakeArray` "..." :!type "Text")))
      (switch `/Game/_Mechanics/DialogueSystem/E_DialogueState` _state_41
        (:`NewEnumerator0`
          (bind _state_42 (`self.AddDialogue` "KAREN" "Yeah. Goddamn businessmen! They wiped out every tree they could to build those stupid business towers." (`|MakeArray` "..." :!type "Text")))
          (switch `/Game/_Mechanics/DialogueSystem/E_DialogueState` _state_42
            (:`NewEnumerator0`
              (bind _state_43 (`self.AddDialogue` "CLIDE" "And to think that North Athens was a model city... Well, nothing money can't handle." (`|MakeArray` "..." :!type "Text")))
              (switch `/Game/_Mechanics/DialogueSystem/E_DialogueState` _state_43
                (:`NewEnumerator0`
                  (bind _state_44 (`self.AddDialogue` "KAREN" "We can barely see a living tree around here!" (`|MakeArray` "..." :!type "Text")))
                  (switch `/Game/_Mechanics/DialogueSystem/E_DialogueState` _state_44
                    (:`NewEnumerator0`
                      (bind _state_45 (`self.AddDialogue` "KAREN" "I skipped biology classes but I'm sure the air would be better if we had more trees like the great one over there." (`|MakeArray` "..." :!type "Text")))
                      (switch `/Game/_Mechanics/DialogueSystem/E_DialogueState` _state_45
                        (:`NewEnumerator0`
                          (bind _state_46 (`self.AddDialogue` "CLIDE" "I'd like to take a look in this tree of yours, If you don't mind." (`|MakeArray` "..." :!type "Text")))
                          (switch `/Game/_Mechanics/DialogueSystem/E_DialogueState` _state_46
                            (:`NewEnumerator0`
                              (bind _state_47 (`self.AddDialogue` "KAREN" "Be my guest. It's the giant elephant in the middle of the room." (`|MakeArray` "..." :!type "Text")))
                              (switch `/Game/_Mechanics/DialogueSystem/E_DialogueState` _state_47
                                (:`NewEnumerator0`
                                  (`self.SetDialogueTreeIndex` false)
                                  (`self.CloseConversation`)
                                  ;[1 0.05177 0] New Mission
                                  (`/Game/_Mechanics/SaveGame/BPI_GameInstance.SetNewProgress` (`self.As BPI Game Instance`) 6)
                                  (`/Game/_Mechanics/SaveGame/BPI_GameInstance.Toggle Tree` (`self.As BPI Game Instance`) true))))))))))))))))
    (:`6`
      (bind _treeinteracted (`/Game/_Mechanics/SaveGame/BPI_GameInstance.GetTreeInteraction` (`self.As BPI Game Instance`)))
      (if _treeinteracted
        ;[1 1 1] Comment
        (set `self.DialogueTreeIndex` _dialogueindexsaved)
        (bind _state_48 (`self.AddDialogue` "CLIDE" "Karen, I need to ask you something." (`|MakeArray` "..." :!type "Text")))
        (switch `/Game/_Mechanics/DialogueSystem/E_DialogueState` _state_48
          (:`NewEnumerator0`
            (bind _state_49 (`self.AddDialogue` "CLIDE" "The city had a breakdown before going into martial law, right?" (`|MakeArray` "..." :!type "Text")))
            (switch `/Game/_Mechanics/DialogueSystem/E_DialogueState` _state_49
              (:`NewEnumerator0`
                (bind _state_50 (`self.AddDialogue` "KAREN" "Yeah. Hospitals went crazy. People couldn't breathe, smoke everywhere." (`|MakeArray` "..." :!type "Text")))
                (switch `/Game/_Mechanics/DialogueSystem/E_DialogueState` _state_50
                  (:`NewEnumerator0`
                    (bind _state_51 (`self.AddDialogue` "KAREN" "The sick went to emergency and died in the spot." (`|MakeArray` "..." :!type "Text")))
                    (switch `/Game/_Mechanics/DialogueSystem/E_DialogueState` _state_51
                      (:`NewEnumerator0`
                        (bind _state_52 (`self.AddDialogue` "KAREN" "The health system was not ready to deal with so many sick people with breathing issues at the same time." (`|MakeArray` "..." :!type "Text")))
                        (switch `/Game/_Mechanics/DialogueSystem/E_DialogueState` _state_52
                          (:`NewEnumerator0`
                            (bind _state_53 (`self.AddDialogue` "KAREN" "And the worst was yet to come: deal with their beloved ones coming back from the dead as... Those monsters." (`|MakeArray` "..." :!type "Text")))
                            (switch `/Game/_Mechanics/DialogueSystem/E_DialogueState` _state_53
                              (:`NewEnumerator0`
                                (bind _state_54 (`self.AddDialogue` "CLIDE" "So, you're telling me people died because of inhaling the city's impure air." (`|MakeArray` "..." :!type "Text")))
                                (switch `/Game/_Mechanics/DialogueSystem/E_DialogueState` _state_54
                                  (:`NewEnumerator0`
                                    (bind _state_55 (`self.AddDialogue` "KAREN" "Seems like it." (`|MakeArray` "..." :!type "Text")))
                                    (switch `/Game/_Mechanics/DialogueSystem/E_DialogueState` _state_55
                                      (:`NewEnumerator0`
                                        (`self.SetDialogueTreeIndex` false)
                                        (`self.CloseConversation`)))))))))))))))))
        (else
          (bind _state_56 (`self.AddDialogue` "KAREN" "Checked your tree, green thumbs?" (`|MakeArray` "..." :!type "Text")))
          (switch `/Game/_Mechanics/DialogueSystem/E_DialogueState` _state_56
            (:`NewEnumerator0`
              (`self.RemoveDialogueProgress` 1)
              (`self.CloseConversation`)
              (`/Game/_Mechanics/SaveGame/BPI_GameInstance.Toggle Tree` (`self.As BPI Game Instance`) true))))))
    (:`7`
      (bind _state_57 (`self.AddDialogue` "CLIDE" "What about you? Where were you when it all started?" (`|MakeArray` "..." :!type "Text")))
      (switch `/Game/_Mechanics/DialogueSystem/E_DialogueState` _state_57
        (:`NewEnumerator0`
          (bind _state_58 (`self.AddDialogue` "KAREN" "I tried to shelter everyone over here, but who would stay in a place full of plants?" (`|MakeArray` "..." :!type "Text")))
          (switch `/Game/_Mechanics/DialogueSystem/E_DialogueState` _state_58
            (:`NewEnumerator0`
              (bind _state_59 (`self.AddDialogue` "CLIDE" "Everyone who wanted to stay alive, apparently." (`|MakeArray` "..." :!type "Text")))
              (switch `/Game/_Mechanics/DialogueSystem/E_DialogueState` _state_59
                (:`NewEnumerator0`
                  (bind _state_60 (`self.AddDialogue` "KAREN" "How come, mate?" (`|MakeArray` "..." :!type "Text")))
                  (switch `/Game/_Mechanics/DialogueSystem/E_DialogueState` _state_60
                    (:`NewEnumerator0`
                      (bind _state_61 (`self.AddDialogue` "CLIDE" "You haven't left the place for long periods, right?" (`|MakeArray` "..." :!type "Text")))
                      (switch `/Game/_Mechanics/DialogueSystem/E_DialogueState` _state_61
                        (:`NewEnumerator0`
                          (bind _state_62 (`self.AddDialogue` "KAREN" "Well, yeah... I only brought food whenever I could. The place has sturdy walls, water, energy..." (`|MakeArray` "..." :!type "Text")))
                          (switch `/Game/_Mechanics/DialogueSystem/E_DialogueState` _state_62
                            (:`NewEnumerator0`
                              (bind _state_63 (`self.AddDialogue` "CLIDE" "And a huge air purifier." (`|MakeArray` "..." :!type "Text")))
                              (switch `/Game/_Mechanics/DialogueSystem/E_DialogueState` _state_63
                                (:`NewEnumerator0`
                                  (bind _state_64 (`self.AddDialogue` "CLIDE" "Tell me, you didn't get sick, did you?" (`|MakeArray` "..." :!type "Text")))
                                  (switch `/Game/_Mechanics/DialogueSystem/E_DialogueState` _state_64
                                    (:`NewEnumerator0`
                                      (bind _state_65 (`self.AddDialogue` "KAREN" "Well... no. How do you know? You're supposed to be the green thumb only.  " (`|MakeArray` "..." :!type "Text")))
                                      (switch `/Game/_Mechanics/DialogueSystem/E_DialogueState` _state_65
                                        (:`NewEnumerator0`
                                          (bind _state_66 (`self.AddDialogue` "KAREN" "Part-time fortune teller?" (`|MakeArray` "..." :!type "Text")))
                                          (switch `/Game/_Mechanics/DialogueSystem/E_DialogueState` _state_66
                                            (:`NewEnumerator0`
                                              (bind _state_67 (`self.AddDialogue` "CLIDE" "You wish. I'm happy to be the green thumb, or you wouldn't figure it out why you're not sick as them." (`|MakeArray` "..." :!type "Text")))
                                              (switch `/Game/_Mechanics/DialogueSystem/E_DialogueState` _state_67
                                                (:`NewEnumerator0`
                                                  (bind _state_68 (`self.AddDialogue` "CLIDE" "The tree's dissipating the smoke around this place, making it an infection-free safe haven." (`|MakeArray` "..." :!type "Text")))
                                                  (switch `/Game/_Mechanics/DialogueSystem/E_DialogueState` _state_68
                                                    (:`NewEnumerator0`
                                                      (bind _state_69 (`self.AddDialogue` "KAREN" "Are you telling me the reason I'm still alive is because I remained here?" (`|MakeArray` "..." :!type "Text")))
                                                      (switch `/Game/_Mechanics/DialogueSystem/E_DialogueState` _state_69
                                                        (:`NewEnumerator0`
                                                          (bind _state_70 (`self.AddDialogue` "CLIDE" "No, but you're been able to breathe because of this wise choice of yours." (`|MakeArray` "..." :!type "Text")))
                                                          (switch `/Game/_Mechanics/DialogueSystem/E_DialogueState` _state_70
                                                            (:`NewEnumerator0`
                                                              (`self.SetDialogueTreeIndex` false)
                                                              (`self.CloseConversation`))))))))))))))))))))))))))))))
    (:`8`
      (bind _state_71 (`self.AddDialogue` "CLIDE" "This tree's been around since..." (`|MakeArray` "..." :!type "Text")))
      (switch `/Game/_Mechanics/DialogueSystem/E_DialogueState` _state_71
        (:`NewEnumerator0`
          (bind _state_72 (`self.AddDialogue` "KAREN" "Since the town was built. They had a plan to grow more of them around the city, but they had another priorities." (`|MakeArray` "..." :!type "Text")))
          (switch `/Game/_Mechanics/DialogueSystem/E_DialogueState` _state_72
            (:`NewEnumerator0`
              (bind _state_73 (`self.AddDialogue` "KAREN" "They brought some saplings, but were never used. It's on the table over there." (`|MakeArray` "..." :!type "Text")))
              (switch `/Game/_Mechanics/DialogueSystem/E_DialogueState` _state_73
                (:`NewEnumerator0`
                  (bind _state_74 (`self.AddDialogue` "KAREN" "See if you can use your magic, green thumbs." (`|MakeArray` "..." :!type "Text")))
                  (switch `/Game/_Mechanics/DialogueSystem/E_DialogueState` _state_74
                    (:`NewEnumerator0`
                      (`self.SetDialogueTreeIndex` false)
                      (`self.CloseConversation`)
                      ;;[1 0.05177 0] New Mission
                      (`/Game/_Mechanics/SaveGame/BPI_GameInstance.SetNewProgress` _as_bpi_game_instance_2 8)
                      (`/Game/_Mechanics/SaveGame/BPI_GameInstance.Toggle Table` _as_bpi_game_instance_2 true))))))))))
    (:`9`
      (bind _tableinteracted (`/Game/_Mechanics/SaveGame/BPI_GameInstance.GetTableInteraction` (`self.As BPI Game Instance`)))
      (if _tableinteracted
        ;[1 1 1] Comment
        (set `self.DialogueTreeIndex` _dialogueindexsaved)
        (bind _state_75 (`self.AddDialogue` "CLIDE" "You said something about this plan of growing trees." (`|MakeArray` "..." :!type "Text")))
        (switch `/Game/_Mechanics/DialogueSystem/E_DialogueState` _state_75
          (:`NewEnumerator0`
            (bind _state_76 (`self.AddDialogue` "KAREN" "Yeah, they built some crop plots around the city. The nearest one's in the Downtown Square." (`|MakeArray` "..." :!type "Text")))
            (switch `/Game/_Mechanics/DialogueSystem/E_DialogueState` _state_76
              (:`NewEnumerator0`
                (bind _state_77 (`self.AddDialogue` "CLIDE" "I want to try and go on with the tree plan." (`|MakeArray` "..." :!type "Text")))
                (switch `/Game/_Mechanics/DialogueSystem/E_DialogueState` _state_77
                  (:`NewEnumerator0`
                    (bind _state_78 (`self.AddDialogue` "KAREN" "What? Mate, you're definitely crazy. Get a mask, you had too much smoke for the day." (`|MakeArray` "..." :!type "Text")))
                    (switch `/Game/_Mechanics/DialogueSystem/E_DialogueState` _state_78
                      (:`NewEnumerator0`
                        (bind _state_79 (`self.AddDialogue` "CLIDE" "No, Karen, hear me out. We're aware that the smoke's responsible for everything around here." (`|MakeArray` "..." :!type "Text")))
                        (switch `/Game/_Mechanics/DialogueSystem/E_DialogueState` _state_79
                          (:`NewEnumerator0`
                            (bind _state_80 (`self.AddDialogue` "CLIDE" "This tree has the power to drive away the smoke." (`|MakeArray` "..." :!type "Text")))
                            (switch `/Game/_Mechanics/DialogueSystem/E_DialogueState` _state_80
                              (:`NewEnumerator0`
                                (bind _state_81 (`self.AddDialogue` "CLIDE" "If I take some of those saplings, I'm positive we'll get rid of the smoke responsible for taking down so many lives." (`|MakeArray` "..." :!type "Text")))
                                (switch `/Game/_Mechanics/DialogueSystem/E_DialogueState` _state_81
                                  (:`NewEnumerator0`
                                    (bind _state_82 (`self.AddDialogue` "KAREN" "Green thumbs, I'll not help you to become zombie food." (`|MakeArray` "..." :!type "Text")))
                                    (switch `/Game/_Mechanics/DialogueSystem/E_DialogueState` _state_82
                                      (:`NewEnumerator0`
                                        (bind _state_83 (`self.AddDialogue` "CLIDE" "With this ankle of yours? Barely. I can do this on my own, Karen." (`|MakeArray` "..." :!type "Text")))
                                        (switch `/Game/_Mechanics/DialogueSystem/E_DialogueState` _state_83
                                          (:`NewEnumerator0`
                                            (bind _state_84 (`self.AddDialogue` "CLIDE" "I just need some ammo, those plants and..." (`|MakeArray` "..." :!type "Text")))
                                            (switch `/Game/_Mechanics/DialogueSystem/E_DialogueState` _state_84
                                              (:`NewEnumerator0`
                                                (bind _state_85 (`self.AddDialogue` "KAREN" "A miracle." (`|MakeArray` "..." :!type "Text")))
                                                (switch `/Game/_Mechanics/DialogueSystem/E_DialogueState` _state_85
                                                  (:`NewEnumerator0`
                                                    (bind _state_86 (`self.AddDialogue` "CLIDE" "Such a hopeless woman." (`|MakeArray` "..." :!type "Text")))
                                                    (switch `/Game/_Mechanics/DialogueSystem/E_DialogueState` _state_86
                                                      (:`NewEnumerator0`
                                                        (bind _state_87 (`self.AddDialogue` "KAREN" "Dealing with a death wishing kid, yeah." (`|MakeArray` "..." :!type "Text")))
                                                        (switch `/Game/_Mechanics/DialogueSystem/E_DialogueState` _state_87
                                                          (:`NewEnumerator0`
                                                            (bind _state_88 (`self.AddDialogue` "KAREN" "Ok, If you want to try this stunt of yours, I'll give you some support through the radio." (`|MakeArray` "..." :!type "Text")))
                                                            (switch `/Game/_Mechanics/DialogueSystem/E_DialogueState` _state_88
                                                              (:`NewEnumerator0`
                                                                (bind _state_89 (`self.AddDialogue` "CLIDE" "Thanks, Karen. Don't worry, I'll be back in one piece." (`|MakeArray` "..." :!type "Text")))
                                                                (switch `/Game/_Mechanics/DialogueSystem/E_DialogueState` _state_89
                                                                  (:`NewEnumerator0`
                                                                    (bind _state_90 (`self.AddDialogue` "KAREN" "Just... Don't do anything reckless, green thumbs." (`|MakeArray` "..." :!type "Text")))
                                                                    (switch `/Game/_Mechanics/DialogueSystem/E_DialogueState` _state_90
                                                                      (:`NewEnumerator0`
                                                                        (`self.SetDialogueTreeIndex` false)
                                                                        (`self.CloseConversation`)
                                                                        (`/Game/_Mechanics/SaveGame/BPI_GameInstance.SetNextMap` (`self.As BPI Game Instance`) "LevelCity")))))))))))))))))))))))))))))))))
        (else
          (bind _state_91 (`self.AddDialogue` "KAREN" "Go on, botanist, cast your spells." (`|MakeArray` "..." :!type "Text")))
          (switch `/Game/_Mechanics/DialogueSystem/E_DialogueState` _state_91
            (:`NewEnumerator0`
              (`self.RemoveDialogueProgress` 1)
              (`self.CloseConversation`))))))
    (:`10`
      (bind _state_92 (`self.AddDialogue` "KAREN" "I'll be glad if you come back alive. Only alive, ok? Good luck." (`|MakeArray` "..." :!type "Text")))
      (switch `/Game/_Mechanics/DialogueSystem/E_DialogueState` _state_92
        (:`NewEnumerator0`
          (`self.SetDialogueTreeIndex` true)
          (`self.CloseConversation`)
          (`/Game/_Mechanics/SaveGame/BPI_GameInstance.SetNewProgress` (`self.As BPI Game Instance`) 10))))))

(fn `DisplayQuest`
  (bind (_questdata_datatable _questdata_rowname) (break `DataTableRowHandle` (`self.QuestData`)))
  (bind _returnvalue (`|GetDataTableRow` _questdata_datatable _questdata_rowname)
    (:`then`
      (bind _returnvalue_2 (`|CreateWidget` "/Game/_Layout/HUD/Content/Quest/WB_QuestLog.WB_QuestLog_C" null _returnvalue _questdata_rowname))
      (`UserWidget.AddToViewport` _returnvalue_2 0))))

(fn `Interact With`
  (returns (ObjectiveID :type String))
  (return "KAREN"))

(fn `toName (int)`
  (params (InInt :type Integer))
  (returns (ReturnValue :type Name))
  (return (`KismetStringLibrary.Conv_StringToName` (`KismetStringLibrary.Conv_IntToString` InInt))))