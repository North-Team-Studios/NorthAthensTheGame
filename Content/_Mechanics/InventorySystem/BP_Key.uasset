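; BP_Key is a spinning key pickup that unlocks progress on a linked Door.
; When the player overlaps its Box, it calls PickUpKey on the Door, removes the trigger and hides the mesh.
; A pop-up widget built at BeginPlay with the key name shows for three seconds before the actor destroys itself.
; Its InteractWith function returns an empty string.
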(event `self.ReceiveBeginPlay`
  (bind _returnvalue (`|CreateWidget` "/Game/_Mechanics/InventorySystem/WB_PopText1.WB_PopText1_C" null "You got:" (`self.Key Name`) "NewEnumerator1"))
  (set `self.Item PopUp` _returnvalue))

(event `self.ReceiveTick`
  (params (DeltaSeconds :type "Float (single-precision)"))
  (`SceneComponent.K2_AddRelativeRotation` (`self.StaticMesh`) (`KismetMathLibrary.MakeRotator` 0.0 0.0 -3.0) false false))

(event `self.Box.OnComponentBeginOverlap`
  (params (OverlappedComponent :type "PrimitiveComponent Object Reference") (OtherActor :type "Actor Object Reference") (OtherComp :type "PrimitiveComponent Object Reference") (OtherBodyIndex :type Integer) (bFromSweep :type Boolean) (SweepResult :type "HitResult Structure (by ref)"))
  (if (== OtherActor (`/Game/_Mechanics/QuestSystem/BPL_CommonFunctionLibrary.GetMyPlayerCharacter`))
    (`/Game/_Mechanics/InventorySystem/BPI_DoorSystem.PickUpKey` (`self.Door`))
    (`ActorComponent.K2_DestroyComponent` (`self.Box`))
    (`SceneComponent.SetVisibility` (`self.StaticMesh`) false false)
    (`self.ShowMessage`)))

(event `ShowMessage`
  (bind _item_popup (`self.Item PopUp`))
  (`UserWidget.AddToViewport` _item_popup 0)
  (`KismetSystemLibrary.Delay` 3.0)
  (`Widget.RemoveFromParent` _item_popup)
  (`self.K2_DestroyActor`))

(fn `Interact With`
  (returns (ObjectiveID :type String))
  (return ""))

(fn `UserConstructionScript`)