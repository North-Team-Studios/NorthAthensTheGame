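; BP_NarrativeArea is a trigger volume that shows a "talk to Karen" prompt on the player's HUD.
; When the player character begins overlapping the Box, it sets that title on the HUD's SafeHaven widget and flags it as collided.
; When the player leaves, it clears the title and collided flag.
; The label is hardcoded, and no dialogue or interaction logic lives here.
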(event `self.ReceiveBeginPlay`)

(event `self.Box.OnComponentBeginOverlap`
  (params (OverlappedComponent :type "PrimitiveComponent Object Reference") (OtherActor :type "Actor Object Reference") (OtherComp :type "PrimitiveComponent Object Reference") (OtherBodyIndex :type Integer) (bFromSweep :type Boolean) (SweepResult :type "HitResult Structure (by ref)"))
  (if (== OtherActor (`/Game/_Mechanics/QuestSystem/BPL_CommonFunctionLibrary.GetMyPlayerCharacter`))
    (`/Game/_Layout/HUD/GM_Huds/WB_HUDSafeHaven.Set Text and Visibility` (`.Safe Haven` (`/Game/_Mechanics/QuestSystem/BPL_CommonFunctionLibrary.GetMyHud` "NewEnumerator2")) "talk to Karen" true)))

(event `self.Box.OnComponentEndOverlap`
  (params (OverlappedComponent :type "PrimitiveComponent Object Reference") (OtherActor :type "Actor Object Reference") (OtherComp :type "PrimitiveComponent Object Reference") (OtherBodyIndex :type Integer))
  (if (== OtherActor (`/Game/_Mechanics/QuestSystem/BPL_CommonFunctionLibrary.GetMyPlayerCharacter`))
    (`/Game/_Layout/HUD/GM_Huds/WB_HUDSafeHaven.Set Text and Visibility` (`.Safe Haven` (`/Game/_Mechanics/QuestSystem/BPL_CommonFunctionLibrary.GetMyHud` "NewEnumerator2")) "" false)))

(fn `UserConstructionScript`)