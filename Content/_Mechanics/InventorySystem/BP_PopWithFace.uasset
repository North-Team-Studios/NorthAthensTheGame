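; BP_PopWithFace is a one-time trigger box that shows a pop-up dialogue widget with a face when the player enters it.
; The first overlap creates WB_PopTextWithFace with the configured speech text and passes input, action text and safe-haven settings to its tutorial command sub-widget.
; The first exit waits a configurable delay, then removes the widget from its parent.
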(event `self.BoxActivate.OnComponentBeginOverlap`
  (params (OverlappedComponent :type "PrimitiveComponent Object Reference") (OtherActor :type "Actor Object Reference") (OtherComp :type "PrimitiveComponent Object Reference") (OtherBodyIndex :type Integer) (bFromSweep :type Boolean) (SweepResult :type "HitResult Structure (by ref)"))
  (if (== OtherActor (`/Game/_Mechanics/QuestSystem/BPL_CommonFunctionLibrary.GetMyPlayerCharacter`))
    (`/Engine/EditorBlueprintResources/StandardMacros.DoOnce` false
      (:`Completed`
        (bind _returnvalue (`|CreateWidget` "/Game/_Layout/HUD/Content/WB_PopTextWithFace.WB_PopTextWithFace_C" null (`self.Text_Speak`)))
        (bind _output_get (set `self.Facie` _returnvalue))
        (`|ExecutionSequence`
          (:`then_0`
            (bind _wb_tutorialcommand (`/Game/_Layout/HUD/Content/WB_PopTextWithFace.WB_TutorialCommand` _output_get))
            (set `/Game/_Mechanics/Input/Actions/CommonInput/Refs/WB_TutorialCommand.InputSelection` (`self.Enumerate`) _wb_tutorialcommand))
          (:`then_1`
            (set `/Game/_Mechanics/Input/Actions/CommonInput/Refs/WB_TutorialCommand.ActionText` (`self.Action from Widget`) _wb_tutorialcommand))
          (:`then_2`
            (set `/Game/_Mechanics/Input/Actions/CommonInput/Refs/WB_TutorialCommand.SafeHaven?` (`self.Safe Bool?`) _wb_tutorialcommand))
          (:`then_3`
            (`UserWidget.AddToViewport` _output_get 0)))))))

(event `self.BoxActivate.OnComponentEndOverlap`
  (params (OverlappedComponent :type "PrimitiveComponent Object Reference") (OtherActor :type "Actor Object Reference") (OtherComp :type "PrimitiveComponent Object Reference") (OtherBodyIndex :type Integer))
  (if (== OtherActor (`/Game/_Mechanics/QuestSystem/BPL_CommonFunctionLibrary.GetMyPlayerCharacter`))
    (`/Engine/EditorBlueprintResources/StandardMacros.DoOnce` false
      (:`Completed`
        (`KismetSystemLibrary.Delay` (`self.DelayToRemove`))
        (bind _facie (`self.Facie`)
          (:`then`
            (`Widget.RemoveFromParent` _facie))
          (:`else`))))))

(fn `UserConstructionScript`)