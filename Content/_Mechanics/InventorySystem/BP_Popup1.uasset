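; BP_Popup1 is a trigger volume that shows a one-time text popup when the player character enters its BoxActivate component.
; On first overlap it creates a WB_PopText widget with its text, adds it to the viewport and removes it after five seconds.
; The first exit removes the widget after a one-second delay.
; Separate DoOnce nodes, never reset, gate entry and exit.
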(event `self.BoxActivate.OnComponentBeginOverlap`
  (params (OverlappedComponent :type "PrimitiveComponent Object Reference") (OtherActor :type "Actor Object Reference") (OtherComp :type "PrimitiveComponent Object Reference") (OtherBodyIndex :type Integer) (bFromSweep :type Boolean) (SweepResult :type "HitResult Structure (by ref)"))
  (if (== OtherActor (`/Game/_Mechanics/QuestSystem/BPL_CommonFunctionLibrary.GetMyPlayerCharacter`))
    (`/Engine/EditorBlueprintResources/StandardMacros.DoOnce` false
      (:`Completed`
        (bind _returnvalue (`|CreateWidget` "/Game/_Layout/HUD/Content/WB_PopText.WB_PopText_C" null (`self.Text_Speak`)))
        (bind _output_get (set `self.Widget` _returnvalue))
        (set `/Game/_Layout/HUD/Content/WB_PopText.Main_ext` (`self.Text`) _output_get)
        (bind _widget (`self.Widget`)
          (:`then`
            (`UserWidget.AddToViewport` _widget 0)
            (`KismetSystemLibrary.Delay` 5.0)
            (`Widget.RemoveFromParent` _widget))
          (:`else`))))))

(event `self.BoxActivate.OnComponentEndOverlap`
  (params (OverlappedComponent :type "PrimitiveComponent Object Reference") (OtherActor :type "Actor Object Reference") (OtherComp :type "PrimitiveComponent Object Reference") (OtherBodyIndex :type Integer))
  (if (== OtherActor (`/Game/_Mechanics/QuestSystem/BPL_CommonFunctionLibrary.GetMyPlayerCharacter`))
    (`/Engine/EditorBlueprintResources/StandardMacros.DoOnce` false
      (:`Completed`
        (`KismetSystemLibrary.Delay` 1.0)
        (bind _widget (`self.Widget`)
          (:`then`
            (`Widget.RemoveFromParent` _widget))
          (:`else`))))))

(fn `UserConstructionScript`)