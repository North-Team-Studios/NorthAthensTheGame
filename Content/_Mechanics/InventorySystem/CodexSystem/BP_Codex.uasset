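; BP_Codex is a spinning codex pickup that can stay locked until the player has killed enough enemies.
; It starts hidden without collision, and Tick polls GM_Level's kill count, when condition-dependent, to reveal it once.
; Player overlap hides it, plays a sound and briefly shows a WB_DoorPopText popup before destroying the actor.
; The pickup itself records nothing in an inventory, and its PickUpKey call never runs.
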(event `self.ReceiveBeginPlay`
  (bind _returnvalue (`|CreateWidget` "/Game/_Mechanics/InventorySystem/DoorLockSystem/WB_DoorPopText.WB_DoorPopText_C" null (`self.Pick Up Text`) (`self.File Name`) "NewEnumerator2"))
  (set `self.Item PopUp` _returnvalue)
  (bind _asgm_level (cast `/Game/_Maps/GameModes/GM_Level` (`GameplayStatics.GetGameMode`)))
  (set `self.Game Mode` _asgm_level)
  (`SceneComponent.SetVisibility` (`self.StaticMesh`) false false)
  (`PrimitiveComponent.SetCollisionEnabled` (`self.Box`) "NoCollision"))

(event `self.ReceiveTick`
  (params (DeltaSeconds :type "Float (single-precision)"))
  (`SceneComponent.K2_AddRelativeRotation` (`self.StaticMesh`) (`KismetMathLibrary.MakeRotator` 0.0 0.0 -3.0) false false)
  (if (not (`self.IsTaken?`))
    ;[1 1 1] Check if it's available
    (bind _item_status (`self.Quantity to Unlock` (`self.ConditionDependant?`) (`self.CountCondition`)))
    (if _item_status
      (`/Engine/EditorBlueprintResources/StandardMacros.DoOnce` false
        (:`Completed`
          (`SceneComponent.SetVisibility` (`self.StaticMesh`) true false)
          (`PrimitiveComponent.SetCollisionEnabled` (`self.Box`) "QueryAndPhysics")
          (`KismetSystemLibrary.PrintString` "Liberadoh"))))))

(event `self.Box.OnComponentBeginOverlap`
  (params (OverlappedComponent :type "PrimitiveComponent Object Reference") (OtherActor :type "Actor Object Reference") (OtherComp :type "PrimitiveComponent Object Reference") (OtherBodyIndex :type Integer) (bFromSweep :type Boolean) (SweepResult :type "HitResult Structure (by ref)"))
  (if (== OtherActor (`/Game/_Mechanics/QuestSystem/BPL_CommonFunctionLibrary.GetMyPlayerCharacter`))
    (`ActorComponent.K2_DestroyComponent` (`self.Box`))
    (`SceneComponent.SetVisibility` (`self.StaticMesh`) false false)
    (`self.ShowMessage`)
    (set `self.IsTaken?` true)
    (`GameplayStatics.PlaySound2D` "/Game/_Materials/Sounds/Effects/SFX_CodexPick.SFX_CodexPick" 1.0 1.0 0.5 null null)))

(event `ShowMessage`
  (bind _item_popup (`self.Item PopUp`))
  (`UserWidget.AddToViewport` _item_popup 0)
  (`KismetSystemLibrary.Delay` 3.0)
  (`Widget.RemoveFromParent` _item_popup)
  (`self.K2_DestroyActor`))

(fn `Interact With`
  (returns (ObjectiveID :type String))
  (return ""))

(fn `Quantity to Unlock`
  (params (`ConditionDependent?` :type Boolean) (CountCondition :type Integer))
  (returns (`Item Status` :type Boolean))
  (if `ConditionDependent?`
    (bind _enemycount (`/Game/_Maps/GameModes/GM_Level.Get Enemies Killed` (`self.Game Mode`)))
    (if (>= _enemycount CountCondition)
      _
      (else
        (return false))))
  (return true))

(fn `UserConstructionScript`)