(event `self.ReceiveBeginPlay`
  (bind _returnvalue (`|CreateWidget` "/Game/_Mechanics/InventorySystem/DoorLockSystem/WB_DoorPopText.WB_DoorPopText_C" null "You got:" (`self.Key Name`) "NewEnumerator1"))
  (set `self.Item PopUp` _returnvalue)
  (switch `/Game/_Materials/Props/E_StaticVariables` (`self.KeyVariables`)
    (:`NewEnumerator0`
      (set `self.New SM` "/Game/_Materials/Props/sm_keys_sm_key_006.sm_keys_sm_key_006"))
    (:`NewEnumerator1`
      (set `self.New SM` "/Game/_Materials/Props/sm_keys_sm_key_007.sm_keys_sm_key_007"))
    (:`NewEnumerator2`
      (set `self.New SM` "/Game/_Materials/Props/sm_keys_sm_key_008.sm_keys_sm_key_008"))
    (:`NewEnumerator3`
      (set `self.New SM` "/Game/_Materials/Props/sm_keys_sm_key_009.sm_keys_sm_key_009")))
  (`StaticMeshComponent.SetStaticMesh` (`self.StaticMesh`) (`self.New SM`)))

(event `self.ReceiveTick`
  (params (DeltaSeconds :type "Float (single-precision)"))
  (`SceneComponent.K2_AddRelativeRotation` (`self.StaticMesh`) (`KismetMathLibrary.MakeRotator` 0.0 0.0 -3.0) false false))

(event `self.Box.OnComponentBeginOverlap`
  (params (OverlappedComponent :type "PrimitiveComponent Object Reference") (OtherActor :type "Actor Object Reference") (OtherComp :type "PrimitiveComponent Object Reference") (OtherBodyIndex :type Integer) (bFromSweep :type Boolean) (SweepResult :type "HitResult Structure (by ref)"))
  (if (== OtherActor (`/Game/_Mechanics/QuestSystem/BPL_CommonFunctionLibrary.GetMyPlayerCharacter`))
    (`/Game/_Mechanics/InventorySystem/DoorLockSystem/BPI_DoorLockSystem.PickUpKey` (`self.Door`))
    (`ActorComponent.K2_DestroyComponent` (`self.Box`))
    (`SceneComponent.SetVisibility` (`self.StaticMesh`) false false)
    (`self.ShowMessage`)
    (`GameplayStatics.PlaySound2D` "/Game/_Materials/Sounds/Effects/SFX_PickUpKey.SFX_PickUpKey" 1.0 1.0 0.0 null null)))

(event `ShowMessage`
  (bind _item_popup (`self.Item PopUp`))
  (`UserWidget.AddToViewport` _item_popup 0)
  (`KismetSystemLibrary.Delay` 3.0)
  (`Widget.RemoveFromParent` _item_popup)
  (`self.K2_DestroyActor`))

(fn `Interact With`
  (returns (ObjectiveID :type String))
  (return ""))

(fn `UserConstructionScript`)