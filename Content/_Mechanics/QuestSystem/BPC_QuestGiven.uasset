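; BPC_QuestGiven is a quest-giver component that offers a quest to the player through a UI widget.
; NewQuest checks the player's BPCQuestLog and, if the quest is not active, calls DisplayQuest and returns the owner's display name, otherwise an empty string.
; DisplayQuest looks up the quest row from a data table handle and shows it in a WB_Quest widget on the viewport.
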(fn `DisplayQuest`
  (bind (_questdata_datatable _questdata_rowname) (break `DataTableRowHandle` (`self.QuestData`)))
  (bind _returnvalue (`|GetDataTableRow` _questdata_datatable _questdata_rowname)
    (:`then`
      (bind _returnvalue_2 (`|CreateWidget` "/Game/_Layout/HUD/Content/WB_Quest.WB_Quest_C" null _returnvalue))
      (`UserWidget.AddToViewport` _returnvalue_2 0))))

(fn `NewQuest`
  (returns (ObjectiveID :type String))
  (bind (_questdata_datatable _questdata_rowname) (break `DataTableRowHandle` (`self.QuestData`)))
  (if (not (`/Game/_Mechanics/QuestSystem/BPC_QuestLog.QueryActiveQuest` (`/Game/Characters/Jogador/Blueprint/BP_Jogador.BPC_QuestLog` (`/Game/_Mechanics/QuestSystem/BPL_CommonFunctionLibrary.GetMyPlayerCharacter`)) _questdata_rowname))
    (`self.DisplayQuest`)
    (return (`KismetSystemLibrary.GetDisplayName` (`self.GetOwner`)))
    (else
      (return ""))))