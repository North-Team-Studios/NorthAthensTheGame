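; Repairable level objective: the player holds an interaction inside its box to fix it, then the game advances progress and loads the 02AreaSegura level.
; Box overlap shows the hold prompt and allows repair; externally triggered Lookat calls accumulate delta time into the HUD repair bar while playing the fix montage with the pistol removed.
; Completion destroys the smoke and Niagara effects and disables the box; Cancel resets timer, bar, animation and pistol.
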(event `self.ReceiveBeginPlay`
  (`|ExecutionSequence`
    (:`then_0`
      (if (`self.ShowDebugBox?`)
        (`KismetSystemLibrary.DrawDebugBox` (`self.K2_GetActorLocation`) (`self.In Box Extent`) (struct :`G` 0.131249 :`B` 1.0 :`A` 1.0) (struct) 999.0 5.0)))
    (:`then_1`
      (bind _returnvalue (`|CreateWidget` "/Game/_Layout/HUD/Content/Interaction/WB_Interaction_Hold.WB_Interaction_Hold_C"))
      (bind _output_get (set `self.HUD Interaction` _returnvalue))
      (`/Game/_Layout/HUD/Content/Interaction/WB_Interaction_Hold.Set_Title_Label` _output_get (`self.Title Lable`))
      (`WidgetComponent.SetWidget` (`self.Widget`) (`self.HUD Interaction`)))))

(event `self.Box.OnComponentBeginOverlap`
  (params (OverlappedComponent :type "PrimitiveComponent Object Reference") (OtherActor :type "Actor Object Reference") (OtherComp :type "PrimitiveComponent Object Reference") (OtherBodyIndex :type Integer) (bFromSweep :type Boolean) (SweepResult :type "HitResult Structure (by ref)"))
  (`SceneComponent.SetVisibility` (`self.Widget`) true false)
  (set `self.Actor` OtherActor)
  (set `self.InteractAllowed?` true)
  (bind _wb_repairingbar (`/Game/_Layout/HUD/GM_Huds/WB_HUD.WB_RepairingBar` (`/Game/_Mechanics/QuestSystem/BPL_CommonFunctionLibrary.GetMyHud` "NewEnumerator0"))
    (:`then`
      (set `self.WB Repairing Bar` _wb_repairingbar))
    (:`else`)))

(event `self.Box.OnComponentEndOverlap`
  (params (OverlappedComponent :type "PrimitiveComponent Object Reference") (OtherActor :type "Actor Object Reference") (OtherComp :type "PrimitiveComponent Object Reference") (OtherBodyIndex :type Integer))
  (`SceneComponent.SetVisibility` (`self.Widget`) false false)
  (set `self.InteractAllowed?` false))

(event `/Game/_Mechanics/BPI_MainInteract.LookAt`
  (bind _myplayercharacter (`/Game/_Mechanics/QuestSystem/BPL_CommonFunctionLibrary.GetMyPlayerCharacter`))
  (set `Widget.Visibility` "HitTestInvisible" (`self.WB Repairing Bar`))
  (if (`self.InteractAllowed?`)
    (bind _output_get (set `self.Time` (+ (`self.Time`) (`GameplayStatics.GetWorldDeltaSeconds`))))
    (if (> _output_get (`self.TimeToBuild`))
      (bind _p_smoke_d (`self.P_Smoke_D`)
        (:`then`
          (`ActorComponent.K2_DestroyComponent` _p_smoke_d)
          ;[1 1 1] Alteration
          (bind _dohere_fx_niagara (`self.DoHere_FX_Niagara`)
            (:`then`
              (`ActorComponent.K2_DestroyComponent` _dohere_fx_niagara)
              (set `Widget.Visibility` "Hidden" (`self.WB Repairing Bar`))
              (`self.RemoveBoxCollider`)
              (set `self.isDone?` true)
              (bind _asbpi_game_instance (cast `/Game/_Mechanics/SaveGame/BPI_GameInstance` (`GameplayStatics.GetGameInstance`)))
              (`/Game/_Mechanics/SaveGame/BPI_GameInstance.SetNewProgress` _asbpi_game_instance 5)
              (set `/Game/Characters/Jogador/Blueprint/BP_Jogador.isInteracting?` false _myplayercharacter)
              (`/Game/Characters/Jogador/Blueprint/BP_Jogador.Add Pistol` _myplayercharacter)
              (`self.EndLevel`))
            (:`else`)))
        (:`else`))
      (else
        (`|ExecutionSequence`
          (:`then_0`
            (`/Game/_Layout/HUD/Content/Fix/WB_RepairingBar.SetPercent` (`self.WB Repairing Bar`) (`self.Time`) (`self.TimeToBuild`)))
          (:`then_1`
            (if (not (`self.isDone?`))
              (`self.Animation`))))))))

(event `RemoveBoxCollider`
  (`/Engine/EditorBlueprintResources/StandardMacros.DoOnce` false
    (:`Completed`
      (bind _box (`self.Box`)
        (:`then`
          (`PrimitiveComponent.SetCollisionEnabled` _box "NoCollision"))
        (:`else`)))))

(event `Animation`
  (bind _myplayercharacter (`/Game/_Mechanics/QuestSystem/BPL_CommonFunctionLibrary.GetMyPlayerCharacter`))
  (`/Engine/EditorBlueprintResources/StandardMacros.DoOnce` false :!label _label
    (:`Completed`
      (`/Game/Characters/Jogador/Blueprint/BP_Jogador.Remove Pistol` _myplayercharacter)
      (set `/Game/Characters/Jogador/Blueprint/BP_Jogador.isInteracting?` true _myplayercharacter)
      (`|PlayMontage` (`Character.Mesh` _myplayercharacter) (`self.Fix Montage`) 0.5
        (:`then`
          (`GameplayStatics.PlaySound2D` "/Game/_Materials/Sounds/PowerFix.PowerFix" 0.05 1.1 0.0 null null))
        (:`OnCompleted`
          (goto _label :!via `Reset`))
        (:`OnInterrupted`
          (goto _label :!via `Reset`))))))

(event `/Game/_Mechanics/BPI_MainInteract.Cancel`
  (bind _myplayercharacter (`/Game/_Mechanics/QuestSystem/BPL_CommonFunctionLibrary.GetMyPlayerCharacter`))
  ;[1 0 0.7708] Cancel
  (set `self.Time` 0.0)
  (`/Game/_Layout/HUD/Content/Fix/WB_RepairingBar.SetPercent` (`self.WB Repairing Bar`) 0.0 (`self.TimeToBuild`))
  (set `Widget.Visibility` "Hidden" (`self.WB Repairing Bar`))
  (`Character.StopAnimMontage` _myplayercharacter (`self.Fix Montage`))
  (`/Game/Characters/Jogador/Blueprint/BP_Jogador.Add Pistol` _myplayercharacter)
  (set `/Game/Characters/Jogador/Blueprint/BP_Jogador.isInteracting?` false (`/Game/_Mechanics/QuestSystem/BPL_CommonFunctionLibrary.GetMyPlayerCharacter`)))

(event `EndLevel`
  ;[1 1 1] End Level
  (`KismetSystemLibrary.Delay` 1.0)
  (bind _asbpi_game_instance (cast `/Game/_Mechanics/SaveGame/BPI_GameInstance` (`GameplayStatics.GetGameInstance`)))
  (`/Game/_Mechanics/SaveGame/BPI_GameInstance.LoadNewLevel` _asbpi_game_instance "02AreaSegura" false))

(fn `Interact With`
  (returns (ObjectiveID :type String))
  (bind _objective_id (`self.Objective ID`))
  (`KismetSystemLibrary.PrintString` _objective_id true true (struct :`G` 0.66 :`B` 1.0 :`A` 1.0) 0.0)
  (return _objective_id))

(fn `IsMoving`
  (returns (`isMoving?` :type Boolean))
  (return (> (`KismetMathLibrary.VSize` (`self.GetVelocity` (`GameplayStatics.GetPlayerCharacter` 0))) 0.0)))

(fn `UserConstructionScript`)