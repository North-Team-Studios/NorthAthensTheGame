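; Hold-to-interact tree objective that the player grows in place, then saves progress and loads the 02AreaSegura level.
; Box overlap shows the widget and enables interaction.
; Lookat accumulates time, scaling the mesh while driving a progress bar, crop FX and a fix montage with the pistol removed.
; Cancel restores prompt, pistol and effects but keeps accumulated time; completion also destroys the marker FX and disables the box.
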(event `self.ReceiveBeginPlay`
  (`|ExecutionSequence`
    (:`then_0`
      (if (`self.ShowDebugBox?`)
        (`KismetSystemLibrary.DrawDebugBox` (`self.K2_GetActorLocation`) (`self.In Box Extent`) (struct :`G` 0.131249 :`B` 1.0 :`A` 1.0) (struct) 999.0 5.0)))
    (:`then_1`
      (bind _returnvalue (`|CreateWidget` "/Game/_Layout/HUD/Content/Interaction/WB_Interaction_Hold.WB_Interaction_Hold_C"))
      (bind _output_get (set `self.HUD Interaction` _returnvalue))
      (`/Game/_Layout/HUD/Content/Interaction/WB_Interaction_Hold.Set_Title_Label` _output_get (`self.Title Lable`))
      (`WidgetComponent.SetWidget` (`self.Widget`) (`self.HUD Interaction`)))
    (:`then_2`
      (bind _returnvalue_2 (`|CreateWidget` "/Game/_Layout/HUD/Content/Fix/WB_RepairingBar.WB_RepairingBar_C"))
      (set `self.HUD ProgressBar` _returnvalue_2))
    (:`then_3`
      (bind _asbpi_game_instance (cast `/Game/_Mechanics/SaveGame/BPI_GameInstance` (`GameplayStatics.GetGameInstance`)))
      (set `self.As BPI Game Instance` _asbpi_game_instance))))

(event `self.Box.OnComponentBeginOverlap`
  (params (OverlappedComponent :type "PrimitiveComponent Object Reference") (OtherActor :type "Actor Object Reference") (OtherComp :type "PrimitiveComponent Object Reference") (OtherBodyIndex :type Integer) (bFromSweep :type Boolean) (SweepResult :type "HitResult Structure (by ref)"))
  (`SceneComponent.SetVisibility` (`self.Widget`) true false)
  (set `self.Actor` OtherActor)
  (set `self.InteractAllowed?` true))

(event `self.Box.OnComponentEndOverlap`
  (params (OverlappedComponent :type "PrimitiveComponent Object Reference") (OtherActor :type "Actor Object Reference") (OtherComp :type "PrimitiveComponent Object Reference") (OtherBodyIndex :type Integer))
  (`SceneComponent.SetVisibility` (`self.Widget`) false false)
  (set `self.InteractAllowed?` false))

(event `self.LookAt`
  (bind _myplayercharacter (`/Game/_Mechanics/QuestSystem/BPL_CommonFunctionLibrary.GetMyPlayerCharacter`))
  (bind _timetobuild (`self.TimeToBuild`))
  (`MovementComponent.StopMovementImmediately` (`Character.CharacterMovement` (`GameplayStatics.GetPlayerCharacter` 0)))
  (if (`self.InteractAllowed?`)
    (bind _output_get (set `self.Time` (+ (`self.Time`) (`GameplayStatics.GetWorldDeltaSeconds`))))
    (bind _returnvalue (* (/ _output_get _timetobuild) 0.45))
    ;[0 1 0.05694] Set Tree Size on Channeling
    (`SceneComponent.SetRelativeScale3D` (`self.StaticMesh`) (`KismetMathLibrary.MakeVector` _returnvalue _returnvalue _returnvalue))
    (if (> _output_get _timetobuild)
      (bind _dohere_fx_niagara (`self.DoHere_FX_Niagara`)
        (:`then`
          (`ActorComponent.K2_DestroyComponent` _dohere_fx_niagara)
          (`self.RemoveBoxCollider`)
          (set `self.isDone?` true)
          (bind _asbpi_game_instance (cast `/Game/_Mechanics/SaveGame/BPI_GameInstance` (`GameplayStatics.GetGameInstance`)))
          (`/Game/_Mechanics/SaveGame/BPI_GameInstance.SetNewProgress` _asbpi_game_instance 12)
          (`/Game/Characters/Jogador/Blueprint/BP_Jogador.Add Pistol` _myplayercharacter)
          (set `/Game/Characters/Jogador/Blueprint/BP_Jogador.isInteracting?` false _myplayercharacter)
          (`self.End Level`))
        (:`else`))
      (else
        (`|ExecutionSequence`
          (:`then_0`
            (`WidgetComponent.SetWidget` (`self.Widget`) (`self.HUD ProgressBar`))
            (`/Game/_Layout/HUD/Content/Fix/WB_RepairingBar.SetPercent` (`self.HUD ProgressBar`) (`self.Time`) (`self.TimeToBuild`))
            (`ActorComponent.Activate` (`self.Cropfx`) false))
          (:`then_1`
            (if (not (`self.isDone?`))
              (`self.Animation`))))))))

(event `self.Cancel`
  (bind _myplayercharacter (`/Game/_Mechanics/QuestSystem/BPL_CommonFunctionLibrary.GetMyPlayerCharacter`))
  (`WidgetComponent.SetWidget` (`self.Widget`) (`self.HUD Interaction`))
  (`/Game/_Layout/HUD/Content/Fix/WB_RepairingBar.SetPercent` (`self.HUD ProgressBar`) 0.0 (`self.TimeToBuild`))
  (`Character.StopAnimMontage` _myplayercharacter (`self.Fix Montage`))
  (`/Game/Characters/Jogador/Blueprint/BP_Jogador.Add Pistol` _myplayercharacter)
  (set `/Game/Characters/Jogador/Blueprint/BP_Jogador.isInteracting?` false _myplayercharacter)
  (`ActorComponent.Deactivate` (`self.Cropfx`)))

(event `RemoveBoxCollider`
  (`/Engine/EditorBlueprintResources/StandardMacros.DoOnce` false
    (:`Completed`
      (bind _box (`self.Box`)
        (:`then`
          (`PrimitiveComponent.SetCollisionEnabled` _box "NoCollision"))
        (:`else`)))))

(event `Animation`
  (bind _myplayercharacter (`/Game/_Mechanics/QuestSystem/BPL_CommonFunctionLibrary.GetMyPlayerCharacter`))
  (`/Engine/EditorBlueprintResources/StandardMacros.DoOnce` false :!label _label
    (:`Completed`
      (`/Game/Characters/Jogador/Blueprint/BP_Jogador.Remove Pistol` _myplayercharacter)
      (set `/Game/Characters/Jogador/Blueprint/BP_Jogador.isInteracting?` true _myplayercharacter)
      (`|PlayMontage` (`Character.Mesh` _myplayercharacter) (`self.Fix Montage`)
        (:`OnCompleted`
          (goto _label :!via `Reset`))
        (:`OnInterrupted`
          (goto _label :!via `Reset`))))))

(event `End Level`
  (`KismetSystemLibrary.Delay` 1.0)
  (`/Game/_Mechanics/SaveGame/BPI_GameInstance.LoadNewLevel` (`self.As BPI Game Instance`) "02AreaSegura" false))

(fn `Interact With`
  (returns (ObjectiveID :type String))
  (bind _objective_id (`self.Objective ID`))
  (`KismetSystemLibrary.PrintString` _objective_id true true (struct :`G` 0.66 :`B` 1.0 :`A` 1.0) 0.0)
  (return _objective_id))

(fn `IsMoving`
  (returns (`isMoving?` :type Boolean))
  (return (> (`KismetMathLibrary.VSize` (`self.GetVelocity` (`GameplayStatics.GetPlayerCharacter` 0))) 0.0)))

(fn `UserConstructionScript`)