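; Safe Haven tree interactable that plays a story beat about the giant tree clearing the smoke.
; Box overlap shows its prompt widgets to the player, with the progress check left unwired.
; Lookat, only at game progress 6, hides them, disables input and shows two timed, DoOnce-guarded popup dialogues.
; It then advances progress to 7 through the GameInstance interface, restores input and makes tree calls marked deprecated.
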(event `self.ReceiveBeginPlay`
  (bind _asbpi_game_instance (cast `/Game/_Mechanics/SaveGame/BPI_GameInstance` (`GameplayStatics.GetGameInstance`)))
  (set `self.As BPI Game Instance` _asbpi_game_instance))

(event `self.Box.OnComponentBeginOverlap`
  (params (OverlappedComponent :type "PrimitiveComponent Object Reference") (OtherActor :type "Actor Object Reference") (OtherComp :type "PrimitiveComponent Object Reference") (OtherBodyIndex :type Integer) (bFromSweep :type Boolean) (SweepResult :type "HitResult Structure (by ref)"))
  (bind _progress (`/Game/_Mechanics/SaveGame/BPI_GameInstance.GetGameProgress` (`self.As BPI Game Instance`)))
  (if true
    (if (== OtherActor (`GameplayStatics.GetPlayerCharacter` 0))
      (`SceneComponent.SetVisibility` (`self.Widget`) true false)
      (`SceneComponent.SetVisibility` (`self.Dohere`) true false))))

(event `self.Box.OnComponentEndOverlap`
  (params (OverlappedComponent :type "PrimitiveComponent Object Reference") (OtherActor :type "Actor Object Reference") (OtherComp :type "PrimitiveComponent Object Reference") (OtherBodyIndex :type Integer))
  (`SceneComponent.SetVisibility` (`self.Widget`) false false))

(event `/Game/_Mechanics/BPI_MainInteract.LookAt`
  (bind _returnvalue (`GameplayStatics.GetPlayerController` 0))
  (bind _as_bpi_game_instance (`self.As BPI Game Instance`))
  (bind _returnvalue_2 (`Controller.K2_GetPawn` _returnvalue))
  (bind _progress (`/Game/_Mechanics/SaveGame/BPI_GameInstance.GetGameProgress` (`self.As BPI Game Instance`)))
  (if (== _progress 6)
    (`SceneComponent.SetVisibility` (`self.Widget`) false false)
    (`SceneComponent.SetVisibility` (`self.DoHere`) false false)
    (`self.DisableInput` _returnvalue_2 _returnvalue)
    (`self.AddDialogue` "The tree's big, strong and full of leaves. You breathe better when close to it." 4.0)
    (`KismetSystemLibrary.Delay` 4.5)
    (`self.AddDialogue` "It looks like the smoke dissipates almost completely when it gets close to the giant tree." 5.0)
    (`KismetSystemLibrary.Delay` 5.0)
    ;[0 1 0.1195] ADD NEW OBJECTIVE HERE
    (`/Game/_Mechanics/SaveGame/BPI_GameInstance.SetNewProgress` _as_bpi_game_instance 7)
    (`self.EnableInput` _returnvalue_2 _returnvalue)
    ;[1 1 1] Deprecated
    (`/Game/_Mechanics/SaveGame/BPI_GameInstance.TreeInteract` _as_bpi_game_instance)
    (`/Game/_Mechanics/SaveGame/BPI_GameInstance.Toggle Tree` _as_bpi_game_instance false)))

(event `AddDialogue`
  (params (Text :type Text) (BoxDuration :type "Float (double-precision)"))
  (`/Engine/EditorBlueprintResources/StandardMacros.DoOnce` false :!label _label
    (:`Completed`
      (bind _returnvalue (`|CreateWidget` "/Game/_Layout/HUD/Content/WB_PopDialog.WB_PopDialog_C" null Text))
      (`UserWidget.AddToViewport` _returnvalue 0)
      (`KismetSystemLibrary.Delay` BoxDuration)
      (`Widget.RemoveFromParent` _returnvalue)
      (goto _label :!via `Reset`))))

(fn `Interact With`
  (returns (ObjectiveID :type String))
  (return ""))

(fn `UserConstructionScript`)